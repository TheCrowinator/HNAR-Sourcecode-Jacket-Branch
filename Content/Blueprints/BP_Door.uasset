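; Door that players open and close and the neighbour AI passes through via a smart nav link, with locking and chair barricades.
; Toggling slides or rotates the door with MoveComponentTo and sound; a placed chair locks it.
; On link arrival the AI plays a direction-aware opening animation and closes behind itself, or rattles or breaks through a chair barricade, depending on settings.
; A looping timer maintains chair lock state and reapplies door pose in multiplayer sessions.
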(event OnComponentBeginOverlap(Box)
  (params (OverlappedComponent :type Primitive%20Component%20Object%20Reference) (OtherActor :type Actor%20Object%20Reference) (OtherComp :type Primitive%20Component%20Object%20Reference) (OtherBodyIndex :type Integer) (bFromSweep :type Boolean) (SweepResult :type Hit%20Result%20Structure%20%28by%20ref%29)))

(event OnComponentBeginOverlap(Box1)
  (params (OverlappedComponent :type Primitive%20Component%20Object%20Reference) (OtherActor :type Actor%20Object%20Reference) (OtherComp :type Primitive%20Component%20Object%20Reference) (OtherBodyIndex :type Integer) (bFromSweep :type Boolean) (SweepResult :type Hit%20Result%20Structure%20%28by%20ref%29))
  (Utilities|Casting|CastToAI OtherActor)
  (Utilities|Casting|CastToCapsuleComponent OtherComp)
  (Variables|Default|SetOutwards? true)
  (Development|PrintString "Outwards" true true "(R=0.978821,G=1.000000,B=0.000000,A=1.000000)"))

(event OnSmartLinkReached(NavLink)
  (params (MovingActor :type Actor%20Object%20Reference) (DestinationPoint :type Vector%20%28by%20ref%29 :default "0, 0, 0"))
  (bind _door (Variables|Default|GetDoor))
  (bind _door_2 (Variables|Default|GetDoor))
  (bind _outwards_ (Variables|Default|GetOutwards?))
  (if (Actor|ActorHasTag (Variables|Default|GetNavLink) "Door")
    (Development|PrintString "open door")
    (bind _asai (Utilities|Casting|CastToAI MovingActor))
    (bind _output_get (Variables|Default|SetAI _asai))
    (if (Variables|Default|GetCanAIOpen?)
      (Transformation|SetActorRotation _output_get (Math|Rotator|MakeRotator 0.0 0.0 (.yaw (Math|Rotator|FindLookatRotation (Transformation|GetActorLocation _output_get) (Transformation|GetWorldLocation (Variables|Default|GetScene))))))
      (if (Variables|Default|GetLocked)
        (if (Variables|Default|GetIsLockedWithChair?)
          (Audio|PlaySoundatLocation (Variables|Default|GetLockedSound) (Transformation|GetWorldLocation (Variables|Default|GetDoor)) "0, 0, 0" 1.0 1.0 0.0 "/Game/Sounds/Attenuation/OnlyDoorAttenuation.OnlyDoorAttenuation" 0 0)
          (Pawn|Components|CharacterMovement|DisableMovement (Variables|/Script/Engine.Character|GetCharacterMovement _output_get))
          (if (Utilities|Enum|Equal(Enum) (Variables|/Game/Blueprints/Characters/AI2/AI.AI_C|GetCurrentState _output_get) "NewEnumerator0")
            (if (Variables|Default|GetCanBreakDownDoorIdle?)
              (if (Variables|Default|GetCanBreakDownDoor?) :!label _label
                (CallFunction|BreakThroughChair)
                (else
                  (bind _anim_length (Default|PlayAnimAI _output_get "/Game/Neighbor/Animations/neighbour_lowpoly_Anim_rig_open_door_outward.neighbour_lowpoly_Anim_rig_open_door_outward" false :!label _label_2))
                  (Audio|PlaySoundatLocation (Variables|Default|GetLockedSound) (Transformation|GetWorldLocation (Variables|Default|GetDoor)) "0, 0, 0" 1.0 1.0 0.0 "/Game/Sounds/Attenuation/OnlyDoorAttenuation.OnlyDoorAttenuation" 0 0)
                  (Utilities|FlowControl|Delay _anim_length)
                  (Components|Animation|SetAnimationMode (Variables|/Script/Engine.Character|GetMesh _output_get) "AnimationBlueprint")
                  (Pawn|Components|CharacterMovement|SetMovementMode (Variables|/Script/Engine.Character|GetCharacterMovement _output_get) "MOVE_Walking" 0)))
              (else
                (goto _label_2)))
            (else
              (goto _label)))
          (else
            (goto _label_2)))
        (else
          (if (Variables|Default|GetOpen)
            (if (Variables|Default|GetCloseDoorIfOpen?)
              _
              (else
                (Utilities|FlowControl|Delay 1.24)))
            (else
              (Variables|/Game/Blueprints/Characters/AI2/AI.AI_C|SetCanAIKick _output_get false)
              (Pawn|Components|CharacterMovement|DisableMovement (Variables|/Script/Engine.Character|GetCharacterMovement _output_get))
              (Components|Animation|SetAnimationMode (Variables|/Script/Engine.Character|GetMesh _output_get) "AnimationSingleNode")
              (if (Variables|Default|GetDoubleDoor?)
                (if _outwards_
                  (Components|Animation|PlayAnimation (Variables|/Script/Engine.Character|GetMesh _output_get) "/Game/Neighbor/Animations/neighbour_lowpoly_Anim_rig_open_double_door_outward.neighbour_lowpoly_Anim_rig_open_double_door_outward" false)
                  (else
                    (Components|Animation|PlayAnimation (Variables|/Script/Engine.Character|GetMesh _output_get) "/Game/Neighbor/Animations/neighbour_lowpoly_Anim_rig_open_double_door_inward.neighbour_lowpoly_Anim_rig_open_double_door_inward" false)))
                (elif _outwards_
                  (Components|Animation|PlayAnimation (Variables|/Script/Engine.Character|GetMesh _output_get) "/Game/Neighbor/Animations/neighbour_lowpoly_Anim_rig_open_door_outward_l_h.neighbour_lowpoly_Anim_rig_open_door_outward_l_h" false)
                  (else
                    (Components|Animation|PlayAnimation (Variables|/Script/Engine.Character|GetMesh _output_get) "/Game/Neighbor/Animations/neighbour_lowpoly_Anim_rig_open_door_inward.neighbour_lowpoly_Anim_rig_open_door_inward" false))))
              (Utilities|FlowControl|Delay 0.4)
              (Variables|Default|SetOpen true)
              (Audio|SpawnSoundatLocation (Variables|Default|GetOpenSound) (Transformation|GetActorLocation) "0, 0, 0" 1.0 1.0 0.0 "/Game/Sounds/Attenuation/OnlyDoorAttenuation.OnlyDoorAttenuation" 0)
              (Collision|SetCollisionEnabled _door "PhysicsOnly")
              (Components|MoveComponentTo _door_2 (Variables|Default|GetDoorOpen_Location) (Variables|Default|GetDoorOpen_Rotation) false false (Variables|Default|GetOverTime) false)
              (Collision|SetCollisionEnabled _door "QueryAndPhysics")
              (Utilities|FlowControl|Delay 0.54)
              (Components|Animation|SetAnimationMode (Variables|/Script/Engine.Character|GetMesh _output_get) "AnimationBlueprint")
              (Pawn|Components|CharacterMovement|SetMovementMode (Variables|/Script/Engine.Character|GetCharacterMovement _output_get) "MOVE_Walking" 0)))
          (Utilities|FlowControl|Delay 1.5)
          (Collision|SetCollisionEnabled _door "QueryOnly")
          (Components|MoveComponentTo _door_2 (Variables|Default|GetDoorClose_Location) (Variables|Default|GetDoorClose_Rotation) false false (Variables|Default|GetOverTime) false)
          (Audio|PlaySoundatLocation (Variables|Default|GetCloseSound) (Transformation|GetActorLocation) "0, 0, 0" 1.0 1.0 0.0 "/Game/Sounds/Attenuation/OnlyDoorAttenuation.OnlyDoorAttenuation" 0 0)
          (Collision|SetCollisionEnabled (Variables|Default|GetDoor) "QueryAndPhysics")
          (Variables|Default|SetOpen false)
          (Variables|/Game/Blueprints/Characters/AI2/AI.AI_C|SetCanAIKick _output_get true)))
      (else
        (Transformation|SetActorRotation _output_get (Math|Rotator|MakeRotator 0.0 0.0 (.yaw (Math|Rotator|FindLookatRotation (Transformation|GetActorLocation _output_get) (Transformation|GetWorldLocation (Variables|Default|GetScene))))))
        (if (Utilities|Enum|Equal(Enum) (Variables|/Game/Blueprints/Characters/AI2/AI.AI_C|GetCurrentState _output_get) "NewEnumerator0")
          (Default|RandomTask _output_get))))))

(event OnComponentEndOverlap(Box1)
  (params (OverlappedComponent :type Primitive%20Component%20Object%20Reference) (OtherActor :type Actor%20Object%20Reference) (OtherComp :type Primitive%20Component%20Object%20Reference) (OtherBodyIndex :type Integer))
  (Utilities|Casting|CastToAI OtherActor)
  (Utilities|Casting|CastToCapsuleComponent OtherComp)
  (Variables|Default|SetOutwards? false)
  (Development|PrintString "Inwards" true true "(R=0.978821,G=1.000000,B=0.000000,A=1.000000)"))

(event Custom|OpenClose
  (params (Component :type Primitive%20Component%20Object%20Reference))
  (bind _door (Variables|Default|GetDoor))
  (if (== Component (Variables|Default|GetDoor))
    (if (Variables|Default|GetLocked)
      (Audio|SpawnSoundatLocation (Variables|Default|GetLockedSound) (Transformation|GetWorldLocation (Variables|Default|GetScene)) "0, 0, 0" 1.0 1.0 0.0 "/Game/Sounds/Attenuation/OnlyDoorAttenuation.OnlyDoorAttenuation" 0)
      (elif (Variables|Default|GetOpen)
        (Utilities|FlowControl|Sequence
          (:then_0
            (Collision|SetCollisionEnabled _door "PhysicsOnly")
            (Components|MoveComponentTo _door (Variables|Default|GetDoorClose_Location) (Variables|Default|GetDoorClose_Rotation) false false (Variables|Default|GetOverTime) false :!label _label)
            (Audio|SpawnSoundatLocation (Variables|Default|GetCloseSound) (Transformation|GetWorldLocation (Variables|Default|GetScene)) "0, 0, 0" 1.0 1.0 0.0 "/Game/Sounds/Attenuation/OnlyDoorAttenuation.OnlyDoorAttenuation" 0)
            (Collision|SetCollisionEnabled _door "QueryAndPhysics")
            (Variables|Default|SetOpen false))
          (:then_1
            (goto _label_2 Stop)))
        (else
          (Audio|SpawnSoundatLocation (Variables|Default|GetOpenSound) (Transformation|GetWorldLocation (Variables|Default|GetScene)) "0, 0, 0" 1.0 1.0 0.0 "/Game/Sounds/Attenuation/OnlyDoorAttenuation.OnlyDoorAttenuation" 0)
          (Utilities|FlowControl|Sequence
            (:then_0
              (Variables|Default|SetOpen true)
              (Collision|SetCollisionEnabled _door "PhysicsOnly")
              (Components|MoveComponentTo _door (Variables|Default|GetDoorOpen_Location) (Variables|Default|GetDoorOpen_Rotation) false false (Variables|Default|GetOverTime) false :!label _label_2)
              (Collision|SetCollisionEnabled _door "QueryAndPhysics"))
            (:then_1
              (goto _label Stop))))))))

(event Custom|CheckIfOpenOnServer
  (Utilities|FlowControl|Sequence
    (:then_0
      (if (Variables|Default|GetOpen)
        (CallFunction|OpenClientDoors :!label _label)))
    (:then_1
      (if (Variables|Default|GetLocked)
        (goto _label)))))

(event Custom|OpenClient)

(event Custom|OpenClientDoors
  (bind _door (Variables|Default|GetDoor))
  (if (Variables|Default|GetOpen)
    (Transformation|SetRelativeLocationAndRotation _door (Variables|Default|GetDoorOpen_Location) (Variables|Default|GetDoorOpen_Rotation) false false)
    (else
      (Transformation|SetRelativeLocationAndRotation _door (Variables|Default|GetDoorClose_Location) (Variables|Default|GetDoorClose_Rotation) false false))))

(event Custom|OpenCloseAI
  (bind _door (Variables|Default|GetDoor))
  (if (Variables|Default|GetLocked)
    (Audio|SpawnSoundatLocation (Variables|Default|GetLockedSound) (Transformation|GetWorldLocation (Variables|Default|GetScene)) "0, 0, 0" 1.0 1.0 0.0 "/Game/Sounds/Attenuation/OnlyDoorAttenuation.OnlyDoorAttenuation" 0)
    (elif (Variables|Default|GetOpen)
      (Utilities|FlowControl|Sequence
        (:then_0
          (Collision|SetCollisionEnabled _door "PhysicsOnly")
          (Components|MoveComponentTo _door (Variables|Default|GetDoorClose_Location) (Variables|Default|GetDoorClose_Rotation) false false (Variables|Default|GetOverTime) false :!label _label)
          (Audio|SpawnSoundatLocation (Variables|Default|GetCloseSound) (Transformation|GetWorldLocation (Variables|Default|GetScene)) "0, 0, 0" 1.0 1.0 0.0 "/Game/Sounds/Attenuation/OnlyDoorAttenuation.OnlyDoorAttenuation" 0)
          (Collision|SetCollisionEnabled _door "QueryAndPhysics")
          (Variables|Default|SetOpen false))
        (:then_1
          (goto _label_2 Stop)))
      (else
        (Audio|SpawnSoundatLocation (Variables|Default|GetOpenSound) (Transformation|GetWorldLocation (Variables|Default|GetScene)) "0, 0, 0" 1.0 1.0 0.0 "/Game/Sounds/Attenuation/OnlyDoorAttenuation.OnlyDoorAttenuation" 0)
        (Utilities|FlowControl|Sequence
          (:then_0
            (Variables|Default|SetOpen true)
            (Collision|SetCollisionEnabled _door "PhysicsOnly")
            (Components|MoveComponentTo _door (Variables|Default|GetDoorOpen_Location) (Variables|Default|GetDoorOpen_Rotation) false false (Variables|Default|GetOverTime) false :!label _label_2)
            (Collision|SetCollisionEnabled _door "QueryAndPhysics"))
          (:then_1
            (goto _label Stop)))))))

(event Custom|OnSmartLinkReached_Event_0
  (params (MovingActor :type Actor%20Object%20Reference) (DestinationPoint :type Vector%20%28by%20ref%29)))

(event Custom|SetChair
  (params (SelectChair :type BP%20Chair%20Object%20Reference))
  (bind _stool (Variables|Default|GetStool))
  (bind _output_get (Variables|Default|SetSelectChair SelectChair))
  (Transformation|SetActorLocationAndRotation _output_get (Transformation|GetWorldLocation _stool) (Transformation|GetWorldRotation _stool) false true)
  (Physics|SetSimulatePhysics (Variables|/Game/Blueprints/PickUpObjects/BP_Interactable.BP_Interactable_C|GetStaticMesh _output_get) false)
  (Variables|Default|SetLocked true)
  (Variables|Default|SetIsLockedWithChair? true)
  (if (not (Variables|Default|GetCanBreakDownDoor?))
    (Class|NavLinkProxy|SetSmartLinkEnabled (Variables|Default|GetNavLink) false)))

(event Custom|OpenOnEvent
  (bind _door (Variables|Default|GetDoor))
  (if (Variables|Default|GetOpen)
    (Utilities|FlowControl|Sequence
      (:then_0
        (Collision|SetCollisionEnabled _door "PhysicsOnly")
        (Components|MoveComponentTo _door (Variables|Default|GetDoorClose_Location) (Variables|Default|GetDoorClose_Rotation) false false (Variables|Default|GetOverTime) false :!label _label)
        (Audio|SpawnSoundatLocation (Variables|Default|GetCloseSound) (Transformation|GetWorldLocation (Variables|Default|GetScene)) "0, 0, 0" 1.0 1.0 0.0 "/Game/Sounds/Attenuation/OnlyDoorAttenuation.OnlyDoorAttenuation" 0)
        (Collision|SetCollisionEnabled _door "QueryAndPhysics")
        (Variables|Default|SetOpen false))
      (:then_1
        (goto _label_2 Stop)))
    (else
      (Audio|SpawnSoundatLocation (Variables|Default|GetOpenSound) (Transformation|GetWorldLocation (Variables|Default|GetScene)) "0, 0, 0" 1.0 1.0 0.0 "/Game/Sounds/Attenuation/OnlyDoorAttenuation.OnlyDoorAttenuation" 0)
      (Utilities|FlowControl|Sequence
        (:then_0
          (Variables|Default|SetOpen true)
          (Collision|SetCollisionEnabled _door "PhysicsOnly")
          (Components|MoveComponentTo _door (Variables|Default|GetDoorOpen_Location) (Variables|Default|GetDoorOpen_Rotation) false false (Variables|Default|GetOverTime) false :!label _label_2)
          (Collision|SetCollisionEnabled _door "QueryAndPhysics"))
        (:then_1
          (goto _label Stop))))))

(event Custom|BreakThroughChair
  (if (Utilities|Enum|Equal(Enum) (Variables|/Game/Blueprints/Characters/AI2/AI.AI_C|GetCurrentState (stale OnSmartLinkReached(NavLink) _output_get)) "NewEnumerator4")
    (Default|Prolong (stale OnSmartLinkReached(NavLink) _output_get)))
  (Components|Animation|SetAnimationMode (Variables|/Script/Engine.Character|GetMesh (stale OnSmartLinkReached(NavLink) _output_get)) "AnimationSingleNode")
  (Components|Animation|PlayAnimation (Variables|/Script/Engine.Character|GetMesh (stale OnSmartLinkReached(NavLink) _output_get)) "/Game/Neighbor/Montages/pushdoor.pushdoor" false)
  (Variables|/Game/Blueprints/Characters/AI2/AI.AI_C|SetCanHear (stale OnSmartLinkReached(NavLink) _output_get) false)
  (Utilities|FlowControl|Delay 4.2)
  (Physics|SetSimulatePhysics (Variables|/Game/Blueprints/PickUpObjects/BP_Interactable.BP_Interactable_C|GetStaticMesh (Variables|Default|GetSelectChair)) true)
  (Variables|Default|SetSelectChair 0)
  (Variables|Default|SetIsLockedWithChair? false)
  (Variables|Default|SetOpen true)
  (Variables|Default|SetLocked false)
  (Components|MoveComponentTo (Variables|Default|GetDoor) (Variables|Default|GetDoorOpen_Location) (Variables|Default|GetDoorOpen_Rotation) false false 0.2 false)
  (Utilities|FlowControl|Delay 0.1)
  (Variables|/Game/Blueprints/Characters/AI2/AI.AI_C|SetCanHear (stale OnSmartLinkReached(NavLink) _output_get) true)
  (Components|Animation|SetAnimationMode (Variables|/Script/Engine.Character|GetMesh (stale OnSmartLinkReached(NavLink) _output_get)) "AnimationBlueprint")
  (Pawn|Components|CharacterMovement|SetMovementMode (Variables|/Script/Engine.Character|GetCharacterMovement (stale OnSmartLinkReached(NavLink) _output_get)) "MOVE_Walking" 0)
  (if (Utilities|Enum|Equal(Enum) (Variables|/Game/Blueprints/Characters/AI2/AI.AI_C|GetCurrentState (stale OnSmartLinkReached(NavLink) _output_get)) "NewEnumerator0")
    (Class|BlackboardComponent|SetValueasInt (AI|GetBlackboard (stale OnSmartLinkReached(NavLink) _output_get)) (Utilities|Name|MakeLiteralName "HuntTask") 1)
    (Default|SetState (stale OnSmartLinkReached(NavLink) _output_get) "NewEnumerator2")
    (else
      (Utilities|FlowControl|Delay 1.5)
      (Collision|SetCollisionEnabled (Variables|Default|GetDoor) "QueryOnly")
      (Components|MoveComponentTo (Variables|Default|GetDoor) (Variables|Default|GetDoorClose_Location) (Variables|Default|GetDoorClose_Rotation) false false (Variables|Default|GetOverTime) false)
      (Audio|PlaySoundatLocation (Variables|Default|GetCloseSound) (Transformation|GetActorLocation) "0, 0, 0" 1.0 1.0 0.0 "/Game/Sounds/Attenuation/OnlyDoorAttenuation.OnlyDoorAttenuation" 0 0)
      (Collision|SetCollisionEnabled (Variables|Default|GetDoor) "QueryAndPhysics")
      (Variables|Default|SetOpen false)
      (Variables|/Game/Blueprints/Characters/AI2/AI.AI_C|SetCanAIKick (stale OnSmartLinkReached(NavLink) _output_get) true))))

(event Custom|Tick
  (Utilities|FlowControl|Sequence
    (:then_0
      (bind _asgame_instance_hnar (Utilities|Casting|CastToGameInstanceHNAR (Game|GetGameInstance)))
      (if (>= (Class|FindSessionsCallbackProxy|GetCurrentPlayers (Variables|/Game/GameInstanceHNAR.GameInstanceHNAR_C|GetSession _asgame_instance_hnar)) 2)
        (Utilities|FlowControl|Delay 1.0)
        (CallFunction|CheckifOpenonServer)))
    (:then_1
      (Utilities|IsValid (Variables|Default|GetSelectChair)
        (:Is%20Valid
          (Variables|Default|SetLocked true)
          (Variables|Default|SetIsLockedWithChair? true)
          (goto _label Reset))
        (:Is%20Not%20Valid
          (Utilities|FlowControl|DoOnce true :!label _label
            (:Completed
              (Variables|Default|SetLocked false)
              (Variables|Default|SetIsLockedWithChair? false))))))))

(event EventBeginPlay
  (bind _selectchair (Variables|Default|GetSelectChair))
  (Utilities|Time|SetTimerbyEvent (delegate Custom|Tick) 0.01 true)
  (Utilities|FlowControl|Sequence
    (:then_0
      (if (Variables|Default|GetOpen)
        (Transformation|SetRelativeLocationAndRotation (Variables|Default|GetDoor) (Variables|Default|GetDoorOpen_Location) (Variables|Default|GetDoorOpen_Rotation) false false)
        (Variables|Default|SetOpen true)
        (else
          (Transformation|SetRelativeLocationAndRotation (Variables|Default|GetDoor) (Variables|Default|GetDoorClose_Location) (Variables|Default|GetDoorClose_Rotation) false false)
          (Variables|Default|SetOpen false))))
    (:then_1
      (if (Variables|Default|GetIsLockedWithChair?)
        (CallFunction|SetChair (Variables|Default|GetSelectChair))))
    (:then_2
      (Utilities|IsValid _selectchair
        (:Is%20Valid
          (Variables|/Game/Blueprints/PickUpObjects/BP_Chair.BP_Chair_C|SetDoor _selectchair self))))))

(event EventTick
  (params (DeltaSeconds :type Float%20%28single-precision%29)))

(fn ConstructionScript)