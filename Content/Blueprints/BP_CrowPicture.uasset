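; BP_CrowPicture is a picture prop that starts simulating physics when the first-person character bumps into it, and makes a sound on hard impacts.
; The mesh's component hit event enables physics when the other actor is the player.
; An actor hit event bound at BeginPlay plays an attenuated sound at the impact point above an impulse threshold, with DoOnce and a short delay limiting repeats.
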(event OnComponentHit(StaticMesh)
  (params (HitComponent :type Primitive%20Component%20Object%20Reference) (OtherActor :type Actor%20Object%20Reference) (OtherComp :type Primitive%20Component%20Object%20Reference) (NormalImpulse :type Vector :default "0, 0, 0") (Hit :type Hit%20Result%20Structure%20%28by%20ref%29))
  (Utilities|Casting|CastToFirstPersonCharacter OtherActor)
  (Physics|SetSimulatePhysics (Variables|Default|GetStaticMesh) true))

(event Custom|HitEvent
  (params (SelfActor :type Actor%20Object%20Reference) (OtherActor :type Actor%20Object%20Reference) (NormalImpulse :type Vector) (Hit :type Hit%20Result%20Structure%20%28by%20ref%29))
  (if (> (Math|Vector|VectorLength NormalImpulse) 9e+03)
    (Utilities|FlowControl|DoOnce false :!label _label
      (:Completed
        (Audio|PlaySoundatLocation "/Game/Sounds/hit/hit_cue.hit_cue" (.impactpoint Hit) "0, 0, 0" 1.0 1.0 0.0 "/Game/Sounds/Attenuation/ItemAtten.ItemAtten" 0 0)
        (Utilities|FlowControl|Delay 0.1)
        (goto _label Reset)))))

(event EventBeginPlay
  (Class|PrimitiveComponent|SetNotifyRigidBodyCollision (Variables|Default|GetStaticMesh) true)
  (Collision|BindEventtoOnActorHit (delegate Custom|HitEvent)))

(event Collision|EventActorBeginOverlap
  (params (OtherActor :type Actor%20Object%20Reference)))

(event EventTick
  (params (DeltaSeconds :type Float%20%28single-precision%29)))

(fn ConstructionScript)