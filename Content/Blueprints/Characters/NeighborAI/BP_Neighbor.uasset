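; BP_Neighbor is the AI Neighbor character that detects, chases and catches the player.
; SetState mirrors its state to the Blackboard and sets chase and catch permissions.
; Tick turns sightings into Attack with chase music, times Hunt back to Idle, and toggles a spotlight and meshes by Ultra Dynamic Sky time.
; Overlapping the player triggers Catch when allowed, while events switch movement speeds and AI perception.
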(event OnComponentBeginOverlap(IfCollide)
  (params (OverlappedComponent :type Primitive%20Component%20Object%20Reference) (OtherActor :type Actor%20Object%20Reference) (OtherComp :type Primitive%20Component%20Object%20Reference) (OtherBodyIndex :type Integer) (bFromSweep :type Boolean) (SweepResult :type Hit%20Result%20Structure%20%28by%20ref%29))
  (Utilities|Casting|CastToFirstPersonCharacter OtherActor)
  (if (Variables|Default|GetCanCatch)
    (Variables|Default|SetCanChase false)
    (CallFunction|SetState "NewEnumerator3")))

(event Custom|Walk
  (Variables|/Script/Engine.CharacterMovementComponent|SetMaxWalkSpeed (Variables|Character|GetCharacterMovement) 1.5e+02))

(event Custom|Run
  (Variables|/Script/Engine.CharacterMovementComponent|SetMaxWalkSpeed (Variables|Character|GetCharacterMovement) 4.5e+02))

(event Custom|RunAttack
  (Variables|/Script/Engine.CharacterMovementComponent|SetMaxWalkSpeed (Variables|Character|GetCharacterMovement) 6e+02))

(event Custom|FootstepEvent
  (Audio|Components|Audio|Play (Variables|Default|GetFootsteps) 0.0))

(event Custom|SetSenseEnabled
  (bind _asneighbor_aicontroller (Utilities|Casting|CastToNeighborAIController (AI|GetAIController 0)))
  (Default|SetPerceptionEnabled _asneighbor_aicontroller))

(event Custom|SetSenseDisabled
  (bind _asneighbor_aicontroller (Utilities|Casting|CastToNeighborAIController (AI|GetAIController 0)))
  (Default|SetPerceptionDisabled _asneighbor_aicontroller))

(event EventBeginPlay
  (Audio|Components|Audio|Stop (Variables|Default|Getattack_Cue))
  (bind _asfirst_person_character (Utilities|Casting|CastToFirstPersonCharacter (Game|GetPlayerCharacter 0)))
  (Variables|/Game/Blueprints/Characters/FirstPersonBP/Blueprints/FirstPersonCharacter.FirstPersonCharacter_C|SetCameraActor _asfirst_person_character (Variables|Default|GetCatchCamera)))

(event EventTick
  (params (DeltaSeconds :type Float%20%28single-precision%29))
  (bind _returnvalue (AI|GetBlackboard 0))
  (bind _returnvalue_2 (Game|GetPlayerCharacter 0))
  (bind _attack_cue (Variables|Default|Getattack_Cue))
  (bind _currentstate (Variables|Default|GetCurrentState))
  (bind _arrow1 (Variables|Default|GetArrow1))
  (bind _returnvalue_3 (== _currentstate 1))
  (Utilities|FlowControl|Sequence
    (:then_0
      (bind _asfirst_person_character (Utilities|Casting|CastToFirstPersonCharacter _returnvalue_2))
      (Utilities|IsValid _asfirst_person_character
        (:Is%20Valid
          (Utilities|FlowControl|Sequence
            (:then_0
              (Utilities|FlowControl|DoOnce false
                (:Completed
                  (bind _asfirst_person_character_2 (Utilities|Casting|CastToFirstPersonCharacter _returnvalue_2)))))
            (:then_1
              (Transformation|SetWorldRotation _arrow1 (Math|Rotator|FindLookatRotation (Transformation|GetWorldLocation _arrow1) (Transformation|GetWorldLocation (Variables|/Game/Blueprints/Characters/FirstPersonBP/Blueprints/FirstPersonCharacter.FirstPersonCharacter_C|GetArrow1 _asfirst_person_character_2))) false false))))))
    (:then_1
      (if (not (Utilities|Enum|Equal(Enum) (Variables|Default|GetCurrentState) "NewEnumerator3"))
        (if (ScalableFloat|GetValueasBool _returnvalue (Utilities|Name|MakeLiteralName "CanSeePlayer"))
          (if (not (Variables|Default|GetSleeping))
            (if (Variables|Default|GetCanChase)
              (Utilities|FlowControl|DoOnce false :!label _label
                (:Completed
                  (CallFunction|SetState "NewEnumerator2")
                  (Audio|Components|Audio|Play (Variables|Default|Getattack_Cue) 0.0)
                  (AI|Components|Blackboard|SetValueasBool _returnvalue (Utilities|Name|MakeLiteralName "IsInvestigating") false)
                  (Utilities|FlowControl|Sequence
                    (:then_1
                      (goto _label_2 Reset))))))))))
    (:then_2
      (if (not (== (Variables|Default|GetCurrentState) 2))
        (goto _label Reset)))
    (:then_3
      (if (not (== (Variables|Default|GetCurrentState) 2))
        (if (Audio|Components|Audio|IsPlaying _attack_cue)
          (Utilities|FlowControl|DoOnce false :!label _label_2
            (:Completed
              (Audio|Components|Audio|FadeOut _attack_cue 1.0 0.0 "Linear" :!class /Script/Engine.AudioComponent))))))
    (:then_4
      (if (== (Variables|Default|GetCurrentState) 3)
        (Audio|Components|Audio|Stop (Variables|Default|Getattack_Cue))))
    (:then_6
      (bind _returnvalue_4 (Actor|GetActorOfClass "/Game/UltraDynamicSky/Blueprints/Ultra_Dynamic_Sky.Ultra_Dynamic_Sky_C"))
      (if (not (Math|Float|InRange(Float) (Variables|/Game/UltraDynamicSky/Blueprints/Ultra_Dynamic_Sky.Ultra_Dynamic_Sky_C|GetTime%20of%20Day _returnvalue_4) 1714.285767 2.4e+03))
        (if (Math|Float|InRange(Float) (Variables|/Game/UltraDynamicSky/Blueprints/Ultra_Dynamic_Sky.Ultra_Dynamic_Sky_C|GetTime%20of%20Day _returnvalue_4) 0.0 708.571472)
          (Rendering|SetVisibility (Variables|Default|GetStaticMesh1) true false)
          (else
            (Rendering|SetVisibility (Variables|Default|GetStaticMesh) false false)))))
    (:then_8
      (if _returnvalue_3
        (Utilities|FlowControl|Delay 1.8e+02)
        (if _returnvalue_3
          (CallFunction|SetState "NewEnumerator0"))))))

(fn ConstructionScript)

(fn UpdateHeadRotation
  (bind _returnvalue (Pawn|GetControlRotation :!class /Script/Engine.Pawn))
  (bind _asneighbor_anim_bp (Utilities|Casting|CastToNeighborAnimBP (Components|SkeletalMesh|GetAnimInstance (Variables|Character|GetMesh))))
  (Variables|/Game/Blueprints/Characters/NeighborAI/NeighborAnimBP.NeighborAnimBP_C|SetHeadRotation _asneighbor_anim_bp (Math|Rotator|MakeRotator (- 0.0 (.pitch _returnvalue)) 0.0 (- (.yaw _returnvalue) (.yaw (Pawn|GetControlRotation :!class /Script/Engine.Pawn))))))

(fn SetState
  (params (NewState :type NeighborEnumStates%20Enum :default "NewEnumerator0"))
  (bind _output_get (Variables|Default|SetCurrentState NewState))
  (AI|Components|Blackboard|SetValueasEnum (AI|GetBlackboard 0) (Utilities|Name|MakeLiteralName "State") _output_get)
  (switch Utilities|FlowControl|Switch|SwitchonNeighborEnumStates _output_get
    (:NewEnumerator0
      (Variables|Default|SetCanChase true :!label _label)
      (Variables|Default|SetCanCatch false))
    (:NewEnumerator1
      (goto _label))
    (:NewEnumerator2
      (Variables|Default|SetCanCatch true)
      (Variables|Default|SetCanChase false))))