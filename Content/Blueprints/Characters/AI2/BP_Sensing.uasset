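; Sight-sensing component for AI characters that periodically checks whether its owner can see player 0.
; A looping timer runs a visibility line trace, then tests the hit against sensing range and a forward cone angle, with optional debug cone drawing.
; Paired DoOnce gates report only changes to the AI's SightSense, saving the player's location when sight is lost.
; Debug message printing is disconnected.
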(event Custom|Sense
  (bind _as_ai (Variables|Default|GetAs%20AI))
  (bind _see_target (CallFunction|SenseforTarget))
  (if _see_target
    (Utilities|FlowControl|DoOnce false :!label _label
      (:Completed
        (Default|SightSense _as_ai _see_target)
        (goto _label_2 Reset)))
    (else
      (Utilities|FlowControl|DoOnce false :!label _label_2
        (:Completed
          (Variables|/Game/Blueprints/Characters/AI2/AI.AI_C|SetPlayerLocation _as_ai (Transformation|GetActorLocation (Variables|/Game/Blueprints/Characters/AI2/AI.AI_C|GetPlayer _as_ai)))
          (Default|SightSense _as_ai _see_target)
          (goto _label Reset))))))

(event Custom|Begin%20Sensing
  (bind _returnvalue (Utilities|Time|SetTimerbyEvent (delegate Custom|Sense) (Variables|Togglable|GetSensing%20Interval) true))
  (Variables|Default|SetSensing%20Timer%20Ref _returnvalue))

(event EventBeginPlay
  (Variables|Default|SetTarget (Game|GetPlayerCharacter 0))
  (bind _asai (Utilities|Casting|CastToAI (Components|GetOwner)))
  (Variables|Default|SetAs%20AI _asai)
  (CallFunction|BeginSensing))

(fn SenseforTarget
  (bind _returnvalue (Transformation|GetWorldLocation))
  (bind _returnvalue_2 (Math|Vector|GetForwardVector))
  (bind _target (Variables|Default|GetTarget))
  (bind _cone_angle (Variables|Togglable|GetCone%20Angle))
  (bind _returnvalue_3 (Transformation|GetActorLocation _target))
  (bind _returnvalue_4 (Math|Vector|GetUnitDirection(Vector) _returnvalue _returnvalue_3))
  (bind _returnvalue_5 (Math|Vector|DotProduct _returnvalue_2 _returnvalue_4))
  (bind _returnvalue_6 (Class|KismetMathLibrary|DegAcos _returnvalue_5))
  (LocalVariables|SetCan%20See false)
  (if (Variables|Default|GetDebug)
    (Class|KismetSystemLibrary|DrawDebugConeinDegrees (.location (Transformation|GetWorldTransform)) (Math|Vector|GetForwardVector) (Variables|Togglable|GetSensing%20Range) _cone_angle _cone_angle 12 "(R=1.000000,G=1.000000,B=1.000000,A=1.000000)" (Variables|Togglable|GetSensing%20Interval) 1.0))
  (bind (_outhit _returnvalue_7) (Collision|LineTraceByChannel (Transformation|GetWorldLocation) (Transformation|GetActorLocation (Variables|Default|GetTarget)) "TraceTypeQuery1" false (Utilities|Array|MakeArray (Components|GetOwner)) (Variables|Default|GetTrace%20Debug)))
  (if _returnvalue_7
    (LocalVariables|SetCurrent%20Hit%20Result _outhit)
    (if (== (.hitactor (LocalVariables|GetCurrent%20Hit%20Result)) (Variables|Default|GetTarget))
      (if (<= (.distance (LocalVariables|GetCurrent%20Hit%20Result)) (Variables|Togglable|GetSensing%20Range))
        (if (<= _returnvalue_6 (Variables|Togglable|GetCone%20Angle))
          (bind _output_get (LocalVariables|SetCan%20See true))
          (return _output_get)
          (else
            (CallFunction|DebugMessage (Utilities|String|Append "Target is out of peripheral vision" "Angle =" (Utilities|String|ToString(Float) _returnvalue_6)))
            (bind _output_get_2 (LocalVariables|SetCan%20See false))
            (return _output_get_2)))
        (else
          (CallFunction|DebugMessage "Target is out of range")))
      (else
        (CallFunction|DebugMessage "Sensing is blocked by wall or object")))
    (bind _output_get_3 (LocalVariables|SetCan%20See false))
    (return _output_get_3)
    (else
      (CallFunction|DebugMessage "Couldn't see target")
      (bind _output_get_4 (LocalVariables|SetCan%20See false))
      (return _output_get_4))))

(fn DebugMessage
  (params (InString :type String)))