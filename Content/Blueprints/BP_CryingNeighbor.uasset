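; BP_CryingNeighbor is a one-shot trigger actor that stages a brief scare when the player reaches it.
; The first FirstPersonCharacter overlap of its Box plays a reverb guest sound and the W_WhiteFlash widget's flash animation.
; After a short delay the actor destroys itself.
; The widget's RemoveFromParent sits behind another delay after DestroyActor, so it depends on a latent action of a destroyed actor.
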(event OnComponentBeginOverlap(Box)
  (params (OverlappedComponent :type Primitive%20Component%20Object%20Reference) (OtherActor :type Actor%20Object%20Reference) (OtherComp :type Primitive%20Component%20Object%20Reference) (OtherBodyIndex :type Integer) (bFromSweep :type Boolean) (SweepResult :type Hit%20Result%20Structure%20%28by%20ref%29))
  (Utilities|Casting|CastToFirstPersonCharacter OtherActor)
  (Utilities|FlowControl|DoOnce false
    (:Completed
      (Audio|PlaySound2D "/Game/Sounds/sequences/guest_reverb_Cue.guest_reverb_Cue" 1.0 1.0 0.0 0 0)
      (bind _returnvalue (UserInterface|CreateWidget "/Game/Blueprints/UI/W_WhiteFlash.W_WhiteFlash_C" (Game|GetPlayerController 0)))
      (UserInterface|Viewport|AddtoViewport _returnvalue 0)
      (UserInterface|Animation|PlayAnimation _returnvalue (Variables|/Game/Blueprints/UI/W_WhiteFlash.W_WhiteFlash_C|GetFlash _returnvalue) 0.0 1 "Forward" 1.0 false)
      (Utilities|FlowControl|Delay 0.35)
      (Actor|DestroyActor)
      (Utilities|FlowControl|Delay 0.15)
      (Widget|RemovefromParent _returnvalue))))

(event EventBeginPlay)

(event Collision|EventActorBeginOverlap
  (params (OtherActor :type Actor%20Object%20Reference)))

(event EventTick
  (params (DeltaSeconds :type Float%20%28single-precision%29)))

(fn ConstructionScript)