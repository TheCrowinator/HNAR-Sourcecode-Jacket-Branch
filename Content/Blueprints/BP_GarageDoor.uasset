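; Garage door actor that swings and slides its static mesh between open and closed when its Open or Close event is called.
; Each event plays a sound at the actor, sets IsOpen and starts one of two timed MoveComponentTo moves while stopping the opposite one, so the door can reverse mid-motion.
; Intermediate half-rotated move steps remain in the graph but never run.
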(event Custom|Open
  (Audio|PlaySoundatLocation "/Game/Sounds/garage_door_open.garage_door_open" (Transformation|GetActorLocation) "0, 0, 0" 1.0 1.0 0.0 0 0 0)
  (Variables|Default|SetIsOpen? true)
  (Utilities|FlowControl|Sequence
    (:then_0
      (Components|MoveComponentTo (Variables|Default|GetStaticMesh) "0,0.000000,-10.000000" "0, 0,-90.000000" false false 4.5 true))
    (:then_1
      (Components|MoveComponentTo (Variables|Default|GetStaticMesh) "0, 0,-270.000000" "0, 0, 0" false false 4.0 true) ; enters at Stop
    )))

(event Custom|Close
  (Audio|PlaySoundatLocation "/Game/Sounds/garage_door_close_Cue.garage_door_close_Cue" (Transformation|GetActorLocation) "0, 0, 0" 1.0 1.0 0.0 0 0 0)
  (Variables|Default|SetIsOpen? false)
  (Utilities|FlowControl|Sequence
    (:then_0
      (Components|MoveComponentTo (Variables|Default|GetStaticMesh) "0, 0,-270.000000" "0, 0, 0" false false 4.0 true))
    (:then_1
      (Components|MoveComponentTo (Variables|Default|GetStaticMesh) "0,0.000000,-10.000000" "0, 0,-90.000000" false false 4.5 true) ; enters at Stop
    )))

(event EventBeginPlay)

(event Collision|EventActorBeginOverlap
  (params (OtherActor :type Actor%20Object%20Reference)))

(event EventTick
  (params (DeltaSeconds :type Float%20%28single-precision%29)))

(fn ConstructionScript)