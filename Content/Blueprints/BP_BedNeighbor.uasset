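; A bed the player can hide under, toggled by the Hiding event, which teleports the player and view between two arrow points.
; Hiding and GoOutOfHiding update movement, player hiding flags, and the neighbor AI's chase flag and blackboard key.
; An under-bed search with look and catch animations exists but is disconnected, leaving Tick's sight check without effect.
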(event Custom|Hiding
  (bind _returnvalue (Utilities|Name|MakeLiteralName "PlayerHidingUnderBed"))
  (bind _returnvalue_2 (Game|GetPlayerController 0))
  (bind _ai (Variables|Default|GetAI))
  (bind _arrow2 (Variables|Default|GetArrow2))
  (bind _returnvalue_3 (AI|GetBlackboard _ai))
  (bind _asfirst_person_character (Utilities|Casting|CastToFirstPersonCharacter (Game|GetPlayerCharacter 0)))
  (if (Variables|/Script/Engine.Character|GetbIsCrouched _asfirst_person_character)
    (Character|UnCrouch _asfirst_person_character)
    (Utilities|FlowControl|Delay 0.1))
  (if (not (Variables|Default|GetNeighborGonnaSearch))
    (if (Variables|/Game/Blueprints/Characters/FirstPersonBP/Blueprints/FirstPersonCharacter.FirstPersonCharacter_C|GetHidingUnderBed? _asfirst_person_character)
      (Transformation|SetActorLocation _asfirst_person_character (Transformation|GetWorldLocation _arrow2) false false)
      (Pawn|SetControlRotation _returnvalue_2 (Transformation|GetWorldRotation _arrow2))
      (Pawn|Components|CharacterMovement|SetMovementMode (Variables|/Script/Engine.Character|GetCharacterMovement _asfirst_person_character) "MOVE_Walking" 0)
      (bind _output_get (Variables|/Game/Blueprints/Characters/FirstPersonBP/Blueprints/FirstPersonCharacter.FirstPersonCharacter_C|SetHidingUnderBed? _asfirst_person_character false))
      (Variables|/Game/Blueprints/Characters/FirstPersonBP/Blueprints/FirstPersonCharacter.FirstPersonCharacter_C|SetIsHiding? _asfirst_person_character _output_get)
      (if (not (Variables|/Game/Blueprints/Characters/AI2/AI.AI_C|GetIsSleeping _ai))
        (Variables|/Game/Blueprints/Characters/AI2/AI.AI_C|SetCanChase _ai true)
        (AI|Components|Blackboard|SetValueasBool _returnvalue_3 _returnvalue _output_get))
      (else
        (Pawn|Components|CharacterMovement|SetMovementMode (Variables|/Script/Engine.Character|GetCharacterMovement _asfirst_person_character) "MOVE_None" 0)
        (Transformation|SetActorLocation _asfirst_person_character (Transformation|GetWorldLocation (Variables|Default|GetArrow1)) false false)
        (Pawn|SetControlRotation _returnvalue_2 (Transformation|GetWorldRotation (Variables|Default|GetArrow1)))
        (bind _output_get_2 (Variables|/Game/Blueprints/Characters/FirstPersonBP/Blueprints/FirstPersonCharacter.FirstPersonCharacter_C|SetHidingUnderBed? _asfirst_person_character true))
        (Variables|/Game/Blueprints/Characters/FirstPersonBP/Blueprints/FirstPersonCharacter.FirstPersonCharacter_C|SetIsHiding? _asfirst_person_character _output_get_2)
        (Variables|/Game/Blueprints/Characters/AI2/AI.AI_C|SetCanChase _ai false)
        (AI|Components|Blackboard|SetValueasBool _returnvalue_3 _returnvalue _output_get_2)
        (bind _output_get_3 (Variables|/Game/Blueprints/Characters/FirstPersonBP/Blueprints/FirstPersonCharacter.FirstPersonCharacter_C|SetHidingBed _asfirst_person_character self))
        (Variables|/Game/Blueprints/Characters/AI2/AI.AI_C|SetHidingBed (Variables|Default|GetAI) _output_get_3)
        (Math|Integer|IncrementInt (Variables|Default|GetHideCount))))))

(event Custom|GoOutOfHiding
  (bind _ai (Variables|Default|GetAI))
  (Pawn|Components|CharacterMovement|SetMovementMode (Variables|/Script/Engine.Character|GetCharacterMovement (stale Custom|Hiding _asfirst_person_character)) "MOVE_Walking" 0)
  (bind _output_get (Variables|/Game/Blueprints/Characters/FirstPersonBP/Blueprints/FirstPersonCharacter.FirstPersonCharacter_C|SetHidingUnderBed? (stale Custom|Hiding _asfirst_person_character) false))
  (Variables|/Game/Blueprints/Characters/FirstPersonBP/Blueprints/FirstPersonCharacter.FirstPersonCharacter_C|SetIsHiding? (stale Custom|Hiding _asfirst_person_character) _output_get)
  (if (not (Variables|/Game/Blueprints/Characters/AI2/AI.AI_C|GetIsSleeping _ai))
    (Variables|/Game/Blueprints/Characters/AI2/AI.AI_C|SetCanChase _ai true)
    (AI|Components|Blackboard|SetValueasBool (AI|GetBlackboard _ai) (Utilities|Name|MakeLiteralName "PlayerHidingUnderBed") _output_get)))

(event EventBeginPlay)

(event Collision|EventActorBeginOverlap
  (params (OtherActor :type Actor%20Object%20Reference)))

(event EventTick
  (params (DeltaSeconds :type Float%20%28single-precision%29))
  (bind _ai (Variables|Default|GetAI))
  (Utilities|FlowControl|Sequence
    (:then_0
      (Utilities|IsValid _ai
        (:Is%20Valid
          (if (Utilities|Enum|Equal(Enum) (Variables|/Game/Blueprints/Characters/AI2/AI.AI_C|GetCurrentState _ai) "NewEnumerator4")
            (if (Variables|/Game/Blueprints/Characters/AI2/AI.AI_C|GetCanSeePlayer _ai)
              (bind _asfirst_person_character (Utilities|Casting|CastToFirstPersonCharacter (Game|GetPlayerCharacter 0)))
              (if (Variables|/Game/Blueprints/Characters/FirstPersonBP/Blueprints/FirstPersonCharacter.FirstPersonCharacter_C|GetHidingUnderBed? _asfirst_person_character)
                _))))))))

(fn ConstructionScript)

(fn MoveUnderBed)