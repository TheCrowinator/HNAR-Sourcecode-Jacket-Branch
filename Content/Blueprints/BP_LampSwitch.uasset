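; A wall light switch that the player toggles to turn linked lamps and sconces on or off.
; Interact on the switch mesh flips the On state, plays a click sound, tilts the mesh with MoveComponentTo and calls SwitchOn or SwitchOff on both connected arrays.
; BeginPlay runs the same switch-off path, sound included, when On starts false; a true start state is not pushed to the lights.
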(event Custom|Interact
  (params (Component :type Primitive%20Component%20Object%20Reference))
  (bind _returnvalue (Transformation|GetActorLocation))
  (bind _staticmesh1 (Variables|Default|GetStaticMesh1))
  (if (== _staticmesh1 Component)
    (if (Variables|Default|GetOn?)
      (Audio|PlaySoundatLocation "/Game/Sounds/light_switch_turn_off_Cue.light_switch_turn_off_Cue" _returnvalue "0, 0, 0" 1.0 1.0 0.0 0 0 0)
      (Components|MoveComponentTo _staticmesh1 "0,0.900000, 0" "0, 0,5.000000" false false 0.1 false)
      (Variables|Default|SetOn? false)
      (Utilities|FlowControl|Sequence
        (:then_0
          (for _array_element (Variables|Default|GetConnected%20Lamp)
            (Default|SwitchOff _array_element)))
        (:then_1
          (for _array_element_2 (Variables|Default|GetConnected%20Sconce)
            (Default|SwitchOff _array_element_2))))
      (else
        (Audio|PlaySoundatLocation "/Game/Sounds/light_switch_turn_on_Cue.light_switch_turn_on_Cue" _returnvalue "0, 0, 0" 1.0 1.0 0.0 0 0 0)
        (Components|MoveComponentTo _staticmesh1 "0,0.900000, 0" "0, 0,-5.000000" false false 0.1 false)
        (Variables|Default|SetOn? true)
        (Utilities|FlowControl|Sequence
          (:then_0
            (for _array_element_3 (Variables|Default|GetConnected%20Lamp)
              (Default|Switchon _array_element_3)))
          (:then_1
            (for _array_element_4 (Variables|Default|GetConnected%20Sconce)
              (Default|Switchon _array_element_4))))))))

(event EventBeginPlay
  (if (not (Variables|Default|GetOn?))
    (Audio|PlaySoundatLocation "/Game/Sounds/light_switch_turn_off_Cue.light_switch_turn_off_Cue" (Transformation|GetActorLocation) "0, 0, 0" 1.0 1.0 0.0 0 0 0)
    (Components|MoveComponentTo (Variables|Default|GetStaticMesh1) "0,0.900000, 0" "0, 0,5.000000" false false 0.1 false)
    (Variables|Default|SetOn? false)
    (Utilities|FlowControl|Sequence
      (:then_0
        (for _array_element (Variables|Default|GetConnected%20Lamp)
          (Default|SwitchOff _array_element)))
      (:then_1
        (for _array_element_2 (Variables|Default|GetConnected%20Sconce)
          (Default|SwitchOff _array_element_2))))))

(fn ConstructionScript)