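; Hanging lamp actor that switches its point light and bulb material on or off through custom switch events.
; BeginPlay applies the OnOff state and starts a looping timer on Tick, where random Delays pace the light changes.
; While powered and on, Flicker randomly blacks out or restores light and bulb; otherwise intensity wavers subtly.
; ForceSwitchOff darkens the lamp regardless of PowerOn, leaving OnOff unchanged.
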(event Custom|Tick
  (bind _pointlight_0 (Variables|Default|GetPointLight_0))
  (bind _staticmesh1 (Variables|Default|GetStaticMesh1))
  (if (and (Variables|Default|GetPowerOn?) (Variables|Default|GetOn/Off))
    (if (Variables|Default|GetFlicker?)
      (Utilities|FlowControl|Delay (Math|Random|RandomFloatinRange 0.1 1.5))
      (if (== (Math|Random|RandomIntegerinRange 0 1) 1)
        (Rendering|Components|Light|SetIntensity _pointlight_0 (Math|Float|MakeLiteralFloat 0.0))
        (Rendering|Material|SetMaterial _staticmesh1 0 "/Game/StarterContent/Materials/M_Glass.M_Glass")
        (else
          (Rendering|Components|Light|SetIntensity _pointlight_0 (Math|Float|MakeLiteralFloat 5e+03))
          (Rendering|Material|SetMaterial _staticmesh1 0 (Variables|Default|GetBulbTexture))))
      (else
        (Utilities|FlowControl|Delay (Math|Random|RandomFloatinRange 0.1 0.5))
        (Rendering|Components|Light|SetIntensity (Variables|Default|GetPointLight_0) (Math|Random|RandomFloatinRange 4e+03 5.5e+03))))))

(event EventBeginPlay
  (bind _staticmesh1 (Variables|Default|GetStaticMesh1))
  (bind _pointlight_0 (Variables|Default|GetPointLight_0))
  (Utilities|FlowControl|Sequence
    (:then_0
      (if (Variables|Default|GetOn/Off)
        (Rendering|Material|SetMaterial _staticmesh1 0 (Variables|Default|GetBulbTexture))
        (Rendering|SetVisibility _pointlight_0 true false)
        (else
          (Rendering|Material|SetMaterial _staticmesh1 0 "/Game/StarterContent/Materials/M_Glass.M_Glass")
          (Rendering|SetVisibility _pointlight_0 false false))))
    (:then_1
      (Utilities|Time|SetTimerbyEvent (delegate Custom|Tick) 0.01 true))))

(event EventSwitchon
  (Variables|Default|SetOn/Off true)
  (if (Variables|Default|GetPowerOn?)
    (Rendering|Material|SetMaterial (Variables|Default|GetStaticMesh1) 0 (Variables|Default|GetBulbTexture))
    (Rendering|SetVisibility (Variables|Default|GetPointLight_0) true false)))

(event EventSwitchOff
  (Variables|Default|SetOn/Off false)
  (if (Variables|Default|GetPowerOn?)
    (Rendering|Material|SetMaterial (Variables|Default|GetStaticMesh1) 0 "/Game/StarterContent/Materials/M_Glass.M_Glass")
    (Rendering|SetVisibility (Variables|Default|GetPointLight_0) false false)))

(event EventForceSwitchOff
  (Rendering|Material|SetMaterial (Variables|Default|GetStaticMesh1) 0 "/Game/StarterContent/Materials/M_Glass.M_Glass")
  (Rendering|SetVisibility (Variables|Default|GetPointLight_0) false false))

(fn ConstructionScript
  (|CallParentFunction))