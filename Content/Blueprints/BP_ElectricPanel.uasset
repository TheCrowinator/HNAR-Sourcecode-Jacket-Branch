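; Electric panel actor with a hinged door and a breaker switch, both toggled through OpenClose based on the passed component.
; Paired MoveComponentTo nodes animate each part, stopping the opposite move and playing sounds; when locked, either part only plays a locked sound.
; Switching the breaker on starts a generator sound, stopped once switched off.
; PowerOn, also called at BeginPlay if PowerWorking, runs the switch-on path, bypassing the lock.
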(event Custom|PowerOn
  (bind _door1 (Variables|Default|GetDoor1))
  (bind _returnvalue (Transformation|GetWorldLocation _door1))
  (Utilities|FlowControl|Sequence
    (:then_0
      (Components|MoveComponentTo _door1 "0.000000,7.000000,25.500000" "0,0.000000,170.000000" false false 0.3 false)
      (Variables|Default|SetOpen_1 true)
      (bind _returnvalue_2 (Audio|SpawnSoundatLocation "/Game/Sounds/generator_working.generator_working" _returnvalue "0, 0, 0" 1.0 1.0 0.0 "/Game/Sounds/Attenuation/PowerAt.PowerAt" 0)))
    (:then_1
      (Components|MoveComponentTo _door1 "0.000000,7.000000,25.500000" "0, 0, 0" false false 0.3 false) ; enters at Stop
    )
    (:then_2
      (Audio|SpawnSoundatLocation "/Game/Sounds/switch_circuit_breaker_on.switch_circuit_breaker_on" (Transformation|GetWorldLocation (Variables|Default|GetDoor1)) "0, 0, 0" 1.0 1.0 0.0 "/Game/Sounds/Attenuation/DoorSoundAttenuation.DoorSoundAttenuation" 0))))

(event EventBeginPlay
  (if (Variables|Default|GetPowerWorking?)
    (CallFunction|Poweron)))

(event EventOpenClose
  (params (Component :type Primitive%20Component%20Object%20Reference))
  (bind _door1 (Variables|Default|GetDoor1))
  (bind _door1_2 (Variables|Default|GetDoor1))
  (bind _door (Variables|Default|GetDoor))
  (bind _returnvalue (Transformation|GetWorldLocation _door1_2))
  (if (== Component (Variables|Default|GetDoor))
    (if (Variables|Default|GetLocked)
      (Audio|PlaySoundatLocation "/Game/Sounds/LockedDoor_Cue.LockedDoor_Cue" (Transformation|GetWorldLocation _door) "0, 0, 0" 1.0 1.0 0.0 "/Game/Sounds/Attenuation/DoorSoundAttenuation.DoorSoundAttenuation" 0 0 :!label _label)
      (elif (Variables|Default|GetOpen)
        (Utilities|FlowControl|Sequence
          (:then_0
            (Variables|Default|SetOpen false)
            (Components|MoveComponentTo _door "-19.000000,11.200000,1.900000" "0, 0, 0" false false 0.5 false :!label _label_2)
            (Audio|SpawnSoundatLocation (Variables|Default|GetCloseSound) (Transformation|GetWorldLocation _door) "0, 0, 0" 1.0 1.0 0.0 "/Game/Sounds/Attenuation/DoorSoundAttenuation.DoorSoundAttenuation" 0))
          (:then_1
            (goto _label_3 Stop)))
        (else
          (Utilities|FlowControl|Sequence
            (:then_0
              (Variables|Default|SetOpen true)
              (Components|MoveComponentTo _door "-19.000000,11.200000,1.900000" "0,145.000000,0.000000" false false 0.5 false :!label _label_3))
            (:then_1
              (goto _label_2 Stop))
            (:then_2
              (Audio|SpawnSoundatLocation (Variables|Default|GetOpenSound) (Transformation|GetWorldLocation _door) "0, 0, 0" 1.0 1.0 0.0 "/Game/Sounds/Attenuation/DoorSoundAttenuation.DoorSoundAttenuation" 0))))))
    (elif (== Component _door1)
      (if (Variables|Default|GetLocked)
        (goto _label)
        (elif (Variables|Default|GetOpen_1)
          (Utilities|FlowControl|Sequence
            (:then_0
              (Components|MoveComponentTo _door1_2 "0.000000,7.000000,25.500000" "0, 0, 0" false false 0.3 false :!label _label_4)
              (Variables|Default|SetOpen_1 false)
              (Audio|SpawnSoundatLocation "/Game/Sounds/switch_circuit_breaker_off.switch_circuit_breaker_off" _returnvalue "0, 0, 0" 1.0 1.0 0.0 "/Game/Sounds/Attenuation/DoorSoundAttenuation.DoorSoundAttenuation" 0)
              (Audio|Components|Audio|Stop (stale _returnvalue_2)))
            (:then_1
              (goto _label_5 Stop)))
          (else
            (Utilities|FlowControl|Sequence
              (:then_0
                (Components|MoveComponentTo _door1_2 "0.000000,7.000000,25.500000" "0,0.000000,170.000000" false false 0.3 false :!label _label_5)
                (Variables|Default|SetOpen_1 true)
                (bind _returnvalue_2 (Audio|SpawnSoundatLocation "/Game/Sounds/generator_working.generator_working" _returnvalue "0, 0, 0" 1.0 1.0 0.0 "/Game/Sounds/Attenuation/PowerAt.PowerAt" 0)))
              (:then_1
                (goto _label_4 Stop))
              (:then_2
                (Audio|SpawnSoundatLocation "/Game/Sounds/switch_circuit_breaker_on.switch_circuit_breaker_on" (Transformation|GetWorldLocation _door1) "0, 0, 0" 1.0 1.0 0.0 "/Game/Sounds/Attenuation/DoorSoundAttenuation.DoorSoundAttenuation" 0)))))))))

(fn ConstructionScript
  (|CallParentFunction))