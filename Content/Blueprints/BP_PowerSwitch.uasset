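; Breaker box with a lockable door and an animated switch that cuts or restores power to linked lamps, sconces and a lift.
; OpenClose animates the door or toggles the switch, whose move completion applies the power state.
; Power loss closes open lattices but keeps their IsOpen flag so restoration reopens them.
; If IsNeighbors, cutting power also reports noise and sets the switch as the AI's blackboard ObjectRef.
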(event Custom|PowerOff
  (bind _lift (Variables|Default|GetLift))
  (bind _door1 (Variables|Default|GetDoor1))
  (bind _lift_2 (Variables|Default|GetLift))
  (bind _lattice (Variables|Default|GetLattice))
  (bind _lattice_2 (Variables|Default|GetLattice))
  (bind _lamps (Variables|Default|GetLamps))
  (bind _ai_0 (Variables|Default|GetAI_0))
  (bind _sconce (Variables|Default|GetSconce))
  (bind _returnvalue (Transformation|GetWorldLocation _door1))
  (Utilities|FlowControl|Sequence
    (:then_0
      (Components|MoveComponentTo _door1 "0.000000,7.000000,25.500000" "0,0.000000,170.000000" false false 0.3 false)
      (Variables|Default|SetPowerWorking? false)
      (Audio|SpawnSoundatLocation "/Game/Sounds/power_down.power_down" _returnvalue "0, 0, 0" 1.0 1.0 0.0 "/Game/Sounds/Attenuation/DoorSoundAttenuation.DoorSoundAttenuation" 0)
      (Utilities|FlowControl|Sequence
        (:then_0
          (for _array_element _lamps
            (Variables|/Game/Blueprints/BP_LampHolder.BP_LampHolder_C|SetPowerOn? _array_element false)
            (if (Variables|/Game/Blueprints/BP_LampHolder.BP_LampHolder_C|GetOn/Off _array_element)
              (Default|ForceSwitchOff _array_element))))
        (:then_1
          (Utilities|IsValid (Utilities|Array|Get(acopy) _sconce)
            (:Is%20Valid
              (for _array_element_2 _sconce
                (Variables|/Game/Blueprints/BP_Sconce.BP_Sconce_C|SetPowerOn? _array_element_2 false)
                (if (Variables|/Game/Blueprints/BP_Sconce.BP_Sconce_C|GetOn/Off _array_element_2)
                  (Default|ForceSwitchOff _array_element_2))))))
        (:then_2
          (Utilities|IsValid _ai_0
            (:Is%20Valid
              (if (Variables|Default|GetIsNeighbor's)
                (Class|AISenseHearing|ReportNoiseEvent (Transformation|GetWorldLocation (Variables|Default|GetArrow)) 1e+02 self 1e+04 "Power")
                (AI|Components|Blackboard|SetValueasObject (AI|GetBlackboard _ai_0) (Utilities|Name|MakeLiteralName "ObjectRef") self)))))
        (:then_3
          (Utilities|IsValid _lift
            (:Is%20Valid
              (Variables|/Game/Blueprints/Lift/BP_Lift.BP_Lift_C|SetPowered? _lift false)
              (Utilities|IsValid (Utilities|Array|Get(acopy) _lattice)
                (:Is%20Valid
                  (for _array_element_3 _lattice
                    (if (Variables|/Game/Blueprints/BP_Lattice.BP_Lattice_C|GetIsOpen _array_element_3)
                      (Default|Close _array_element_3)
                      (Utilities|FlowControl|Delay 0.1)
                      (Variables|/Game/Blueprints/BP_Lattice.BP_Lattice_C|SetIsOpen _array_element_3 true))))))))))
    (:then_1
      (Components|MoveComponentTo _door1 "0.000000,7.000000,25.500000" "0, 0, 0" false false 0.3 false) ; enters at Stop
    )
    (:then_2
      (Audio|SpawnSoundatLocation "/Game/Sounds/switch_circuit_breaker_on.switch_circuit_breaker_on" (Transformation|GetWorldLocation (Variables|Default|GetDoor1)) "0, 0, 0" 1.0 1.0 0.0 "/Game/Sounds/Attenuation/DoorSoundAttenuation.DoorSoundAttenuation" 0))))

(event Custom|PowerOnOff
  (bind _lift (Variables|Default|GetLift))
  (bind _door1 (Variables|Default|GetDoor1))
  (bind _lift_2 (Variables|Default|GetLift))
  (bind _lattice (Variables|Default|GetLattice))
  (bind _lattice_2 (Variables|Default|GetLattice))
  (bind _lamps (Variables|Default|GetLamps))
  (bind _ai_0 (Variables|Default|GetAI_0))
  (bind _sconce (Variables|Default|GetSconce))
  (bind _returnvalue (Transformation|GetWorldLocation _door1))
  (if (Variables|Default|GetPowerWorking?)
    (Utilities|FlowControl|Sequence
      (:then_0
        (Components|MoveComponentTo _door1 "0.000000,7.000000,25.500000" "0,0.000000,170.000000" false false 0.3 false :!label _label)
        (Variables|Default|SetPowerWorking? false)
        (Audio|SpawnSoundatLocation "/Game/Sounds/power_down.power_down" _returnvalue "0, 0, 0" 1.0 1.0 0.0 "/Game/Sounds/Attenuation/DoorSoundAttenuation.DoorSoundAttenuation" 0)
        (Utilities|FlowControl|Sequence
          (:then_0
            (for _array_element _lamps
              (Variables|/Game/Blueprints/BP_LampHolder.BP_LampHolder_C|SetPowerOn? _array_element false)
              (if (Variables|/Game/Blueprints/BP_LampHolder.BP_LampHolder_C|GetOn/Off _array_element)
                (Default|ForceSwitchOff _array_element))))
          (:then_1
            (Utilities|IsValid (Utilities|Array|Get(acopy) _sconce)
              (:Is%20Valid
                (for _array_element_2 _sconce
                  (Variables|/Game/Blueprints/BP_Sconce.BP_Sconce_C|SetPowerOn? _array_element_2 false)
                  (if (Variables|/Game/Blueprints/BP_Sconce.BP_Sconce_C|GetOn/Off _array_element_2)
                    (Default|ForceSwitchOff _array_element_2))))))
          (:then_2
            (Utilities|IsValid _ai_0
              (:Is%20Valid
                (if (Variables|Default|GetIsNeighbor's)
                  (Class|AISenseHearing|ReportNoiseEvent (Transformation|GetWorldLocation (Variables|Default|GetArrow)) 1e+02 self 1e+04 "Power")
                  (AI|Components|Blackboard|SetValueasObject (AI|GetBlackboard _ai_0) (Utilities|Name|MakeLiteralName "ObjectRef") self)))))
          (:then_3
            (Utilities|IsValid _lift
              (:Is%20Valid
                (Variables|/Game/Blueprints/Lift/BP_Lift.BP_Lift_C|SetPowered? _lift false)
                (Utilities|IsValid (Utilities|Array|Get(acopy) _lattice)
                  (:Is%20Valid
                    (for _array_element_3 _lattice
                      (if (Variables|/Game/Blueprints/BP_Lattice.BP_Lattice_C|GetIsOpen _array_element_3)
                        (Default|Close _array_element_3)
                        (Utilities|FlowControl|Delay 0.1)
                        (Variables|/Game/Blueprints/BP_Lattice.BP_Lattice_C|SetIsOpen _array_element_3 true))))))))))
      (:then_1
        (goto _label_2 Stop))
      (:then_2
        (Audio|SpawnSoundatLocation "/Game/Sounds/switch_circuit_breaker_on.switch_circuit_breaker_on" (Transformation|GetWorldLocation (Variables|Default|GetDoor1)) "0, 0, 0" 1.0 1.0 0.0 "/Game/Sounds/Attenuation/DoorSoundAttenuation.DoorSoundAttenuation" 0)))
    (else
      (Utilities|FlowControl|Sequence
        (:then_0
          (Components|MoveComponentTo _door1 "0.000000,7.000000,25.500000" "0, 0, 0" false false 0.3 false :!label _label_2)
          (Variables|Default|SetPowerWorking? true)
          (Audio|SpawnSoundatLocation "/Game/Sounds/switch_circuit_breaker_off.switch_circuit_breaker_off" _returnvalue "0, 0, 0" 1.0 1.0 0.0 "/Game/Sounds/Attenuation/DoorSoundAttenuation.DoorSoundAttenuation" 0)
          (Utilities|FlowControl|Sequence
            (:then_0
              (for _array_element_4 _lamps
                (Variables|/Game/Blueprints/BP_LampHolder.BP_LampHolder_C|SetPowerOn? _array_element_4 true)
                (if (Variables|/Game/Blueprints/BP_LampHolder.BP_LampHolder_C|GetOn/Off _array_element_4)
                  (Default|Switchon _array_element_4))))
            (:then_1
              (Utilities|IsValid (Utilities|Array|Get(acopy) _sconce)
                (:Is%20Valid
                  (for _array_element_5 _sconce
                    (Variables|/Game/Blueprints/BP_Sconce.BP_Sconce_C|SetPowerOn? _array_element_5 true)
                    (if (Variables|/Game/Blueprints/BP_Sconce.BP_Sconce_C|GetOn/Off _array_element_5)
                      (Default|Switchon _array_element_5))))))
            (:then_2
              (Utilities|IsValid _lift_2
                (:Is%20Valid
                  (Variables|/Game/Blueprints/Lift/BP_Lift.BP_Lift_C|SetPowered? _lift_2 true)
                  (Utilities|IsValid (Utilities|Array|Get(acopy) _lattice_2)
                    (:Is%20Valid
                      (for _array_element_6 _lattice_2
                        (if (Variables|/Game/Blueprints/BP_Lattice.BP_Lattice_C|GetIsOpen _array_element_6)
                          (Default|Open _array_element_6))))))))))
        (:then_1
          (goto _label Stop))))))

(event EventBeginPlay
  (if (not (Variables|Default|GetPowerWorking?))
    (CallFunction|PowerOff)))

(event EventOpenClose
  (params (Component :type Primitive%20Component%20Object%20Reference))
  (bind _door1 (Variables|Default|GetDoor1))
  (bind _lift (Variables|Default|GetLift))
  (bind _door1_2 (Variables|Default|GetDoor1))
  (bind _lift_2 (Variables|Default|GetLift))
  (bind _lattice (Variables|Default|GetLattice))
  (bind _lattice_2 (Variables|Default|GetLattice))
  (bind _door (Variables|Default|GetDoor))
  (bind _lamps (Variables|Default|GetLamps))
  (bind _ai_0 (Variables|Default|GetAI_0))
  (bind _sconce (Variables|Default|GetSconce))
  (bind _returnvalue (Transformation|GetWorldLocation _door1_2))
  (if (== Component (Variables|Default|GetDoor))
    (if (Variables|Default|GetLocked)
      (Audio|PlaySoundatLocation "/Game/Sounds/LockedDoor_Cue.LockedDoor_Cue" (Transformation|GetWorldLocation _door) "0, 0, 0" 1.0 1.0 0.0 "/Game/Sounds/Attenuation/DoorSoundAttenuation.DoorSoundAttenuation" 0 0)
      (elif (Variables|Default|GetOpen)
        (Utilities|FlowControl|Sequence
          (:then_0
            (Variables|Default|SetOpen false)
            (Components|MoveComponentTo _door "-19.000000,11.200000,1.900000" "0, 0, 0" false false 0.5 false :!label _label)
            (Audio|SpawnSoundatLocation (Variables|Default|GetCloseSound) (Transformation|GetWorldLocation _door) "0, 0, 0" 1.0 1.0 0.0 "/Game/Sounds/Attenuation/DoorSoundAttenuation.DoorSoundAttenuation" 0))
          (:then_1
            (goto _label_2 Stop)))
        (else
          (Utilities|FlowControl|Sequence
            (:then_0
              (Variables|Default|SetOpen true)
              (Components|MoveComponentTo _door "-19.000000,11.200000,1.900000" "0,145.000000,0.000000" false false 0.5 false :!label _label_2))
            (:then_1
              (goto _label Stop))
            (:then_2
              (Audio|SpawnSoundatLocation (Variables|Default|GetOpenSound) (Transformation|GetWorldLocation _door) "0, 0, 0" 1.0 1.0 0.0 "/Game/Sounds/Attenuation/DoorSoundAttenuation.DoorSoundAttenuation" 0))))))
    (elif (== Component _door1)
      (if (Variables|Default|GetPowerWorking?)
        (Utilities|FlowControl|Sequence
          (:then_0
            (Components|MoveComponentTo _door1_2 "0.000000,7.000000,25.500000" "0,0.000000,170.000000" false false 0.3 false :!label _label_3)
            (Variables|Default|SetPowerWorking? false)
            (Audio|SpawnSoundatLocation "/Game/Sounds/power_down.power_down" _returnvalue "0, 0, 0" 1.0 1.0 0.0 "/Game/Sounds/Attenuation/DoorSoundAttenuation.DoorSoundAttenuation" 0)
            (Utilities|FlowControl|Sequence
              (:then_0
                (for _array_element _lamps
                  (Variables|/Game/Blueprints/BP_LampHolder.BP_LampHolder_C|SetPowerOn? _array_element false)
                  (if (Variables|/Game/Blueprints/BP_LampHolder.BP_LampHolder_C|GetOn/Off _array_element)
                    (Default|ForceSwitchOff _array_element))))
              (:then_1
                (Utilities|IsValid (Utilities|Array|Get(acopy) _sconce)
                  (:Is%20Valid
                    (for _array_element_2 _sconce
                      (Variables|/Game/Blueprints/BP_Sconce.BP_Sconce_C|SetPowerOn? _array_element_2 false)
                      (if (Variables|/Game/Blueprints/BP_Sconce.BP_Sconce_C|GetOn/Off _array_element_2)
                        (Default|ForceSwitchOff _array_element_2))))))
              (:then_2
                (Utilities|IsValid _ai_0
                  (:Is%20Valid
                    (if (Variables|Default|GetIsNeighbor's)
                      (Class|AISenseHearing|ReportNoiseEvent (Transformation|GetWorldLocation (Variables|Default|GetArrow)) 1e+02 self 1e+04 "Power")
                      (AI|Components|Blackboard|SetValueasObject (AI|GetBlackboard _ai_0) (Utilities|Name|MakeLiteralName "ObjectRef") self)))))
              (:then_3
                (Utilities|IsValid _lift
                  (:Is%20Valid
                    (Variables|/Game/Blueprints/Lift/BP_Lift.BP_Lift_C|SetPowered? _lift false)
                    (Utilities|IsValid (Utilities|Array|Get(acopy) _lattice)
                      (:Is%20Valid
                        (for _array_element_3 _lattice
                          (if (Variables|/Game/Blueprints/BP_Lattice.BP_Lattice_C|GetIsOpen _array_element_3)
                            (Default|Close _array_element_3)
                            (Utilities|FlowControl|Delay 0.1)
                            (Variables|/Game/Blueprints/BP_Lattice.BP_Lattice_C|SetIsOpen _array_element_3 true))))))))))
          (:then_1
            (goto _label_4 Stop))
          (:then_2
            (Audio|SpawnSoundatLocation "/Game/Sounds/switch_circuit_breaker_on.switch_circuit_breaker_on" (Transformation|GetWorldLocation _door1) "0, 0, 0" 1.0 1.0 0.0 "/Game/Sounds/Attenuation/DoorSoundAttenuation.DoorSoundAttenuation" 0)))
        (else
          (Utilities|FlowControl|Sequence
            (:then_0
              (Components|MoveComponentTo _door1_2 "0.000000,7.000000,25.500000" "0, 0, 0" false false 0.3 false :!label _label_4)
              (Variables|Default|SetPowerWorking? true)
              (Audio|SpawnSoundatLocation "/Game/Sounds/switch_circuit_breaker_off.switch_circuit_breaker_off" _returnvalue "0, 0, 0" 1.0 1.0 0.0 "/Game/Sounds/Attenuation/DoorSoundAttenuation.DoorSoundAttenuation" 0)
              (Utilities|FlowControl|Sequence
                (:then_0
                  (for _array_element_4 _lamps
                    (Variables|/Game/Blueprints/BP_LampHolder.BP_LampHolder_C|SetPowerOn? _array_element_4 true)
                    (if (Variables|/Game/Blueprints/BP_LampHolder.BP_LampHolder_C|GetOn/Off _array_element_4)
                      (Default|Switchon _array_element_4))))
                (:then_1
                  (Utilities|IsValid (Utilities|Array|Get(acopy) _sconce)
                    (:Is%20Valid
                      (for _array_element_5 _sconce
                        (Variables|/Game/Blueprints/BP_Sconce.BP_Sconce_C|SetPowerOn? _array_element_5 true)
                        (if (Variables|/Game/Blueprints/BP_Sconce.BP_Sconce_C|GetOn/Off _array_element_5)
                          (Default|Switchon _array_element_5))))))
                (:then_2
                  (Utilities|IsValid _lift_2
                    (:Is%20Valid
                      (Variables|/Game/Blueprints/Lift/BP_Lift.BP_Lift_C|SetPowered? _lift_2 true)
                      (Utilities|IsValid (Utilities|Array|Get(acopy) _lattice_2)
                        (:Is%20Valid
                          (for _array_element_6 _lattice_2
                            (if (Variables|/Game/Blueprints/BP_Lattice.BP_Lattice_C|GetIsOpen _array_element_6)
                              (Default|Open _array_element_6))))))))))
            (:then_1
              (goto _label_3 Stop))))))))

(fn ConstructionScript
  (|CallParentFunction))