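; BP_Toaster is a toaster actor that spawns BP_Slice toast at its Arrow component's transform.
; The Spawn Toast function returns the slice found by GetActorOfClass if it nearly matches the arrow's transform, otherwise it spawns and returns a new one.
; Only that one found slice is checked, so other slices at the arrow go unnoticed.
; A separate SpawnToast event always spawns a slice without this check.
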(event Custom|SpawnToast
  (Game|SpawnActorfromClass "/Game/Blueprints/PickUpObjects/BP_Slice.BP_Slice_C" (Transformation|GetWorldTransform (Variables|Default|GetArrow)) "AlwaysSpawn" 0 0))

(event EventBeginPlay)

(event Collision|EventActorBeginOverlap
  (params (OtherActor :type Actor%20Object%20Reference)))

(event EventTick
  (params (DeltaSeconds :type Float%20%28single-precision%29)))

(fn ConstructionScript)

(fn SpawnToast
  (bind _arrow (Variables|Default|GetArrow))
  (bind _returnvalue (Transformation|GetWorldTransform _arrow))
  (bind _returnvalue_2 (Actor|GetActorOfClass "/Game/Blueprints/PickUpObjects/BP_Slice.BP_Slice_C"))
  (Utilities|IsValid _returnvalue_2
    (:Is%20Valid
      (if (Class|KismetMathLibrary|NearlyEqualTransformTransform _returnvalue (Transformation|GetWorldTransform (Variables|/Script/Engine.Actor|GetRootComponent _returnvalue_2)) 1e+01 1e+01 1.0)
        (return _returnvalue_2)
        (else
          _)))
    (:Is%20Not%20Valid
      _))
  (bind _returnvalue_3 (Game|SpawnActorfromClass "/Game/Blueprints/PickUpObjects/BP_Slice.BP_Slice_C" _returnvalue "AlwaysSpawn" 0 0))
  (return _returnvalue_3))