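; BP_Stereo is an interactable stereo that the player or a neighbor can switch on and off, with a switch sound on each toggle.
; Both interact events flip OnOff and play or stop the Audio component.
; Only when the player switches it on does it report a "Stereo"-tagged noise event and write itself to the ObjectRef blackboard key of the AI found through GetActorOfClass.
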(event Custom|PlayerInteract
  (bind _returnvalue (Transformation|GetActorLocation))
  (bind _audio (Variables|Default|GetAudio))
  (if (Variables|Default|GetOnOff)
    (Audio|PlaySoundatLocation "/Game/Sounds/train_switch_on.train_switch_on" _returnvalue "0, 0, 0" 1.0 1.0 0.0 "/Game/Sounds/Attenuation/ItemAtten.ItemAtten" 0 0)
    (Audio|Components|Audio|Stop _audio)
    (Variables|Default|SetOnOff false)
    (else
      (Audio|PlaySoundatLocation "/Game/Sounds/train_switch_on.train_switch_on" _returnvalue "0, 0, 0" 1.0 1.0 0.0 "/Game/Sounds/Attenuation/ItemAtten.ItemAtten" 0 0)
      (Audio|Components|Audio|Play _audio 0.0)
      (Variables|Default|SetOnOff true)
      (Class|AISenseHearing|ReportNoiseEvent (Transformation|GetActorLocation) 5.0 self 7e+02 "Stereo")
      (bind _returnvalue_2 (Actor|GetActorOfClass "/Game/Blueprints/Characters/AI2/AI.AI_C"))
      (AI|Components|Blackboard|SetValueasObject (AI|GetBlackboard _returnvalue_2) (Utilities|Name|MakeLiteralName "ObjectRef") self))))

(event Custom|NeighborInteract
  (bind _returnvalue (Transformation|GetActorLocation))
  (bind _audio (Variables|Default|GetAudio))
  (if (Variables|Default|GetOnOff)
    (Audio|PlaySoundatLocation "/Game/Sounds/train_switch_on.train_switch_on" _returnvalue "0, 0, 0" 1.0 1.0 0.0 "/Game/Sounds/Attenuation/ItemAtten.ItemAtten" 0 0)
    (Audio|Components|Audio|Stop _audio)
    (Variables|Default|SetOnOff false)
    (else
      (Audio|PlaySoundatLocation "/Game/Sounds/train_switch_on.train_switch_on" _returnvalue "0, 0, 0" 1.0 1.0 0.0 "/Game/Sounds/Attenuation/ItemAtten.ItemAtten" 0 0)
      (Audio|Components|Audio|Play _audio 0.0)
      (Variables|Default|SetOnOff true))))

(event EventBeginPlay)

(event Collision|EventActorBeginOverlap
  (params (OtherActor :type Actor%20Object%20Reference)))

(event EventTick
  (params (DeltaSeconds :type Float%20%28single-precision%29)))

(fn ConstructionScript)