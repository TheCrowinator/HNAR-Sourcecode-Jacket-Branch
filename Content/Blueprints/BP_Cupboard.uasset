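; Two-door cupboard the player can open, close and hide in, and that the AI can search.
; A fast looping timer combines player overlap and door state to update hiding and the AI's chase and catch flags.
; AI overlaps open or close the doors depending on its state, catching a hidden player or playing a pass-by cue.
; Searches animate the AI and doors, then catch the player or close up.
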(event OnComponentBeginOverlap(Box1)
  (params (OverlappedComponent :type Primitive%20Component%20Object%20Reference) (OtherActor :type Actor%20Object%20Reference) (OtherComp :type Primitive%20Component%20Object%20Reference) (OtherBodyIndex :type Integer) (bFromSweep :type Boolean) (SweepResult :type Hit%20Result%20Structure%20%28by%20ref%29))
  (bind _asai (Utilities|Casting|CastToAI OtherActor))
  (Utilities|Casting|CastToCapsuleComponent OtherComp)
  (if (Variables|Default|GetInHiding)
    (if (Utilities|Enum|Equal(Enum) (Variables|/Game/Blueprints/Characters/AI2/AI.AI_C|GetCurrentState _asai) "NewEnumerator0")
      (Utilities|FlowControl|DoOnce false :!label _label
        (:Completed
          (Audio|Components|Audio|Play (Variables|Default|GetPass_By) 0.3)
          (Utilities|FlowControl|Delay 10.7)
          (goto _label Reset))))))

(event OnComponentBeginOverlap(Box_0)
  (params (OverlappedComponent :type Primitive%20Component%20Object%20Reference) (OtherActor :type Actor%20Object%20Reference) (OtherComp :type Primitive%20Component%20Object%20Reference) (OtherBodyIndex :type Integer) (bFromSweep :type Boolean) (SweepResult :type Hit%20Result%20Structure%20%28by%20ref%29))
  (bind _asai (Utilities|Casting|CastToAI OtherActor))
  (if (Utilities|Enum|Equal(Enum) (Variables|/Game/Blueprints/Characters/AI2/AI.AI_C|GetCurrentState _asai) "NewEnumerator4")
    (if (Variables|Default|GetInHiding)
      (Utilities|FlowControl|DoOnce false
        (:Completed
          (Pawn|Components|CharacterMovement|DisableMovement (Variables|/Script/Engine.Character|GetCharacterMovement _asai))
          (Pawn|SetControlRotation (AI|GetAIController _asai) (Math|Rotator|Lerp(Rotator) (Pawn|GetControlRotation (AI|GetAIController _asai) :!class /Script/Engine.Controller) (Math|Rotator|FindLookatRotation (Transformation|GetActorLocation) (Transformation|GetActorLocation _asai)) 0.0))
          (CallFunction|AiOpen _asai)
          (bind _anim_length (Default|PlayAnimAI _asai "/Game/Neighbor/Animations/neighbour_lowpoly_Anim_rig_open_double_door_inward.neighbour_lowpoly_Anim_rig_open_double_door_inward" false))
          (Utilities|FlowControl|Delay _anim_length)
          (Variables|/Game/Blueprints/Characters/AI2/AI.AI_C|SetCanCatch _asai true)
          (Default|Catch _asai))))
    (elif (Utilities|Enum|Equal(Enum) (Variables|/Game/Blueprints/Characters/AI2/AI.AI_C|GetCurrentState _asai) "NewEnumerator2")
      (if (not (and (Variables|Default|GetOpen) (Variables|Default|GetOpen_1)))
        (CallFunction|AiOpen _asai)
        (Utilities|FlowControl|Delay 1.0)))))

(event OnComponentEndOverlap(Box_0)
  (params (OverlappedComponent :type Primitive%20Component%20Object%20Reference) (OtherActor :type Actor%20Object%20Reference) (OtherComp :type Primitive%20Component%20Object%20Reference) (OtherBodyIndex :type Integer))
  (bind _asai (Utilities|Casting|CastToAI OtherActor))
  (if (Utilities|Enum|Equal(Enum) (Variables|/Game/Blueprints/Characters/AI2/AI.AI_C|GetCurrentState _asai) "NewEnumerator2")
    (if (and (Variables|Default|GetOpen) (Variables|Default|GetOpen_1))
      (CallFunction|AiClose _asai))))

(event Custom|CustomTick
  (bind _ai_0 (Variables|Default|GetAI_0))
  (bind _player (Variables|Default|GetPlayer))
  (bind _currentstate (Variables|/Game/Blueprints/Characters/AI2/AI.AI_C|GetCurrentState _ai_0))
  (bind _returnvalue (Utilities|Enum|Equal(Enum) _currentstate "NewEnumerator4"))
  (if (Class|PrimitiveComponent|IsOverlappingComponent (Variables|Default|GetBox) (Variables|/Script/Engine.Character|GetCapsuleComponent (Variables|Default|GetPlayer)))
    (if (Variables|Default|GetOpen_1)
      _
      (elif (Variables|Default|GetOpen)
        _
        (else
          (Utilities|FlowControl|DoOnce false :!label _label
            (:Completed
              (if (Variables|/Game/Blueprints/Characters/FirstPersonBP/Blueprints/FirstPersonCharacter.FirstPersonCharacter_C|GetInside? (Variables|Default|GetPlayer))
                (Variables|/Game/Blueprints/Characters/AI2/AI.AI_C|SetCanChase _ai_0 false))
              (Variables|/Game/Blueprints/Characters/AI2/AI.AI_C|SetCanCatch _ai_0 false)
              (bind _output_get (Variables|Default|SetInHiding true))
              (Variables|/Game/Blueprints/Characters/FirstPersonBP/Blueprints/FirstPersonCharacter.FirstPersonCharacter_C|SetIsHiding? _player _output_get)
              (Development|PrintString "HIDING IN CUPBOARD")
              (Math|Integer|IncrementInt (Variables|Default|GetHideCount)
                (:%20%20
                  (goto _label_2 Reset))))))))
    (Utilities|FlowControl|DoOnce false :!label _label_2
      (:Completed
        (if _returnvalue
          (Variables|/Game/Blueprints/Characters/AI2/AI.AI_C|SetCanChase _ai_0 true :!label _label_3)
          (bind _output_get_2 (Variables|Default|SetInHiding false :!label _label_4))
          (Variables|/Game/Blueprints/Characters/FirstPersonBP/Blueprints/FirstPersonCharacter.FirstPersonCharacter_C|SetIsHiding? _player _output_get_2)
          (if _returnvalue
            (Variables|/Game/Blueprints/Characters/AI2/AI.AI_C|SetCanCatch _ai_0 true)
            (else
              (Variables|/Game/Blueprints/Characters/AI2/AI.AI_C|SetCanCatch _ai_0 false)))
          (Development|PrintString "NOT HIDING IN CUPBOARD")
          (goto _label Reset)
          (else
            (Class|AIPerceptionComponent|ForgetAll (Variables|/Game/Blueprints/Characters/AI2/AI.AI_C|GetAIPerception _ai_0))
            (if (not (Variables|/Game/Blueprints/Characters/AI2/AI.AI_C|GetIsSleeping _ai_0))
              (if (Variables|/Game/Blueprints/Characters/FirstPersonBP/Blueprints/FirstPersonCharacter.FirstPersonCharacter_C|GetInside? (Variables|Default|GetPlayer))
                (goto _label_3)
                (else
                  (goto _label_4))))))))))

(event Custom|SearchCupboard
  (params (AI :type AI%20Object%20Reference) (Player :type First%20Person%20Character%20Object%20Reference))
  (bind _returnvalue (AI|GetAIController AI))
  (bind _charactermovement (Variables|/Script/Engine.Character|GetCharacterMovement AI))
  (Development|PrintString "Hello")
  (AI|SetFocus _returnvalue self)
  (if (and (Variables|Default|GetOpen) (Variables|Default|GetOpen_1))
    (Pawn|Components|CharacterMovement|DisableMovement _charactermovement)
    (Utilities|FlowControl|Delay 1.0)
    (AI|ClearFocus _returnvalue)
    (Pawn|Components|CharacterMovement|SetMovementMode _charactermovement "MOVE_Walking" 0)
    (else
      (Pawn|Components|CharacterMovement|DisableMovement _charactermovement)
      (bind _anim_length (Default|PlayAnimAI AI "/Game/Neighbor/Animations/neighbour_lowpoly_Anim_rig_open_double_door_inward.neighbour_lowpoly_Anim_rig_open_double_door_inward" false))
      (Utilities|FlowControl|Sequence
        (:then_0
          (Components|MoveComponentTo (Variables|Default|GetStaticMesh_0) "46.000000,28.000000,108.000000" "0,-100.000000, 0" false false 0.5 false))
        (:then_1
          (Components|MoveComponentTo (Variables|Default|GetDoor) "-46.000000,28.000000,108.000000" "0,100.000000, 0" false false 0.5 false))
        (:then_2
          (Utilities|FlowControl|Delay _anim_length)
          (if (Variables|Default|GetInHiding)
            (bind _anim_length_2 (Default|PlayAnimAI AI "/Game/Neighbor/Animations/neighbour_lowpoly_Anim_rig_spotted.neighbour_lowpoly_Anim_rig_spotted" false))
            (Utilities|FlowControl|Delay _anim_length_2)
            (Default|Catch AI)
            (Utilities|FlowControl|Delay 5.0)
            (else
              (bind _anim_length_3 (Default|PlayAnimAI AI "/Game/Neighbor/Animations/neighbour_lowpoly_Anim_rig_open_door_outward.neighbour_lowpoly_Anim_rig_open_door_outward" false))
              (Utilities|FlowControl|Sequence
                (:then_0
                  (Components|MoveComponentTo (Variables|Default|GetDoor) "-46.000000,28.000000,108.000000" "0,10.000000, 0" false false 0.5 false))
                (:then_1
                  (Components|MoveComponentTo (Variables|Default|GetStaticMesh_0) "46.000000,28.000000,108.000000" "0,-10.000000, 0" false false 0.5 false))
                (:then_2
                  (Utilities|FlowControl|Delay _anim_length_3)
                  (Pawn|Components|CharacterMovement|SetMovementMode (Variables|/Script/Engine.Character|GetCharacterMovement AI) "MOVE_Walking" 0)
                  (Components|Animation|SetAnimationMode (Variables|/Script/Engine.Character|GetMesh AI) "AnimationBlueprint")
                  (AI|ClearFocus _returnvalue))))))))))

(event Custom|AiOpen
  (params (Target :type AI%20Object%20Reference))
  (bind _door (Variables|Default|GetDoor))
  (bind _staticmesh_0 (Variables|Default|GetStaticMesh_0))
  (Utilities|FlowControl|Sequence
    (:then_0
      (Variables|Default|SetOpen true)
      (Collision|SetCollisionEnabled _door "NoCollision")
      (Components|MoveComponentTo _door "-46.000000,28.000000,108.000000" "0.000000,100.000000, 0" false false 0.5 false)
      (Collision|SetCollisionEnabled _door "QueryAndPhysics"))
    (:then_1
      (Variables|Default|SetOpen_1 true)
      (Collision|SetCollisionEnabled _staticmesh_0 "NoCollision")
      (Components|MoveComponentTo _staticmesh_0 "46.000000,28.000000,108.000000" "0,-100.000000, 0" false false 0.5 false)
      (Utilities|FlowControl|Delay 0.2)
      (if (Class|PrimitiveComponent|IsOverlappingComponent (Variables|Default|GetBox) (Variables|/Script/Engine.Character|GetCapsuleComponent (Variables|Default|GetPlayer)))
        (Default|Catch (Variables|Default|GetAI_0))))))

(event Custom|AiClose
  (params (Target :type AI%20Object%20Reference))
  (bind _staticmesh_0 (Variables|Default|GetStaticMesh_0))
  (bind _door (Variables|Default|GetDoor))
  (Utilities|FlowControl|Sequence
    (:then_0
      (Variables|Default|SetOpen false)
      (Components|MoveComponentTo _door "-46.000000,28.000000,108.000000" "0,10.000000, 0" false false 0.5 false)
      (Collision|SetCollisionEnabled _door "QueryAndPhysics"))
    (:then_1
      (Variables|Default|SetOpen_1 false)
      (Components|MoveComponentTo _staticmesh_0 "46.000000,28.000000,108.000000" "0,-10.000000, 0" false false 0.5 false)
      (Collision|SetCollisionEnabled _staticmesh_0 "QueryAndPhysics"))))

(event EventBeginPlay
  (bind _asfirst_person_character (Utilities|Casting|CastToFirstPersonCharacter (Game|GetPlayerCharacter 0)))
  (Variables|Default|SetPlayer _asfirst_person_character)
  (Utilities|Time|SetTimerbyEvent (delegate Custom|CustomTick) 0.01 true))

(event EventOpenClose
  (params (Component :type Primitive%20Component%20Object%20Reference))
  (bind _staticmesh_0 (Variables|Default|GetStaticMesh_0))
  (bind _door (Variables|Default|GetDoor))
  (if (== Component (Variables|Default|GetDoor))
    (if (not (Variables|Default|GetLocked))
      (if (Variables|Default|GetOpen)
        (Utilities|FlowControl|Sequence
          (:then_0
            (Variables|Default|SetOpen false)
            (Components|MoveComponentTo _door "-46.000000,28.000000,108.000000" "0,10.000000, 0" false false 0.5 false :!label _label))
          (:then_1
            (goto _label_2 Stop)))
        (else
          (Utilities|FlowControl|Sequence
            (:then_0
              (Variables|Default|SetOpen true)
              (Components|MoveComponentTo _door "-46.000000,28.000000,108.000000" "0,100.000000, 0" false false 0.5 false :!label _label_2))
            (:then_1
              (goto _label Stop))))))
    (elif (== Component (Variables|Default|GetStaticMesh_0))
      (if (not (Variables|Default|GetLocked))
        (if (Variables|Default|GetOpen_1)
          (Utilities|FlowControl|Sequence
            (:then_0
              (Variables|Default|SetOpen_1 false)
              (Components|MoveComponentTo _staticmesh_0 "46.000000,28.000000,108.000000" "0,-10.000000, 0" false false 0.5 false :!label _label_3))
            (:then_1
              (goto _label_4 Stop)))
          (else
            (Utilities|FlowControl|Sequence
              (:then_0
                (Variables|Default|SetOpen_1 true)
                (Components|MoveComponentTo _staticmesh_0 "46.000000,28.000000,108.000000" "0,-100.000000, 0" false false 0.5 false :!label _label_4))
              (:then_1
                (goto _label_3 Stop)))))))))

(fn ConstructionScript
  (|CallParentFunction))

(fn AISearchCupboard
  (params (AI :type AI%20Object%20Reference))
  (CallFunction|SearchCupboard AI (Variables|Default|GetPlayer))
  (return))