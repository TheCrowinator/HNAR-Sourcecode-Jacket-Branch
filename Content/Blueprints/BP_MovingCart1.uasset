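; Cart actor that rides along the spline of a referenced track, travelling backward from the spline's end toward its start.
; When Move is enabled, it waits a random delay, then reverses the Mover timeline from StartOffset, with play rate derived from Duration.
; Each update maps timeline alpha to spline distance to set location and rotation.
; On finishing, it waits another random delay and replays from the end, looping indefinitely.
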(event Custom|MoveCart
  (bind _mover (Variables|Default|GetMover))
  (bind _trackref (Variables|Default|GetTrackRef))
  (bind _spline (Variables|/Game/Blueprints/BP_Spline.BP_Spline_C|GetSpline _trackref))
  (Components|Timeline|SetPlayRate _mover (/ 1.0 (Variables|Default|GetDuration)))
  (Components|Timeline|SetNewTime _mover (Variables|Default|GetStartOffset))
  (bind _alpha (Timeline|Mover Reverse)
    (:Update
      (Variables|Default|SetAlpha _alpha)
      (Transformation|SetActorLocationAndRotation (Spline|GetLocationatDistanceAlongSpline _spline (Math|Float|Lerp 0.0 (Spline|GetSplineLength _spline) (Variables|Default|GetAlpha)) "World") (Spline|GetRotationatDistanceAlongSpline _spline (Math|Float|Lerp 0.0 (Spline|GetSplineLength _spline) (Variables|Default|GetAlpha)) "World")))
    (:Finished
      (Utilities|FlowControl|Delay (Math|Conversions|ToFloat(Integer) (Math|Random|RandomIntegerinRange 0 30)))
      (Timeline|Mover ReverseFromEnd))))

(event EventBeginPlay
  (if (Variables|Default|GetMove)
    (Utilities|FlowControl|Delay (Math|Conversions|ToFloat(Integer) (Math|Random|RandomIntegerinRange 0 30)))
    (CallFunction|MoveCart)))

(fn ConstructionScript)