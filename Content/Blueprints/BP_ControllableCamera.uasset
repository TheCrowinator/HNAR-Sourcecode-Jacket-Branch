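; Controllable security-style camera actor whose static mesh pans in yaw on Right, Left and RightStop events.
; Right and Left only act while the actor is the view target, playing or reversing a timeline that sets yaw.
; The timeline starts at ZValue and restarts from the opposite end on finishing, so panning continues in the same direction.
; An unconnected FlipFlop holds view switching between this camera and the first-person player, with widget visibility toggles.
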(event Custom|Right
  (if (Variables|Default|GetControllable?)
    (Variables|Default|SetRight? true)
    (bind _value (Timeline|Timeline_0 Play)
      (:Update
        (Transformation|SetWorldRotation (Variables|Default|GetStaticMesh) (Math|Rotator|MakeRotator 0.0 0.0 _value) false false))
      (:Finished
        (if (Variables|Default|GetRight?)
          (Timeline|Timeline_0 PlayFromStart)
          (else
            (Timeline|Timeline_0 ReverseFromEnd)))))))

(event Custom|RightStop
  (bind _value (Timeline|Timeline_0 Stop)
    (:Update
      (Transformation|SetWorldRotation (Variables|Default|GetStaticMesh) (Math|Rotator|MakeRotator 0.0 0.0 _value) false false))
    (:Finished
      (if (Variables|Default|GetRight?)
        (Timeline|Timeline_0 PlayFromStart)
        (else
          (Timeline|Timeline_0 ReverseFromEnd))))))

(event Custom|Left
  (if (Variables|Default|GetControllable?)
    (Variables|Default|SetRight? false)
    (bind _value (Timeline|Timeline_0 Reverse)
      (:Update
        (Transformation|SetWorldRotation (Variables|Default|GetStaticMesh) (Math|Rotator|MakeRotator 0.0 0.0 _value) false false))
      (:Finished
        (if (Variables|Default|GetRight?)
          (Timeline|Timeline_0 PlayFromStart)
          (else
            (Timeline|Timeline_0 ReverseFromEnd)))))))

(event EventBeginPlay
  (bind _asfirst_person_character (Utilities|Casting|CastToFirstPersonCharacter (Game|GetPlayerCharacter 0)))
  (Variables|Default|SetPlayer _asfirst_person_character)
  (bind _value (Timeline|Timeline_0 SetNewTime)
    (:Update
      (Transformation|SetWorldRotation (Variables|Default|GetStaticMesh) (Math|Rotator|MakeRotator 0.0 0.0 _value) false false))
    (:Finished
      (if (Variables|Default|GetRight?)
        (Timeline|Timeline_0 PlayFromStart)
        (else
          (Timeline|Timeline_0 ReverseFromEnd))))))

(event EventOnBecomeViewTarget
  (params (PC :type Player%20Controller%20Object%20Reference))
  (Variables|Default|SetControllable? true))

(event EventOnEndViewTarget
  (params (PC :type Player%20Controller%20Object%20Reference))
  (Variables|Default|SetControllable? false))

(event Input|ActionEvents|InputActionChangeCamera
  (params (Key :type Key%20Structure)))

(fn ConstructionScript)