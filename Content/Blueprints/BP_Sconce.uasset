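; BP_Sconce is a switchable wall light that pairs a bulb mesh material with a SpotLight.
; On BeginPlay, if PowerOn is set, it applies the OnOff state by swapping between BulbTexture and M_StatueGlass and toggling spotlight visibility.
; SwitchOn and SwitchOff always record OnOff but only change the visuals when powered.
; ForceSwitchOff darkens the light regardless of power, leaving OnOff untouched.
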(event Custom|SwitchOn
  (Variables|Default|SetOn/Off true)
  (if (Variables|Default|GetPowerOn?)
    (Rendering|Material|SetMaterial (Variables|Default|GetStaticMesh1) 0 (Variables|Default|GetBulbTexture))
    (Rendering|SetVisibility (Variables|Default|GetSpotLight) true false)))

(event Custom|SwitchOff
  (Variables|Default|SetOn/Off false)
  (if (Variables|Default|GetPowerOn?)
    (Rendering|Material|SetMaterial (Variables|Default|GetStaticMesh1) 0 "/Game/StarterContent/Props/Materials/M_StatueGlass.M_StatueGlass")
    (Rendering|SetVisibility (Variables|Default|GetSpotLight) false false)))

(event Custom|Force%20Switch%20Off
  (Rendering|Material|SetMaterial (Variables|Default|GetStaticMesh1) 0 "/Game/StarterContent/Props/Materials/M_StatueGlass.M_StatueGlass")
  (Rendering|SetVisibility (Variables|Default|GetSpotLight) false false))

(event EventBeginPlay
  (bind _spotlight (Variables|Default|GetSpotLight))
  (bind _staticmesh1 (Variables|Default|GetStaticMesh1))
  (if (Variables|Default|GetPowerOn?)
    (if (Variables|Default|GetOn/Off)
      (Rendering|Material|SetMaterial _staticmesh1 0 (Variables|Default|GetBulbTexture))
      (Rendering|SetVisibility _spotlight true false)
      (else
        (Rendering|Material|SetMaterial _staticmesh1 0 "/Game/StarterContent/Props/Materials/M_StatueGlass.M_StatueGlass")
        (Rendering|SetVisibility _spotlight false false)))))

(fn ConstructionScript)