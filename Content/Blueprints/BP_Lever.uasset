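; BP_Lever is an interactable lever that toggles between open and closed states.
; Interact on StaticMesh1, when CanOpen is set, passes a DoOnce gate and swings the mesh with MoveComponentTo toward the opposite state while stopping the reverse move.
; On completion it plays the switch sound, updates Open, calls the empty OnOpen or OnClose hook and resets the gate, so input during the swing is ignored.
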(event Custom|Interact
  (params (Component :type Object%20Object%20Reference))
  (bind _staticmesh1 (Variables|Default|GetStaticMesh1))
  (if (== Component (Variables|Default|GetStaticMesh1))
    (if (Variables|Default|GetCanOpen)
      (Utilities|FlowControl|DoOnce false :!label _label
        (:Completed
          (if (Variables|Default|GetOpen)
            (Utilities|FlowControl|Sequence
              (:then_0
                (Components|MoveComponentTo _staticmesh1 "0,7.000000, 0" "0, 0,175.000000" false false 0.3 false :!label _label_2)
                (Audio|PlaySoundatLocation "/Game/Sounds/switch_off.switch_off" (Transformation|GetActorLocation) "0, 0, 0" 1.0 1.0 0.0 "/Game/Sounds/Attenuation/FridgeAttenuation.FridgeAttenuation" 0 0)
                (Variables|Default|SetOpen false)
                (CallFunction|OnClose)
                (goto _label Reset))
              (:then_1
                (goto _label_3 Stop)))
            (else
              (Utilities|FlowControl|Sequence
                (:then_0
                  (Components|MoveComponentTo _staticmesh1 "0,7.000000, 0" "0, 0, 0" false false 0.3 false :!label _label_3)
                  (Audio|PlaySoundatLocation "/Game/Sounds/switch_off.switch_off" (Transformation|GetActorLocation) "0, 0, 0" 1.0 1.0 0.0 "/Game/Sounds/Attenuation/FridgeAttenuation.FridgeAttenuation" 0 0)
                  (Variables|Default|SetOpen true)
                  (CallFunction|OnOpen)
                  (goto _label Reset))
                (:then_1
                  (goto _label_2 Stop))))))))))

(event Custom|OnOpen)

(event Custom|OnClose)

(event EventBeginPlay)

(event Collision|EventActorBeginOverlap
  (params (OtherActor :type Actor%20Object%20Reference)))

(event EventTick
  (params (DeltaSeconds :type Float%20%28single-precision%29)))

(fn ConstructionScript)