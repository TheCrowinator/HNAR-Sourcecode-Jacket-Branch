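; Keypad actor that unlocks a linked Door when the player enters a four-button code, picked at random and debug-printed on BeginPlay.
; Interact uses CheckButtons to reject repeated presses, then appends the button's name, pushes it in and makes it emissive, behind a re-entry gate.
; A wrong code resets all buttons; a correct one disables the keypad.
; A looping timer also syncs the door lock to the entered code.
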(event Custom|Interact
  (params (Component :type Primitive%20Component%20Object%20Reference))
  (bind _0 (Variables|Default|Get0))
  (bind _9 (Variables|Default|Get9))
  (bind _1 (Variables|Default|Get1))
  (bind _2 (Variables|Default|Get2))
  (bind _3 (Variables|Default|Get3))
  (bind _4 (Variables|Default|Get4))
  (bind _5 (Variables|Default|Get5))
  (bind _6 (Variables|Default|Get6))
  (bind _7 (Variables|Default|Get7))
  (bind _8 (Variables|Default|Get8))
  (if (Variables|Default|GetInteractable?)
    (Utilities|FlowControl|Gate false :!label _label
      (:Exit
        (Utilities|FlowControl|Sequence
          (:then_0
            (goto _label Close))
          (:then_1
            (bind _output_get (Variables|Default|SetComponent Component))
            (bind (_button _accepted) (CallFunction|CheckButtons _output_get))
            (if _accepted
              (Math|Integer|IncrementInt (Variables|Default|GetTotalButtonsPressed)
                (:%20%20
                  (bind _output_get_2 (Variables|Default|SetCodeEntered (Utilities|String|Append (Variables|Default|GetCodeEntered) (Utilities|GetObjectName _button))))
                  (Development|PrintString _output_get_2 true true "(R=0.000000,G=0.660000,B=1.000000,A=1.000000)" 5.0)
                  (Components|MoveComponentTo _button "0,-1.000000, 0" "0, 0, 0" false false 0.2 false)
                  (Rendering|Material|SetMaterial _button 0 "/Game/Materials/Instances/MI_Panel_Emissive.MI_Panel_Emissive")
                  (if (== (Variables|Default|GetTotalButtonsPressed) 4)
                    (if (Utilities|Enum|Equal(Enum) (Variables|Default|GetCodeEntered) (Variables|Default|GetCode))
                      (Variables|Default|SetInteractable? false)
                      (Utilities|FlowControl|Delay 0.1)
                      (Variables|/Game/Blueprints/BP_Door.BP_Door_C|SetLocked (Variables|Default|GetDoor) false)
                      (else
                        (Utilities|FlowControl|Sequence
                          (:then_0
                            (Components|MoveComponentTo _0 "0, 0, 0" "0, 0, 0" false false 0.2 false)
                            (Rendering|Material|SetMaterial _0 0 "/Game/Materials/Instances/MI_Panel.MI_Panel")
                            (Variables|Default|SetTotalButtonsPressed 0)
                            (Variables|Default|SetCodeEntered "")
                            (Utilities|Array|Clear (Variables|Default|GetPressedButtons))
                            (goto _label Open))
                          (:then_1
                            (Components|MoveComponentTo _1 "0, 0, 0" "0, 0, 0" false false 0.2 false)
                            (Rendering|Material|SetMaterial _1 0 "/Game/Materials/Instances/MI_Panel.MI_Panel"))
                          (:then_2
                            (Components|MoveComponentTo _2 "0, 0, 0" "0, 0, 0" false false 0.2 false)
                            (Rendering|Material|SetMaterial _2 0 "/Game/Materials/Instances/MI_Panel.MI_Panel"))
                          (:then_3
                            (Components|MoveComponentTo _3 "0, 0, 0" "0, 0, 0" false false 0.2 false)
                            (Rendering|Material|SetMaterial _3 0 "/Game/Materials/Instances/MI_Panel.MI_Panel"))
                          (:then_4
                            (Components|MoveComponentTo _4 "0, 0, 0" "0, 0, 0" false false 0.2 false)
                            (Rendering|Material|SetMaterial _4 0 "/Game/Materials/Instances/MI_Panel.MI_Panel"))
                          (:then_5
                            (Components|MoveComponentTo _5 "0, 0, 0" "0, 0, 0" false false 0.2 false)
                            (Rendering|Material|SetMaterial _5 0 "/Game/Materials/Instances/MI_Panel.MI_Panel"))
                          (:then_6
                            (Components|MoveComponentTo _6 "0, 0, 0" "0, 0, 0" false false 0.2 false)
                            (Rendering|Material|SetMaterial _6 0 "/Game/Materials/Instances/MI_Panel.MI_Panel"))
                          (:then_7
                            (Components|MoveComponentTo _7 "0, 0, 0" "0, 0, 0" false false 0.2 false)
                            (Rendering|Material|SetMaterial _7 0 "/Game/Materials/Instances/MI_Panel.MI_Panel"))
                          (:then_8
                            (Components|MoveComponentTo _8 "0, 0, 0" "0, 0, 0" false false 0.2 false)
                            (Rendering|Material|SetMaterial _8 0 "/Game/Materials/Instances/MI_Panel.MI_Panel"))
                          (:then_9
                            (Components|MoveComponentTo _9 "0, 0, 0" "0, 0, 0" false false 0.2 false)
                            (Rendering|Material|SetMaterial _9 0 "/Game/Materials/Instances/MI_Panel.MI_Panel")))))
                    (else
                      (Development|PrintString "NOT ENOUGH BUTTONS PRESSED" true true "(R=1.000000,G=0.849572,B=0.000000,A=1.000000)" 5.0)
                      (goto _label Open)))))
              (else
                (Development|PrintString "ButtonNotAccepted" true true "(R=1.000000,G=0.006586,B=0.000000,A=1.000000)")
                (goto _label Open)))))))
    (else
      (Development|PrintString "NOT INTERACTABLE"))))

(event Custom|Tick
  (bind _door (Variables|Default|GetDoor))
  (Utilities|FlowControl|Sequence
    (:then_0
      (if (Utilities|Enum|Equal(Enum) (Variables|Default|GetCodeEntered) (Variables|Default|GetCode))
        (Utilities|FlowControl|DoOnce false
          (:Completed
            (Variables|/Game/Blueprints/BP_Door.BP_Door_C|SetLocked _door false)))
        (else
          (Variables|/Game/Blueprints/BP_Door.BP_Door_C|SetLocked _door true))))))

(event EventBeginPlay
  (Utilities|IsValid (Variables|Default|GetDoor)
    (:Is%20Valid
      (Utilities|Time|SetTimerbyEvent (delegate Custom|Tick) 0.01 true)
      (bind _output_get (Variables|Default|SetCode (.OutItem (Utilities|Array|Random (Variables|Default|GetPossibleCodeVariations)))))
      (Development|PrintString _output_get true true "(R=1.000000,G=0.235953,B=0.565338,A=1.000000)" 1e+01)
      (Variables|Default|SetPerformAction (Variables|Default|GetInteractable?)))))

(fn ConstructionScript)

(fn CheckButtons
  (params (Component :type Primitive%20Component%20Object%20Reference))
  (bind _9 (Variables|Default|Get9))
  (bind _0 (Variables|Default|Get0))
  (bind _7 (Variables|Default|Get7))
  (bind _8 (Variables|Default|Get8))
  (bind _pressedbuttons (Variables|Default|GetPressedButtons))
  (bind _1 (Variables|Default|Get1))
  (bind _2 (Variables|Default|Get2))
  (bind _3 (Variables|Default|Get3))
  (bind _4 (Variables|Default|Get4))
  (bind _5 (Variables|Default|Get5))
  (bind _6 (Variables|Default|Get6))
  (if (== Component _0)
    (bind _output_get (Variables|Default|SetButtonPressed _0))
    (if (== (Utilities|Array|Get(acopy) _pressedbuttons) _output_get) :!label _label
      _
      (elif (== (Utilities|Array|Get(acopy) _pressedbuttons 1) _output_get)
        _
        (elif (== (Utilities|Array|Get(acopy) _pressedbuttons 2) _output_get)
          _
          (else
            (Utilities|Array|Add _pressedbuttons _output_get)
            (return _output_get true)))))
    (elif (== Component _1)
      (Variables|Default|SetButtonPressed _1)
      (goto _label)
      (elif (== Component _2)
        (Variables|Default|SetButtonPressed _2)
        (goto _label)
        (elif (== Component _3)
          (Variables|Default|SetButtonPressed _3)
          (goto _label)
          (elif (== Component _4)
            (Variables|Default|SetButtonPressed _4)
            (goto _label)
            (elif (== Component _5)
              (Variables|Default|SetButtonPressed _5)
              (goto _label)
              (elif (== Component _6)
                (Variables|Default|SetButtonPressed _6)
                (goto _label)
                (elif (== Component _7)
                  (Variables|Default|SetButtonPressed _7)
                  (goto _label)
                  (elif (== Component _8)
                    (Variables|Default|SetButtonPressed _8)
                    (goto _label)
                    (elif (== Component _9)
                      (Variables|Default|SetButtonPressed _9)
                      (goto _label)
                      (else
                        _)))))))))))
  (return 0 false))