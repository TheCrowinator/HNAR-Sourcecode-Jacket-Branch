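; BP_Train is a powerable train car with sliding doors, a start button and spline-following movement.
; Power events toggle lights and meshes; the Box trigger slides the doors for the player when powered and stationary.
; The one-shot Cylinder button plays audio, changes lights and materials, and sets Moving.
; MoveCart drives the actor along TrackRef's spline via the Mover timeline, but its only call here is disconnected.
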(event OnComponentBeginOverlap(Box)
  (params (OverlappedComponent :type Primitive%20Component%20Object%20Reference) (OtherActor :type Actor%20Object%20Reference) (OtherComp :type Primitive%20Component%20Object%20Reference) (OtherBodyIndex :type Integer) (bFromSweep :type Boolean) (SweepResult :type Hit%20Result%20Structure%20%28by%20ref%29))
  (bind _cube (Variables|Default|GetCube))
  (bind _cube1 (Variables|Default|GetCube1))
  (Utilities|Casting|CastToFirstPersonCharacter OtherActor)
  (if (Variables|Default|GetPowered)
    (if (not (Variables|Default|GetMoving))
      (Utilities|FlowControl|Sequence
        (:then_0
          (Collision|SetCollisionEnabled _cube "NoCollision")
          (Components|MoveComponentTo _cube "103.000000,-82.000000,104.000000" "0, 0, 0" false false 0.3 false))
        (:then_1
          (Components|MoveComponentTo _cube1 "103.000000,-232.000000,104.000000" "0, 0, 0" false false 0.3 false))
        (:then_2
          (Components|MoveComponentTo _cube "103.000000,-132.000000,104.000000" "0, 0, 0" false false 0.3 false) ; enters at Stop
        )
        (:then_3
          (Components|MoveComponentTo _cube1 "103.000000,-182.000000,104.000000" "0, 0, 0" false false 0.3 false) ; enters at Stop
        )))))

(event OnComponentEndOverlap(Box)
  (params (OverlappedComponent :type Primitive%20Component%20Object%20Reference) (OtherActor :type Actor%20Object%20Reference) (OtherComp :type Primitive%20Component%20Object%20Reference) (OtherBodyIndex :type Integer))
  (bind _cube1 (Variables|Default|GetCube1))
  (Utilities|Casting|CastToFirstPersonCharacter OtherActor)
  (if (Variables|Default|GetPowered)
    (if (not (Variables|Default|GetMoving))
      (Utilities|FlowControl|Sequence
        (:then_0
          (Collision|SetCollisionEnabled _cube1 "QueryAndPhysics")
          (Components|MoveComponentTo (Variables|Default|GetCube) "103.000000,-132.000000,104.000000" "0, 0, 0" false false 0.3 false))
        (:then_1
          (Components|MoveComponentTo _cube1 "103.000000,-182.000000,104.000000" "0, 0, 0" false false 0.3 false))
        (:then_2
          (Components|MoveComponentTo _cube1 "103.000000,-232.000000,104.000000" "0, 0, 0" false false 0.3 false) ; enters at Stop
        )
        (:then_3
          (Components|MoveComponentTo _cube1 "103.000000,-232.000000,104.000000" "0, 0, 0" false false 0.3 false) ; enters at Stop
        )))))

(event Custom|MoveCart
  (bind _trackref (Variables|Default|GetTrackRef))
  (bind _mover (Variables|Default|GetMover))
  (bind _spline (Variables|/Game/Blueprints/BP_SplineMesh.BP_SplineMesh_C|GetSpline _trackref))
  (Components|Timeline|SetPlayRate _mover (/ 1.0 (Variables|Default|GetDuration)))
  (Components|Timeline|SetNewTime _mover (Variables|Default|GetStartOffset))
  (bind _alpha (Timeline|Mover Play)
    (:Update
      (Variables|Default|SetAlpha _alpha)
      (Transformation|SetActorLocationAndRotation (Spline|GetLocationatDistanceAlongSpline _spline (Math|Float|Lerp 0.0 (Spline|GetSplineLength _spline) (Variables|Default|GetAlpha)) "World") (Spline|GetRotationatDistanceAlongSpline _spline (Math|Float|Lerp 0.0 (Spline|GetSplineLength _spline) (Variables|Default|GetAlpha)) "World")))
    (:Finished
      (Audio|Components|Audio|Stop (Variables|Default|Gettrain_loop_move_Cue))
      (Variables|Default|SetMoving false))))

(event Custom|PressButton
  (params (Component :type Primitive%20Component%20Object%20Reference))
  (bind _cylinder (Variables|Default|GetCylinder))
  (if (== Component _cylinder)
    (Utilities|FlowControl|DoOnce false
      (:Completed
        (Audio|PlaySoundatLocation "/Game/Sounds/train_switch_on.train_switch_on" (Transformation|GetWorldLocation _cylinder) "0, 0, 0" 1.0 1.0 0.0 "/Game/Sounds/Attenuation/FridgeAttenuation.FridgeAttenuation" 0 0)
        (Rendering|SetVisibility (Variables|Default|GetPointLight1) false false)
        (Rendering|Material|SetMaterial (Variables|Default|GetCube13) 0 "/Game/StarterContent/Materials/M_Glass.M_Glass")
        (Audio|Components|Audio|Play (Variables|Default|Gettrain_loop_move_Cue) 0.0)
        (Variables|Default|SetMoving true)))))

(event Custom|PowerOnOff
  (if (Variables|Default|GetPowered)
    (CallFunction|PowerOff)
    (else
      (CallFunction|Poweron))))

(event Custom|PowerOff
  (Rendering|SetVisibility (Variables|Default|GetSpotLight) false false)
  (Variables|Default|SetPowered false))

(event Custom|PowerOn
  (Rendering|SetVisibility (Variables|Default|GetSpotLight) true false)
  (Variables|Default|SetPowered true))

(event EventBeginPlay
  (bind _asfirst_person_character (Utilities|Casting|CastToFirstPersonCharacter (Game|GetPlayerCharacter 0)))
  (Variables|Default|SetAs%20Player _asfirst_person_character)
  (Utilities|FlowControl|Sequence
    (:then_0
      (Audio|Components|Audio|Stop (Variables|Default|Gettrain_loop_move_Cue))
      (Variables|Default|SetMoving false))
    (:then_1
      (if (Variables|Default|GetPoweredByDefault?)
        (CallFunction|Poweron)
        (else
          (CallFunction|PowerOff))))))

(fn ConstructionScript)