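; BP_Fence is a fence actor built from six static mesh pieces, each toggled by its own in-use boolean.
; On BeginPlay, a sequence checks each flag and either shows its mesh with query and physics collision or hides it with collision disabled.
; The construction script is empty, so the toggles take effect only at runtime, not as an editor preview.
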(event EventBeginPlay
  (bind _staticmesh4 (Variables|Default|GetStaticMesh4))
  (bind _staticmesh5 (Variables|Default|GetStaticMesh5))
  (bind _staticmesh (Variables|Default|GetStaticMesh))
  (bind _staticmesh1 (Variables|Default|GetStaticMesh1))
  (bind _staticmesh2 (Variables|Default|GetStaticMesh2))
  (bind _staticmesh3 (Variables|Default|GetStaticMesh3))
  (Utilities|FlowControl|Sequence
    (:then_0
      (if (Variables|Default|Get1inuse)
        (Rendering|SetVisibility _staticmesh true false)
        (Collision|SetCollisionEnabled _staticmesh "QueryAndPhysics")
        (else
          (Rendering|SetVisibility _staticmesh false false)
          (Collision|SetCollisionEnabled _staticmesh "NoCollision"))))
    (:then_1
      (if (Variables|Default|Get2inuse)
        (Rendering|SetVisibility _staticmesh1 true false)
        (Collision|SetCollisionEnabled _staticmesh1 "QueryAndPhysics")
        (else
          (Rendering|SetVisibility _staticmesh1 false false)
          (Collision|SetCollisionEnabled _staticmesh1 "NoCollision"))))
    (:then_2
      (if (Variables|Default|Get3inuse)
        (Rendering|SetVisibility _staticmesh2 true false)
        (Collision|SetCollisionEnabled _staticmesh2 "QueryAndPhysics")
        (else
          (Rendering|SetVisibility _staticmesh2 false false)
          (Collision|SetCollisionEnabled _staticmesh2 "NoCollision"))))
    (:then_3
      (if (Variables|Default|Get4inuse)
        (Rendering|SetVisibility _staticmesh3 true false)
        (Collision|SetCollisionEnabled _staticmesh3 "QueryAndPhysics")
        (else
          (Rendering|SetVisibility _staticmesh3 false false)
          (Collision|SetCollisionEnabled _staticmesh3 "NoCollision"))))
    (:then_4
      (if (Variables|Default|Get5inuse)
        (Rendering|SetVisibility _staticmesh4 true false)
        (Collision|SetCollisionEnabled _staticmesh4 "QueryAndPhysics")
        (else
          (Rendering|SetVisibility _staticmesh4 false false)
          (Collision|SetCollisionEnabled _staticmesh4 "NoCollision"))))
    (:then_5
      (if (Variables|Default|Get6inuse)
        (Rendering|SetVisibility _staticmesh5 true false)
        (Collision|SetCollisionEnabled _staticmesh5 "QueryAndPhysics")
        (else
          (Rendering|SetVisibility _staticmesh5 false false)
          (Collision|SetCollisionEnabled _staticmesh5 "NoCollision"))))))

(fn ConstructionScript)