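; A breakable two-pane window that alerts the AI to shattered glass and can open a path through itself.
; Each pane's first fracture plays a sound and, if the AI can hear, reports noise, stores an investigate transform and sets the window as blackboard ObjectRef.
; Optional smart links start disabled and enable per broken pane in that hearing branch.
; Reaching a link turns the AI and briefly disables capsule and mesh collision.
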(event OnComponentFracture(Destructible)
  (params (HitPoint :type Vector%20%28by%20ref%29 :default "0, 0, 0") (HitDirection :type Vector%20%28by%20ref%29 :default "0, 0, 0"))
  (bind _self self)
  (bind _arrow (Variables|Default|GetArrow))
  (bind _navlink1 (Variables|Default|GetNavLink1))
  (Utilities|FlowControl|DoOnce false
    (:Completed
      (Audio|PlaySoundatLocation "/Game/Sounds/GlassBreak.GlassBreak" (Transformation|GetActorLocation (Components|GetOwner (Variables|Default|GetDestructible))) "0, 0, 0" 1.0 1.0 0.0 "/Game/Sounds/Attenuation/DoorSoundAttenuation.DoorSoundAttenuation" 0 0)
      (if (Variables|/Game/Blueprints/Characters/AI2/AI.AI_C|GetCanHear (Variables|Default|GetAI))
        (Class|AISenseHearing|ReportNoiseEvent (Transformation|GetWorldLocation _arrow) 5.0 _self 6e+02 "Window")
        (if (Variables|Default|GetNavLinksInUse)
          (Utilities|IsValid _navlink1
            (:Is%20Valid
              (Class|NavLinkProxy|SetSmartLinkEnabled _navlink1 true))
            (:Is%20Not%20Valid
              _)))
        (Variables|Default|SetInvestigateTransform (Transformation|GetWorldTransform _arrow))
        (Variables|Default|SetIsBroken_1 true)
        (AI|Components|Blackboard|SetValueasObject (AI|GetBlackboard (Variables|Default|GetAI)) (Utilities|Name|MakeLiteralName "ObjectRef") _self)))))

(event OnComponentFracture(Destructible1)
  (params (HitPoint :type Vector%20%28by%20ref%29 :default "0, 0, 0") (HitDirection :type Vector%20%28by%20ref%29 :default "0, 0, 0"))
  (bind _self self)
  (bind _navlink2 (Variables|Default|GetNavLink2))
  (bind _arrow1 (Variables|Default|GetArrow1))
  (Utilities|FlowControl|DoOnce false
    (:Completed
      (Audio|PlaySoundatLocation "/Game/Sounds/GlassBreak.GlassBreak" (Transformation|GetActorLocation (Components|GetOwner (Variables|Default|GetDestructible1))) "0, 0, 0" 1.0 1.0 0.0 "/Game/Sounds/Attenuation/DoorSoundAttenuation.DoorSoundAttenuation" 0 0)
      (if (Variables|/Game/Blueprints/Characters/AI2/AI.AI_C|GetCanHear (Variables|Default|GetAI))
        (Class|AISenseHearing|ReportNoiseEvent (Transformation|GetWorldLocation _arrow1) 5.0 _self 6e+02 "Window")
        (if (Variables|Default|GetNavLinksInUse)
          (Utilities|IsValid _navlink2
            (:Is%20Valid
              (Class|NavLinkProxy|SetSmartLinkEnabled _navlink2 true))
            (:Is%20Not%20Valid
              _)))
        (Variables|Default|SetInvestigateTransform (Transformation|GetWorldTransform _arrow1))
        (Variables|Default|SetIsBroken_2 true)
        (AI|Components|Blackboard|SetValueasObject (AI|GetBlackboard (Variables|Default|GetAI)) (Utilities|Name|MakeLiteralName "ObjectRef") _self)))))

(event OnSmartLinkReached(NavLink1)
  (params (MovingActor :type Actor%20Object%20Reference) (DestinationPoint :type Vector%20%28by%20ref%29 :default "0, 0, 0"))
  (bind _ai (Variables|Default|GetAI))
  (bind _capsulecomponent (Variables|/Script/Engine.Character|GetCapsuleComponent _ai))
  (Transformation|SetActorRotation _ai (Math|Rotator|MakeRotator 0.0 0.0 (.yaw (Math|Rotator|FindLookatRotation (Transformation|GetActorLocation _ai) (Transformation|GetActorLocation)))))
  (Collision|SetCollisionEnabled _capsulecomponent "NoCollision")
  (Utilities|FlowControl|Delay 0.6)
  (Collision|SetCollisionEnabled _capsulecomponent "QueryAndPhysics")
  (Utilities|FlowControl|RetriggerableDelay 0.5)
  (Collision|SetCollisionEnabled (Variables|Default|GetStaticMesh) "QueryAndPhysics"))

(event OnSmartLinkReached(NavLink2)
  (params (MovingActor :type Actor%20Object%20Reference) (DestinationPoint :type Vector%20%28by%20ref%29 :default "0, 0, 0"))
  (bind _ai (Variables|Default|GetAI))
  (bind _capsulecomponent (Variables|/Script/Engine.Character|GetCapsuleComponent _ai))
  (Transformation|SetActorRotation _ai (Math|Rotator|MakeRotator 0.0 0.0 (.yaw (Math|Rotator|FindLookatRotation (Transformation|GetActorLocation _ai) (Transformation|GetActorLocation)))))
  (Collision|SetCollisionEnabled _capsulecomponent "NoCollision")
  (Utilities|FlowControl|Delay 0.6)
  (Collision|SetCollisionEnabled _capsulecomponent "QueryAndPhysics")
  (Utilities|FlowControl|RetriggerableDelay 0.5)
  (Collision|SetCollisionEnabled (Variables|Default|GetStaticMesh) "QueryAndPhysics"))

(event EventBeginPlay
  (bind _navlink1 (Variables|Default|GetNavLink1))
  (bind _navlink2 (Variables|Default|GetNavLink2))
  (bind _returnvalue (Actor|GetActorOfClass "/Game/Blueprints/Characters/AI2/AI.AI_C"))
  (Variables|Default|SetAI _returnvalue)
  (if (Variables|Default|GetNavLinksInUse)
    (Utilities|FlowControl|Sequence
      (:then_0
        (Utilities|IsValid _navlink1
          (:Is%20Valid
            (Class|NavLinkProxy|SetSmartLinkEnabled _navlink1 false))))
      (:then_1
        (Utilities|IsValid _navlink2
          (:Is%20Valid
            (Class|NavLinkProxy|SetSmartLinkEnabled _navlink2 false)))))))

(fn ConstructionScript)