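; BP_PlayerArea is a trigger volume that makes the AI abandon its pursuit of the player on entering the area.
; If the overlapping AI is in a specific state and sees the player, it stops and plays an "it's a trap" animation.
; After the animation delay it starts a random task, regains movement, disables catching and clears its perception.
; Older BP_Neighbor logic toggling chase, catch and perception remains in the graph but never runs.
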(event OnComponentBeginOverlap(Box)
  (params (OverlappedComponent :type Primitive%20Component%20Object%20Reference) (OtherActor :type Actor%20Object%20Reference) (OtherComp :type Primitive%20Component%20Object%20Reference) (OtherBodyIndex :type Integer) (bFromSweep :type Boolean) (SweepResult :type Hit%20Result%20Structure%20%28by%20ref%29))
  (bind _asai (Utilities|Casting|CastToAI OtherActor))
  (bind _output_get (Variables|Default|SetAI _asai))
  (if (and (Utilities|Enum|Equal(Enum) (Variables|/Game/Blueprints/Characters/AI2/AI.AI_C|GetCurrentState _output_get) "NewEnumerator4") (Variables|/Game/Blueprints/Characters/AI2/AI.AI_C|GetCanSeePlayer _output_get))
    (Default|DisableMovement _asai)
    (Default|SetState _output_get "NewEnumerator7")
    (Variables|/Game/Blueprints/Characters/AI2/AI.AI_C|SetCanChase _output_get false)
    (Variables|/Game/Blueprints/Characters/AI2/AI.AI_C|SetCanHear _output_get false)
    (bind _anim_length (Default|PlayAnimAI _output_get "/Game/Neighbor/Animations/neighbour_lowpoly_Anim_rig_it_s_a_trap_.neighbour_lowpoly_Anim_rig_it_s_a_trap_" true))
    (Utilities|FlowControl|Delay _anim_length)
    (Default|RandomTask _output_get)
    (Default|SetState _output_get "NewEnumerator0")
    (Default|EnableMovement _output_get)
    (Default|DisableCatch _output_get)
    (Utilities|FlowControl|Delay 0.5)
    (Variables|/Game/Blueprints/Characters/AI2/AI.AI_C|SetCanSeePlayer _output_get false)
    (Class|AIPerceptionComponent|ForgetAll (Variables|/Game/Blueprints/Characters/AI2/AI.AI_C|GetAIPerception _output_get))))

(fn ConstructionScript)