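; Police car Blueprint that flashes alternating red and blue roof lights.
; BeginPlay waits a random interval of up to two seconds, then calls CustomTick, which re-registers itself on a looping timer in place of the empty Tick.
; Delays and a DoOnce gate pace each cycle, swapping materials on two cubes and toggling two point lights so only one side is lit at a time.
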(event Custom|CustomTick
  (Utilities|Time|SetTimerbyEvent (delegate Custom|CustomTick) 0.1 true)
  (Utilities|FlowControl|Delay 0.4)
  (Utilities|FlowControl|DoOnce false :!label _label
    (:Completed
      (Rendering|Material|SetMaterial (Variables|Default|GetCube1) 0 "/Game/Materials/111Base.111Base")
      (Rendering|Material|SetMaterial (Variables|Default|GetCube2) 0 "/Game/Materials/111blue.111blue")
      (Rendering|SetVisibility (Variables|Default|GetPointLight1) true false)
      (Rendering|SetVisibility (Variables|Default|GetPointLight) false false)
      (Utilities|FlowControl|Delay 0.2)
      (Rendering|Material|SetMaterial (Variables|Default|GetCube2) 0 "/Game/Materials/111Base.111Base")
      (Rendering|Material|SetMaterial (Variables|Default|GetCube1) 0 "/Game/Materials/111Red.111Red")
      (Rendering|SetVisibility (Variables|Default|GetPointLight) true false)
      (Rendering|SetVisibility (Variables|Default|GetPointLight1) false false)
      (goto _label Reset))))

(event EventBeginPlay
  (Utilities|FlowControl|Delay (Math|Random|RandomFloatinRange 2.0 0.0))
  (CallFunction|CustomTick))

(event EventTick
  (params (DeltaSeconds :type Float%20%28single-precision%29)))

(fn ConstructionScript)