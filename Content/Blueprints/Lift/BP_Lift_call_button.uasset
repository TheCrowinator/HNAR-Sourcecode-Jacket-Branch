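; BP_Lift_call_button is a lift call button that summons its referenced Lift to the button's floor.
; CallLift acts when given the button mesh: it plays a click sound and, if the lift is powered, either opens the lift and floor doors or sets the target floor and starts MoveElevator.
; When the lift moves, a DoOnce lights the button material, then restores it after a delay scaled by travel distance and lift time.
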(event Custom|Call%20Lift
  (params (Component :type Primitive%20Component%20Object%20Reference))
  (bind _lift (Variables|Default|GetLift))
  (bind _staticmesh1 (Variables|Default|GetStaticMesh1))
  (bind _floor (Variables|Default|GetFloor))
  (if (== Component (Variables|Default|GetStaticMesh1))
    (Audio|PlaySoundatLocation "/Game/Sounds/train_room_button.train_room_button" (Transformation|GetActorLocation) "0, 0, 0" 1.0 1.0 0.0 "/Game/Sounds/Attenuation/ItemAtten.ItemAtten" 0 0)
    (if (Variables|/Game/Blueprints/Lift/BP_Lift.BP_Lift_C|GetPowered? _lift)
      (if (== (Variables|/Game/Blueprints/Lift/BP_Lift.BP_Lift_C|GetCurrentFloor _lift) _floor)
        (Default|OpenDoors _lift)
        (Default|Open (Utilities|Array|Get(acopy) (Variables|/Game/Blueprints/Lift/BP_Lift.BP_Lift_C|GetLiftDoors _lift) _floor))
        (else
          (Variables|/Game/Blueprints/Lift/BP_Lift.BP_Lift_C|SetFloorPressed _lift _floor)
          (Default|MoveElevator _lift)
          (Utilities|FlowControl|DoOnce false :!label _label
            (:Completed
              (Rendering|Material|SetMaterial _staticmesh1 0 "/Game/Materials/111White1.111White1")
              (Utilities|FlowControl|Delay 1.0)
              (Utilities|FlowControl|Delay (* (Variables|/Game/Blueprints/Lift/BP_Lift.BP_Lift_C|GetDistance _lift) (Variables|/Game/Blueprints/Lift/BP_Lift.BP_Lift_C|GetLiftTime _lift)))
              (Rendering|Material|SetMaterial _staticmesh1 0 "/Game/CubeMaterialOverride.CubeMaterialOverride")
              (goto _label Reset))))))))

(event EventBeginPlay)

(event Collision|EventActorBeginOverlap
  (params (OtherActor :type Actor%20Object%20Reference)))

(event EventTick
  (params (DeltaSeconds :type Float%20%28single-precision%29)))

(fn ConstructionScript)