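; Sliding double door for a lift that opens and closes by moving two static mesh panels apart and together along local X.
; Open and Close are gated by CanOpen, update IsOpen, and drive both panels with timed MoveComponentTo calls.
; Each direction has its own DoOnce, reset from the second panel's move branch.
; OpenClose toggles between the two based on IsOpen.
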(event Custom|Open
  (if (Variables|Default|GetCanOpen?)
    (Utilities|FlowControl|DoOnce false :!label _label
      (:Completed
        (Variables|Default|SetIsOpen true)
        (Utilities|FlowControl|Sequence
          (:then_0
            (Components|MoveComponentTo (Variables|Default|GetStaticMesh1) "82.000000, 0, 0" "0, 0, 0" false false 1.0 false))
          (:then_1
            (Components|MoveComponentTo (Variables|Default|GetStaticMesh2) "-82.000000, 0, 0" "0, 0, 0" false false 1.0 false)
            (goto _label Reset)))))))

(event Custom|Close
  (if (Variables|Default|GetCanOpen?)
    (Utilities|FlowControl|DoOnce false :!label _label
      (:Completed
        (Variables|Default|SetIsOpen false)
        (Utilities|FlowControl|Sequence
          (:then_0
            (Components|MoveComponentTo (Variables|Default|GetStaticMesh1) "25.000000, 0, 0" "0, 0, 0" false false 1.0 false))
          (:then_1
            (Components|MoveComponentTo (Variables|Default|GetStaticMesh2) "-25.000000, 0, 0" "0, 0, 0" false false 1.0 false)
            (goto _label Reset)))))))

(event Custom|OpenClose
  (if (Variables|Default|GetIsOpen)
    (CallFunction|Close)
    (else
      (CallFunction|Open))))

(event EventBeginPlay)

(event Collision|EventActorBeginOverlap
  (params (OtherActor :type Actor%20Object%20Reference)))

(event EventTick
  (params (DeltaSeconds :type Float%20%28single-precision%29)))

(fn ConstructionScript)