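; Powered four-floor elevator that a first-person player operates with buttons while standing inside the car.
; A press lights the button and moves the car to that floor's actor location over a distance-scaled time, with audio and an enabled collision box.
; Car doors and per-floor LiftDoors close before travel and open on arrival, with DoOnce gates blocking repeat requests.
; A fast looping timer drives a Tick event that switches lights with power.
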(event OnComponentBeginOverlap(Inside)
  (params (OverlappedComponent :type Primitive%20Component%20Object%20Reference) (OtherActor :type Actor%20Object%20Reference) (OtherComp :type Primitive%20Component%20Object%20Reference) (OtherBodyIndex :type Integer) (bFromSweep :type Boolean) (SweepResult :type Hit%20Result%20Structure%20%28by%20ref%29))
  (Utilities|Casting|CastToFirstPersonCharacter OtherActor)
  (Variables|Default|SetCanPress true))

(event OnComponentEndOverlap(Inside)
  (params (OverlappedComponent :type Primitive%20Component%20Object%20Reference) (OtherActor :type Actor%20Object%20Reference) (OtherComp :type Primitive%20Component%20Object%20Reference) (OtherBodyIndex :type Integer))
  (Utilities|Casting|CastToFirstPersonCharacter OtherActor)
  (Variables|Default|SetCanPress false))

(event Custom|PressedButton
  (params (Component :type Primitive%20Component%20Object%20Reference))
  (bind _button1 (Variables|Default|Getbutton1))
  (bind _button2 (Variables|Default|Getbutton2))
  (bind _button3 (Variables|Default|Getbutton3))
  (bind _button4 (Variables|Default|Getbutton4))
  (if (Variables|Default|GetCanPress)
    (if (Variables|Default|GetPowered?)
      (if (== Component _button1)
        (if (not (Variables|Default|GetIsMoving))
          (Variables|Default|SetFloorPressed 0)
          (Rendering|Material|SetScalarParameterValueonMaterials _button1 "Emission" 1.0)
          (Utilities|FlowControl|DoOnce false :!label _label
            (:Completed
              (Variables|Default|SetIsMoving true)
              (CallFunction|MoveElevator)
              (Audio|PlaySoundatLocation "/Game/Sounds/train_room_button.train_room_button" (Transformation|GetWorldLocation Component) "0, 0, 0" 1.0 1.0 0.0 "/Game/Sounds/Attenuation/ItemAtten.ItemAtten" 0 0)
              (Collision|SetCollisionEnabled (Variables|Default|GetBox) "QueryAndPhysics"))))
        (elif (== Component _button2)
          (if (not (Variables|Default|GetIsMoving))
            (Variables|Default|SetFloorPressed 1)
            (Rendering|Material|SetScalarParameterValueonMaterials _button2 "Emission" 1.0)
            (goto _label))
          (elif (== Component _button3)
            (if (not (Variables|Default|GetIsMoving))
              (Variables|Default|SetFloorPressed 2)
              (Rendering|Material|SetScalarParameterValueonMaterials _button3 "Emission" 1.0)
              (goto _label))
            (elif (== Component _button4)
              (if (not (Variables|Default|GetIsMoving))
                (Variables|Default|SetFloorPressed 3)
                (Rendering|Material|SetScalarParameterValueonMaterials _button4 "Emission" 1.0)
                (goto _label)))))))))

(event Custom|MoveElevator
  (bind _audio (Variables|Default|GetAudio))
  (if (Variables|Default|GetPowered?)
    (if (== (Variables|Default|GetFloorPressed) (Variables|Default|GetCurrentFloor))
      (Variables|Default|SetIsMoving false :!label _label)
      (Utilities|FlowControl|DoOnce false) ; enters at Reset
      (else
        (Utilities|FlowControl|DoOnce false :!label _label_2
          (:Completed
            (Utilities|FlowControl|Sequence
              (:then_0
                (Default|Close (Utilities|Array|Get(acopy) (Variables|Default|GetLiftDoors) (Variables|Default|GetCurrentFloor)))
                (CallFunction|CloseDoors)
                (Utilities|FlowControl|Delay 1.0)
                (Audio|Components|Audio|Play _audio 0.0)
                (Audio|Components|Audio|Play (Variables|Default|GetElev1_Cue) 0.8)
                (Components|MoveComponentTo (Variables|Default|GetStaticMesh) (Transformation|GetActorLocation (Utilities|Array|Get(acopy) (Variables|Default|GetFloors) (Variables|Default|GetFloorPressed))) "0, 0, 0" false false (* (Variables|Default|GetDistance) (Variables|Default|GetLiftTime)) false)
                (Audio|Components|Audio|Stop _audio)
                (bind _output_get (Variables|Default|SetCurrentFloor (Variables|Default|GetFloorPressedTEMP)))
                (Variables|Default|SetFloorPressed -1)
                (Rendering|Material|SetScalarParameterValueonMaterials (Variables|Default|Getbutton2) "Emission" 0.0)
                (Default|Open (Utilities|Array|Get(acopy) (Variables|Default|GetLiftDoors) _output_get))
                (CallFunction|OpenDoors)
                (Collision|SetCollisionEnabled (Variables|Default|GetBox) "NoCollision")
                (Utilities|FlowControl|Delay 1.5)
                (Utilities|FlowControl|Sequence
                  (:then_0
                    (goto _label))
                  (:then_1
                    (goto _label_2 Reset))))
              (:then_1
                (if (> (- (Variables|Default|GetFloorPressed) (Variables|Default|GetCurrentFloor)) (Variables|Default|GetCurrentFloor))
                  (bind _output_get_2 (Variables|Default|SetDistance (- (Variables|Default|GetFloorPressed) (Variables|Default|GetCurrentFloor)) :!label _label_3))
                  (Development|PrintString (Utilities|String|ToString(Integer) _output_get_2))
                  (elif (== (- (Variables|Default|GetFloorPressed) (Variables|Default|GetCurrentFloor)) 1)
                    (goto _label_3)
                    (else
                      (bind _output_get_3 (Variables|Default|SetDistance (* (- (Variables|Default|GetFloorPressed) (Variables|Default|GetCurrentFloor)) -1)))
                      (Development|PrintString (Utilities|String|ToString(Integer) _output_get_3))))))
              (:then_2
                (Variables|Default|SetFloorPressedTEMP (Variables|Default|GetFloorPressed))))))))))

(event Custom|OpenDoors
  (Utilities|FlowControl|Sequence
    (:then_0
      (Components|MoveComponentTo (Variables|Default|Getdoor) "75.000000,106.000000,-3.000000" "0, 0, 0" false false 1.0 false))
    (:then_1
      (Components|MoveComponentTo (Variables|Default|Getdoor1) "-75.000000,106.000000,-3.000000" "0, 0, 0" false false 1.0 false))))

(event Custom|CloseDoors
  (Utilities|FlowControl|Sequence
    (:then_0
      (Components|MoveComponentTo (Variables|Default|Getdoor) "25.000000,106.000000,-3.000000" "0, 0, 0" false false 1.0 false))
    (:then_1
      (Components|MoveComponentTo (Variables|Default|Getdoor1) "-25.000000,106.000000,-3.000000" "0, 0, 0" false false 1.0 false))))

(event Custom|Tick
  (bind _light1 (Variables|Default|GetLight1))
  (if (Variables|Default|GetPowered?)
    (Utilities|FlowControl|DoOnce false :!label _label
      (:Completed
        (Rendering|SetVisibility _light1 true false)
        (goto _label_2 Reset)))
    (else
      (Utilities|FlowControl|DoOnce false :!label _label_2
        (:Completed
          (Rendering|SetVisibility _light1 false false)
          (goto _label Reset))))))

(event EventBeginPlay
  (Utilities|Time|SetTimerbyEvent (delegate Custom|Tick) 0.01 true)
  (Collision|SetCollisionEnabled (Variables|Default|GetBox) "NoCollision"))

(fn ConstructionScript)