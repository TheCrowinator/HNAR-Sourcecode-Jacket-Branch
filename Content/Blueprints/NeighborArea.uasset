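; NeighborArea is a trigger volume that plays scary inside ambience while the player character is within its box.
; Entering spawns the 2D sound through a DoOnce gate; leaving fades it out, then resets the gate after a short delay.
; BeginPlay caches the BP_Neighbor actor, which the graph never uses.
; Disconnected nodes hold an unused two-track ambience variant.
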(event OnComponentBeginOverlap(Box)
  (params (OverlappedComponent :type Primitive%20Component%20Object%20Reference) (OtherActor :type Actor%20Object%20Reference) (OtherComp :type Primitive%20Component%20Object%20Reference) (OtherBodyIndex :type Integer) (bFromSweep :type Boolean) (SweepResult :type Hit%20Result%20Structure%20%28by%20ref%29))
  (Utilities|Casting|CastToFirstPersonCharacter OtherActor)
  (Utilities|FlowControl|DoOnce false
    (:Completed
      (bind _returnvalue (Audio|SpawnSound2D "/Game/Sounds/inside_scary_Cue.inside_scary_Cue" 1.0 1.0 0.0 0)))))

(event OnComponentEndOverlap(Box)
  (params (OverlappedComponent :type Primitive%20Component%20Object%20Reference) (OtherActor :type Actor%20Object%20Reference) (OtherComp :type Primitive%20Component%20Object%20Reference) (OtherBodyIndex :type Integer))
  (Utilities|Casting|CastToFirstPersonCharacter OtherActor)
  (Audio|Components|Audio|FadeOut (stale OnComponentBeginOverlap(Box) _returnvalue) 0.5 0.0 "Linear" :!class /Script/Engine.AudioComponent)
  (Utilities|FlowControl|Delay 0.5)
  (Utilities|FlowControl|DoOnce false) ; enters at Reset
)

(event EventBeginPlay
  (bind _returnvalue (Actor|GetActorOfClass "/Game/Blueprints/Characters/NeighborAI/BP_Neighbor.BP_Neighbor_C"))
  (Variables|Default|SetSosed _returnvalue))

(fn ConstructionScript)