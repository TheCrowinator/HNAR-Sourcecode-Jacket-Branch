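; Double door actor with two independently toggled leaves, lock sounds, AI passage and an optional chair barricade.
; OpenClose swings the chosen leaf with paired MoveComponentTo calls that cancel each other, relaxing collision during motion.
; A smart nav link lets permitted AI pass unbarricaded doors, timing Door1's movement with delays.
; BreakThroughChair plays a push animation, releases the chair to physics, bursts both leaves open, may change AI state, then recloses them.
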(event OnSmartLinkReached(NavLink)
  (params (MovingActor :type Actor%20Object%20Reference) (DestinationPoint :type Vector%20%28by%20ref%29 :default "0, 0, 0"))
  (bind _door1 (Variables|Default|GetDoor1))
  (bind _door1_2 (Variables|Default|GetDoor1))
  (bind _asai (Utilities|Casting|CastToAI MovingActor))
  (bind _output_get (Variables|Default|SetAI _asai))
  (if (Variables|Default|GetCanAIOpen?)
    (if (not (Variables|Default|GetIsLockedWithChair?))
      (if (Variables|Default|GetOpen_1)
        (if (not (Variables|Default|GetOpen))
          (if (Variables|Default|GetOutwards?)
            (Components|Animation|PlayAnimation (Variables|/Script/Engine.Character|GetMesh _output_get) "/Game/Neighbor/Animations/neighbour_lowpoly_Anim_rig_open_double_door_outward.neighbour_lowpoly_Anim_rig_open_double_door_outward" false)
            (else
              (Components|Animation|PlayAnimation (Variables|/Script/Engine.Character|GetMesh _output_get) "/Game/Neighbor/Animations/neighbour_lowpoly_Anim_rig_open_double_door_inward.neighbour_lowpoly_Anim_rig_open_double_door_inward" false)))
          (Utilities|FlowControl|Delay 0.94)
          (Utilities|FlowControl|Delay 1.5 :!label _label)
          (Collision|SetCollisionEnabled _door1_2 "PhysicsOnly")
          (Components|MoveComponentTo _door1_2 "170.000000,10.000000,0.000000" "0,-180.000000, 0" false false 0.5 false)
          (Collision|SetCollisionEnabled _door1_2 "QueryAndPhysics")
          (Variables|Default|SetOpen_1 false))
        (else
          (Pawn|Components|CharacterMovement|DisableMovement (Variables|/Script/Engine.Character|GetCharacterMovement _output_get))
          (Utilities|FlowControl|Delay 0.4)
          (Variables|Default|SetOpen_1 true)
          (Collision|SetCollisionEnabled _door1 "PhysicsOnly")
          (Components|MoveComponentTo _door1 "170.000000,10.000000, 0" "0,-280.000000,0.000000" false false 0.5 false)
          (Collision|SetCollisionEnabled _door1 "QueryAndPhysics")
          (Utilities|FlowControl|Delay 0.54)
          (Pawn|Components|CharacterMovement|SetMovementMode (Variables|/Script/Engine.Character|GetCharacterMovement _output_get) "MOVE_Walking" 0)
          (Components|Animation|SetAnimationMode (Variables|/Script/Engine.Character|GetMesh _output_get) "AnimationBlueprint")
          (goto _label))))))

(event EventBeginPlay
  (bind _door1 (Variables|Default|GetDoor1))
  (bind _selectchair (Variables|Default|GetSelectChair))
  (|CallParentFunction)
  (Utilities|FlowControl|Sequence
    (:then_0
      (if (Variables|Default|GetOpen_1)
        (Transformation|SetRelativeLocationAndRotation _door1 "170.000000,10.000000, 0" "0,-280.000000, 0" false false)
        (else
          (Transformation|SetRelativeLocationAndRotation _door1 "170.000000,10.000000, 0" (Variables|Default|GetNew%20Rotation) false false))))
    (:then_1
      (if (Variables|Default|GetIsLockedWithChair?)
        (Utilities|FlowControl|Delay 0.02)
        (CallFunction|SetChair (Variables|Default|GetSelectChair))))
    (:then_2
      (Utilities|IsValid _selectchair
        (:Is%20Valid
          (Variables|/Game/Blueprints/PickUpObjects/BP_Chair.BP_Chair_C|SetDoor _selectchair self))))))

(event EventBreakThroughChair
  (bind _ai (Variables|Default|GetAI))
  (bind _door1 (Variables|Default|GetDoor1))
  (bind _mesh (Variables|/Script/Engine.Character|GetMesh _ai))
  (Components|Animation|SetAnimationMode _mesh "AnimationSingleNode")
  (Components|Animation|PlayAnimation _mesh "/Game/Neighbor/Montages/pushdoor.pushdoor" false)
  (Utilities|FlowControl|Delay 4.2)
  (Variables|Default|SetOpen true)
  (Physics|SetSimulatePhysics (Variables|/Game/Blueprints/PickUpObjects/BP_Interactable.BP_Interactable_C|GetStaticMesh (Variables|Default|GetSelectChair)) true)
  (Variables|Default|SetSelectChair 0)
  (Utilities|FlowControl|Sequence
    (:then_0
      (Components|MoveComponentTo (Variables|Default|GetDoor) (Variables|Default|GetDoorOpen_Location) (Variables|Default|GetDoorOpen_Rotation) false false 0.1 false)
      (Variables|Default|SetOpen true)
      (Utilities|FlowControl|Delay 0.2)
      (Components|Animation|SetAnimationMode _mesh "AnimationBlueprint")
      (Pawn|Components|CharacterMovement|SetMovementMode (Variables|/Script/Engine.Character|GetCharacterMovement _ai) "MOVE_Walking" 0)
      (if (Utilities|Enum|Equal(Enum) (Variables|/Game/Blueprints/Characters/AI2/AI.AI_C|GetCurrentState _ai) "NewEnumerator0")
        (Class|BlackboardComponent|SetValueasInt (AI|GetBlackboard _ai) (Utilities|Name|MakeLiteralName "HuntTask") 1)
        (Default|SetState _ai "NewEnumerator2"))
      (Utilities|FlowControl|Delay 0.5)
      (Utilities|FlowControl|Sequence
        (:then_0
          (Components|MoveComponentTo _door1 "170.000000,10.000000, 0" "0,-180.000000, 0" false false 0.5 false)
          (Audio|PlaySoundatLocation (Variables|Default|GetCloseSound) (Transformation|GetActorLocation) "0, 0, 0" 1.0 1.0 0.0 "/Game/Sounds/Attenuation/DoorSoundAttenuation.DoorSoundAttenuation" 0 0)
          (Collision|SetCollisionEnabled _door1 "QueryAndPhysics")
          (Variables|Default|SetOpen_1 false))
        (:then_1
          (Components|MoveComponentTo (Variables|Default|GetDoor) (Variables|Default|GetDoorClose_Location) (Variables|Default|GetDoorClose_Rotation) false false 0.5 false)
          (Variables|Default|SetOpen false))))
    (:then_1
      (Components|MoveComponentTo (Variables|Default|GetDoor1) "170.000000,10.000000, 0" "0,-280.000000, 0" false false 0.1 false)
      (Variables|Default|SetOpen_1 true))))

(event EventOpenClose
  (params (Component :type Primitive%20Component%20Object%20Reference))
  (bind _door1 (Variables|Default|GetDoor1))
  (bind _door (Variables|Default|GetDoor))
  (if (== Component (Variables|Default|GetDoor))
    (if (Variables|Default|GetLocked)
      (Audio|PlaySoundatLocation "/Game/Sounds/LockedDoor_Cue.LockedDoor_Cue" (Transformation|GetWorldLocation (Variables|Default|GetScene)) "0, 0, 0" 1.0 1.0 0.0 "/Game/Sounds/Attenuation/DoorSoundAttenuation.DoorSoundAttenuation" 0 0 :!label _label)
      (elif (Variables|Default|GetOpen)
        (Utilities|FlowControl|Sequence
          (:then_0
            (Collision|SetCollisionEnabled _door "PhysicsOnly")
            (Components|MoveComponentTo _door "-1.000000,10.000000, 0" "0, 0, 0" false false 0.5 false :!label _label_2)
            (Audio|SpawnSoundatLocation (Variables|Default|GetCloseSound) (Transformation|GetWorldLocation (Variables|Default|GetScene)) "0, 0, 0" 1.0 1.0 0.0 "/Game/Sounds/Attenuation/DoorSoundAttenuation.DoorSoundAttenuation" 0)
            (Collision|SetCollisionEnabled _door "QueryAndPhysics")
            (Variables|Default|SetOpen false))
          (:then_1
            (goto _label_3 Stop)))
        (else
          (Utilities|FlowControl|Sequence
            (:then_0
              (Variables|Default|SetOpen true)
              (Collision|SetCollisionEnabled _door "PhysicsOnly")
              (Components|MoveComponentTo _door "-1.000000,10.000000, 0" "0,100.000000, 0" false false 0.5 false :!label _label_3)
              (Collision|SetCollisionEnabled _door "QueryAndPhysics"))
            (:then_1
              (goto _label_2 Stop))
            (:then_2
              (Audio|SpawnSoundatLocation "/Game/Sounds/Entrance_Door_Open.Entrance_Door_Open" (Transformation|GetWorldLocation (Variables|Default|GetScene)) "0, 0, 0" 1.0 1.0 0.0 "/Game/Sounds/Attenuation/DoorSoundAttenuation.DoorSoundAttenuation" 0))))))
    (elif (== Component (Variables|Default|GetDoor1))
      (if (Variables|Default|GetLocked)
        (goto _label)
        (elif (Variables|Default|GetOpen_1)
          (Utilities|FlowControl|Sequence
            (:then_0
              (Collision|SetCollisionEnabled _door1 "PhysicsOnly")
              (Components|MoveComponentTo _door1 "170.000000,10.000000, 0" "0,-180.000000, 0" false false 0.5 false :!label _label_4)
              (Audio|SpawnSoundatLocation (Variables|Default|GetCloseSound) (Transformation|GetWorldLocation (Variables|Default|GetScene)) "0, 0, 0" 1.0 1.0 0.0 "/Game/Sounds/Attenuation/DoorSoundAttenuation.DoorSoundAttenuation" 0)
              (Collision|SetCollisionEnabled _door1 "QueryAndPhysics")
              (Variables|Default|SetOpen_1 false))
            (:then_1
              (goto _label_5 Stop)))
          (else
            (Utilities|FlowControl|Sequence
              (:then_0
                (Variables|Default|SetOpen_1 true)
                (Collision|SetCollisionEnabled _door1 "PhysicsOnly")
                (Components|MoveComponentTo _door1 "170.000000,10.000000, 0" "0,-280.000000, 0" false false 0.5 false :!label _label_5)
                (Collision|SetCollisionEnabled _door1 "QueryAndPhysics"))
              (:then_1
                (goto _label_4 Stop))
              (:then_2
                (Audio|SpawnSoundatLocation "/Game/Sounds/Entrance_Door_Open.Entrance_Door_Open" (Transformation|GetWorldLocation (Variables|Default|GetScene)) "0, 0, 0" 1.0 1.0 0.0 "/Game/Sounds/Attenuation/DoorSoundAttenuation.DoorSoundAttenuation" 0)))))))))

(fn ConstructionScript
  (|CallParentFunction))