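; BP_Button is an interactable button that plays a switch sound and sinks when pressed, granting a trophy in the Limbo level.
; Interact checks Pressed, then restarts a timeline that lowers the Cylinder along its Z axis.
; Timeline updates also check the level name and pass ID and Name to the FirstPersonCharacter's AddTrophy through a DoOnce.
; The node setting Pressed is disconnected, so this graph never blocks repeat presses.
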(event Custom|Interact
  (if (not (Variables|Default|GetPressed))
    (Audio|PlaySound2D "/Game/Sounds/train_switch_on.train_switch_on" 1.0 1.0 0.0 0 0)
    (bind _press (Timeline|Press PlayFromStart)
      (:Update
        (Transformation|SetRelativeLocation (Variables|Default|GetCylinder) (Math|Vector|MakeVector 0.0 0.0 (Math|Float|Lerp 0.0 -8.0 _press)) false false)
        (bind _asfirst_person_character (Utilities|Casting|CastToFirstPersonCharacter (Game|GetPlayerCharacter 0)))
        (bind _returnvalue (Game|GetCurrentLevelName true))
        (if (Utilities|Enum|Equal(Enum) _returnvalue "Limbo")
          (Utilities|FlowControl|DoOnce false
            (:Completed
              (Default|AddTrophy _asfirst_person_character (Variables|Default|GetID) (Variables|Default|GetName)))))))))

(event EventBeginPlay)

(event Collision|EventActorBeginOverlap
  (params (OtherActor :type Actor%20Object%20Reference)))

(event EventTick
  (params (DeltaSeconds :type Float%20%28single-precision%29)))

(fn ConstructionScript)