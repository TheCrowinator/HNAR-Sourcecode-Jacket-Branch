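; Trash can pickup object that sets its socket from the player character's Trashcan socket and can be kicked by the neighbor AI.
; NeighborKick, guarded by a resettable DoOnce, freezes the AI, plays a kick animation and launches the mesh with a timed impulse before restoring movement and Animation Blueprint mode.
; Box1 overlaps track whether the AI is inside the can, in which case it is nudged along world X by teleport after the kick.
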(event OnComponentBeginOverlap(Box1)
  (params (OverlappedComponent :type Primitive%20Component%20Object%20Reference) (OtherActor :type Actor%20Object%20Reference) (OtherComp :type Primitive%20Component%20Object%20Reference) (OtherBodyIndex :type Integer) (bFromSweep :type Boolean) (SweepResult :type Hit%20Result%20Structure%20%28by%20ref%29))
  (Utilities|Casting|CastToAI OtherActor)
  (Variables|Default|SetInTrashCan true))

(event OnComponentEndOverlap(Box1)
  (params (OverlappedComponent :type Primitive%20Component%20Object%20Reference) (OtherActor :type Actor%20Object%20Reference) (OtherComp :type Primitive%20Component%20Object%20Reference) (OtherBodyIndex :type Integer))
  (Utilities|Casting|CastToAI OtherActor)
  (Variables|Default|SetInTrashCan false))

(event EventBeginPlay
  (|CallParentFunction) ; This node is disabled and will not be called.\nDrag off pins to build functionality.
)

(event Collision|EventActorBeginOverlap
  (params (OtherActor :type Actor%20Object%20Reference)))

(event EventTick
  (params (DeltaSeconds :type Float%20%28single-precision%29)))

(event EventSetSocket
  (bind _asfirst_person_character (Utilities|Casting|CastToFirstPersonCharacter (Game|GetPlayerCharacter 0)))
  (Variables|Default|SetSocket (Variables|/Game/Blueprints/Characters/FirstPersonBP/Blueprints/FirstPersonCharacter.FirstPersonCharacter_C|GetTrashcan _asfirst_person_character)))

(event EventNeighborKick
  (params (AI :type AI%20Object%20Reference))
  (bind _mesh (Variables|/Script/Engine.Character|GetMesh AI))
  (bind _returnvalue (Transformation|GetWorldLocation _mesh))
  (Utilities|FlowControl|DoOnce false :!label _label
    (:Completed
      (Default|DisableMovement AI)
      (Default|PlayAnimAI AI "/Game/Neighbor/Animations/neighbour_lowpoly_Anim_rig_kick.neighbour_lowpoly_Anim_rig_kick" false)
      (Utilities|FlowControl|Delay 0.55)
      (Physics|AddImpulse (Variables|Default|GetStaticMesh) (Variables|Default|GetKickImpulse) "None" true)
      (Utilities|FlowControl|Delay 0.81)
      (Default|EnableMovement AI)
      (Components|Animation|SetAnimationMode (Variables|/Script/Engine.Character|GetMesh AI) "AnimationBlueprint")
      (if (Variables|Default|GetInTrashCan)
        (Transformation|Teleport AI (Math|Vector|MakeVector (+ (.x _returnvalue) 7e+01) (.y _returnvalue) (.z _returnvalue)) "0, 0, 0")
        (goto _label Reset)
        (else
          (goto _label Reset))))))

(fn ConstructionScript
  (|CallParentFunction))