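; BP_Radio is a radio object, likely a pickup, that toggles its audio on and off and can lure the AI.
; Interact and Use share one toggle; switching on also reports a tagged noise event and writes the radio into the AI's blackboard as ObjectRef.
; AIOnOff toggles it without alerting the AI.
; SetSocket takes its socket from the first-person character's Radio reference.
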(event Custom|AI%20OnOff
  (bind _radio (Variables|Default|GetRadio))
  (if (Variables|Default|GetOnOff)
    (Variables|Default|SetOnOff false)
    (Audio|PlaySoundatLocation "/Game/Sounds/switch_off_Cue.switch_off_Cue" (Transformation|GetActorLocation) "0, 0, 0" 0.25 1.0 0.0 "/Game/Sounds/Attenuation/ItemAtten.ItemAtten" 0 0)
    (Audio|Components|Audio|Stop _radio)
    (else
      (Variables|Default|SetOnOff true)
      (Audio|PlaySoundatLocation "/Game/Sounds/switch_off_Cue.switch_off_Cue" (Transformation|GetActorLocation) "0, 0, 0" 0.25 1.0 0.0 "/Game/Sounds/Attenuation/ItemAtten.ItemAtten" 0 0)
      (Audio|Components|Audio|Play _radio 0.0))))

(event EventBeginPlay
  (|CallParentFunction) ; This node is disabled and will not be called.\nDrag off pins to build functionality.
)

(event Collision|EventActorBeginOverlap
  (params (OtherActor :type Actor%20Object%20Reference)))

(event EventTick
  (params (DeltaSeconds :type Float%20%28single-precision%29)))

(event EventSetSocket
  (bind _asfirst_person_character (Utilities|Casting|CastToFirstPersonCharacter (Game|GetPlayerCharacter 0)))
  (Variables|Default|SetSocket (Variables|/Game/Blueprints/Characters/FirstPersonBP/Blueprints/FirstPersonCharacter.FirstPersonCharacter_C|GetRadio _asfirst_person_character)))

(event EventInteract
  (bind _returnvalue (Transformation|GetActorLocation))
  (bind _radio (Variables|Default|GetRadio))
  (if (Variables|Default|GetOnOff)
    (Variables|Default|SetOnOff false)
    (Audio|PlaySoundatLocation "/Game/Sounds/switch_off_Cue.switch_off_Cue" (Transformation|GetActorLocation) "0, 0, 0" 0.25 1.0 0.0 "/Game/Sounds/Attenuation/ItemAtten.ItemAtten" 0 0)
    (Audio|Components|Audio|Stop _radio)
    (else
      (Variables|Default|SetOnOff true)
      (Audio|PlaySoundatLocation "/Game/Sounds/switch_off_Cue.switch_off_Cue" _returnvalue "0, 0, 0" 0.25 1.0 0.0 "/Game/Sounds/Attenuation/ItemAtten.ItemAtten" 0 0)
      (Audio|Components|Audio|Play _radio 0.0)
      (Class|AISenseHearing|ReportNoiseEvent _returnvalue 3.0 self 5e+02 "Radio")
      (bind _returnvalue_2 (Actor|GetActorOfClass "/Game/Blueprints/Characters/AI2/AI.AI_C"))
      (Utilities|IsValid _returnvalue_2
        (:Is%20Valid
          (AI|Components|Blackboard|SetValueasObject (AI|GetBlackboard _returnvalue_2) (Utilities|Name|MakeLiteralName "ObjectRef") self))))))

(event EventUse
  (bind _returnvalue (Transformation|GetActorLocation))
  (bind _radio (Variables|Default|GetRadio))
  (if (Variables|Default|GetOnOff)
    (Variables|Default|SetOnOff false)
    (Audio|PlaySoundatLocation "/Game/Sounds/switch_off_Cue.switch_off_Cue" (Transformation|GetActorLocation) "0, 0, 0" 0.25 1.0 0.0 "/Game/Sounds/Attenuation/ItemAtten.ItemAtten" 0 0)
    (Audio|Components|Audio|Stop _radio)
    (else
      (Variables|Default|SetOnOff true)
      (Audio|PlaySoundatLocation "/Game/Sounds/switch_off_Cue.switch_off_Cue" _returnvalue "0, 0, 0" 0.25 1.0 0.0 "/Game/Sounds/Attenuation/ItemAtten.ItemAtten" 0 0)
      (Audio|Components|Audio|Play _radio 0.0)
      (Class|AISenseHearing|ReportNoiseEvent _returnvalue 3.0 self 5e+02 "Radio")
      (bind _returnvalue_2 (Actor|GetActorOfClass "/Game/Blueprints/Characters/AI2/AI.AI_C"))
      (Utilities|IsValid _returnvalue_2
        (:Is%20Valid
          (AI|Components|Blackboard|SetValueasObject (AI|GetBlackboard _returnvalue_2) (Utilities|Name|MakeLiteralName "ObjectRef") self))))))

(fn ConstructionScript
  (|CallParentFunction))