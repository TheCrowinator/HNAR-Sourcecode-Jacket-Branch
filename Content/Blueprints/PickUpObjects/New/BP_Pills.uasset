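; BP_Pills is a pickup item that lets the first-person player poison milk meant for the AI.
; On SetSocket it takes the character's Apple value as its socket.
; On Use it runs the character's short visibility trace, and if that hits an unpoisoned BP_MilkForAI, it poisons it, plays a hit sound there and destroys itself.
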(event EventBeginPlay
  (|CallParentFunction) ; This node is disabled and will not be called.\nDrag off pins to build functionality.
)

(event Collision|EventActorBeginOverlap
  (params (OtherActor :type Actor%20Object%20Reference)))

(event EventTick
  (params (DeltaSeconds :type Float%20%28single-precision%29)))

(event EventSetSocket
  (bind _asfirst_person_character (Utilities|Casting|CastToFirstPersonCharacter (Game|GetPlayerCharacter 0)))
  (Variables|Default|SetSocket (Variables|/Game/Blueprints/Characters/FirstPersonBP/Blueprints/FirstPersonCharacter.FirstPersonCharacter_C|GetApple _asfirst_person_character)))

(event EventUse
  (bind _asfirst_person_character (Utilities|Casting|CastToFirstPersonCharacter (Game|GetPlayerCharacter 0)))
  (bind (_out_hit _return_value) (Default|Trace _asfirst_person_character "TraceTypeQuery1" "None" 2.5e+02))
  (if _return_value
    (bind _asbp_milk_for_ai (Utilities|Casting|CastToBP_MilkForAI (.HitActor (Collision|BreakHitResult _out_hit))))
    (if (not (Variables|/Game/Blueprints/PickUpObjects/BP_MilkForAI.BP_MilkForAI_C|GetIsPoisoned? _asbp_milk_for_ai))
      (Default|Poison _asbp_milk_for_ai)
      (Audio|PlaySoundatLocation "/Game/Sounds/hit/pills_hit.pills_hit" (Transformation|GetActorLocation _asbp_milk_for_ai) "0, 0, 0" 1.0 1.0 0.0 "/Game/Sounds/Attenuation/ItemAtten.ItemAtten" 0 0)
      (Actor|DestroyActor))))

(fn ConstructionScript
  (|CallParentFunction))