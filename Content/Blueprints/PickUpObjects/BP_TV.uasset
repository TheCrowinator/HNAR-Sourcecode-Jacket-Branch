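; Pickup TV that the player can switch on and off or throw, drawing AI attention through noise.
; Toggling plays static video and audio, with a timer flickering the screen spotlight.
; A TV starting on plays the Deadman video with attached sound until switched off.
; Switching on and hard thrown impacts report noise and set the AI blackboard's ObjectRef, except window hits, which only increment the AI's ItemFallCount.
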(event Custom|TurnOnOff
  (bind _returnvalue (Transformation|GetActorLocation))
  (bind _spotlight1 (Variables|Default|GetSpotLight1))
  (bind _staticmesh (Variables|Default|GetStaticMesh))
  (bind _audio (Variables|Default|GetAudio))
  (if (Variables|Default|GetOnOff)
    (Variables|Default|SetOnOff false)
    (Audio|PlaySoundatLocation "/Game/Sounds/TV_Turn_Off.TV_Turn_Off" _returnvalue "0, 0, 0" 1.0 1.0 0.0 "/Game/Sounds/Attenuation/FridgeAttenuation.FridgeAttenuation" 0 0)
    (if (Variables|Default|GetNeighbor%20tv%20on)
      (CallFunction|Off)
      (else
        (Rendering|Material|SetMaterial _staticmesh 0 "/Game/Materials/tv_monitor_dif_Mat.tv_monitor_dif_Mat")
        (Audio|Components|Audio|Stop _audio)
        (Rendering|SetVisibility _spotlight1 false false)))
    (else
      (Audio|PlaySoundatLocation "/Game/Sounds/TV_Turn_On.TV_Turn_On" _returnvalue "0, 0, 0" 1.0 1.0 0.0 "/Game/Sounds/Attenuation/FridgeAttenuation.FridgeAttenuation" 0 0)
      (Utilities|FlowControl|Delay 0.5)
      (Rendering|Material|SetMaterial _staticmesh 0 "/Game/Movies/tv_static_player_Video_Mat.tv_static_player_Video_Mat")
      (Media|MediaPlayer|OpenSource (Variables|Default|GetScreen) "/Game/Movies/tv_static.tv_static")
      (Media|MediaPlayer|OpenSource (Variables|Default|GetLight) "/Game/Movies/tv_static.tv_static")
      (Rendering|SetVisibility _spotlight1 true false)
      (Audio|Components|Audio|Play _audio 1.0)
      (Variables|Default|SetOnOff true)
      (Class|AISenseHearing|ReportNoiseEvent (Transformation|GetWorldLocation (Variables|Default|GetStaticMesh)) 3.0 self 5e+02 "TV")
      (bind _returnvalue_2 (Actor|GetActorOfClass "/Game/Blueprints/Characters/AI2/AI.AI_C"))
      (AI|Components|Blackboard|SetValueasObject (AI|GetBlackboard _returnvalue_2) (Utilities|Name|MakeLiteralName "ObjectRef") self))))

(event Custom|On
  (bind _staticmesh (Variables|Default|GetStaticMesh))
  (Utilities|FlowControl|Delay 0.5)
  (Rendering|Material|SetMaterial _staticmesh 0 "/Game/Movies/tv_static_player_Video_Mat.tv_static_player_Video_Mat")
  (Media|MediaPlayer|OpenSource (Variables|Default|GetScreen) "/Game/Movies/deadman_tv_video.deadman_tv_video")
  (Media|MediaPlayer|OpenSource (Variables|Default|GetLight) "/Game/Movies/deadman_tv_video.deadman_tv_video")
  (bind _returnvalue (Audio|SpawnSoundAttached "/Game/Sounds/TV_sound_Cue.TV_sound_Cue" _staticmesh "None" "0, 0, 0" "0, 0, 0" "KeepRelativeOffset" false 1.0 1.0 0.0 "/Game/Sounds/Attenuation/RadioAtten.RadioAtten" 0))
  (Rendering|SetVisibility (Variables|Default|GetSpotLight1) true false)
  (Variables|Default|SetOnOff true)
  (Variables|Default|SetNeighbor%20tv%20on true))

(event Custom|Off
  (Rendering|Material|SetMaterial (Variables|Default|GetStaticMesh) 0 "/Game/Materials/tv_monitor_dif_Mat.tv_monitor_dif_Mat")
  (Audio|Components|Audio|Stop (stale Custom|On _returnvalue))
  (Rendering|SetVisibility (Variables|Default|GetSpotLight1) false false)
  (Variables|Default|SetOnOff false)
  (Variables|Default|SetNeighbor%20tv%20on false))

(event Custom|OffHunt
  (Variables|Default|SetOnOff false)
  (Rendering|Material|SetMaterial (Variables|Default|GetStaticMesh) 0 "/Game/Materials/tv_monitor_dif_Mat.tv_monitor_dif_Mat")
  (Audio|Components|Audio|Stop (Variables|Default|GetAudio))
  (Rendering|SetVisibility (Variables|Default|GetSpotLight1) false false))

(event Custom|Tick
  (if (Variables|Default|GetOnOff)
    (Rendering|Components|Light|SetIntensity (Variables|Default|GetSpotLight1) (Math|Random|RandomFloatinRange 1.1e+04 5e+03))))

(event Custom|CustomEvent
  (params (SelfActor :type Actor%20Object%20Reference) (OtherActor :type Actor%20Object%20Reference) (NormalImpulse :type Vector) (Hit :type Hit%20Result%20Structure%20%28by%20ref%29))
  (if (> (Math|Vector|VectorLength NormalImpulse) (Variables|Default|GetImpulse%20Threshold))
    (if (Variables|Default|GetPlayerThrown?)
      (if (Variables|Default|GetCanBeHeard?)
        (if (Utilities|String|Contains (Utilities|GetDisplayName OtherActor) "BP_Window")
          (Math|Integer|IncrementInt (Variables|/Game/Blueprints/Characters/AI2/AI.AI_C|GetItemFallCount (stale _returnvalue)) :!label _label
            (:%20%20
              _))
          (else
            (Class|AISenseHearing|ReportNoiseEvent (Transformation|GetActorLocation) 3.0 self 3e+02 "ThrownItem")
            (Development|PrintString "Thrown Item Loudly" true true "(R=0.000000,G=1.000000,B=0.707907,A=1.000000)")
            (bind _returnvalue (Actor|GetActorOfClass "/Game/Blueprints/Characters/AI2/AI.AI_C"))
            (Utilities|IsValid _returnvalue
              (:Is%20Valid
                (AI|Components|Blackboard|SetValueasObject (AI|GetBlackboard _returnvalue) (Utilities|Name|MakeLiteralName "ObjectRef") self)
                (goto _label))
              (:Is%20Not%20Valid
                _)))))
      (Variables|Default|SetPlayerThrown? false))
    (Utilities|FlowControl|DoOnce false :!label _label_2
      (:Completed
        (Audio|PlaySoundatLocation (Variables|Default|GetHit%20Sound) (.impactpoint Hit) "0, 0, 0" 1.0 1.0 0.0 0 0 0)
        (Utilities|FlowControl|Delay 0.1)
        (goto _label_2 Reset)))))

(event EventBeginPlay
  (Utilities|Time|SetTimerbyEvent (delegate Custom|Tick) 0.1 true)
  (Utilities|FlowControl|Sequence
    (:then_0
      (if (Variables|Default|GetOnOff)
        (CallFunction|On)))
    (:then_1
      (if (Variables|Default|GetHang?)
        (Physics|SetSimulatePhysics (Variables|Default|GetStaticMesh) false)))
    (:then_2
      (Utilities|FlowControl|Delay 1.0)
      (Variables|Default|SetStartTransform (Transformation|GetActorTransform)))
    (:then_3
      (Collision|BindEventtoOnActorHit (delegate Custom|CustomEvent)))))

(event EventSetSocket
  (bind _asfirst_person_character (Utilities|Casting|CastToFirstPersonCharacter (Game|GetPlayerCharacter 0)))
  (Variables|Default|SetSocket (Variables|/Game/Blueprints/Characters/FirstPersonBP/Blueprints/FirstPersonCharacter.FirstPersonCharacter_C|GetTV _asfirst_person_character)))

(event EventInteract
  (bind _returnvalue (Transformation|GetActorLocation))
  (bind _spotlight1 (Variables|Default|GetSpotLight1))
  (bind _staticmesh (Variables|Default|GetStaticMesh))
  (bind _audio (Variables|Default|GetAudio))
  (if (Variables|Default|GetOnOff)
    (Variables|Default|SetOnOff false)
    (Audio|PlaySoundatLocation "/Game/Sounds/TV_Turn_Off.TV_Turn_Off" _returnvalue "0, 0, 0" 1.0 1.0 0.0 "/Game/Sounds/Attenuation/FridgeAttenuation.FridgeAttenuation" 0 0)
    (if (Variables|Default|GetNeighbor%20tv%20on)
      (CallFunction|Off)
      (else
        (Rendering|Material|SetMaterial _staticmesh 0 "/Game/Materials/tv_monitor_dif_Mat.tv_monitor_dif_Mat")
        (Audio|Components|Audio|Stop _audio)
        (Rendering|SetVisibility _spotlight1 false false)))
    (else
      (Audio|PlaySoundatLocation "/Game/Sounds/TV_Turn_On.TV_Turn_On" _returnvalue "0, 0, 0" 1.0 1.0 0.0 "/Game/Sounds/Attenuation/FridgeAttenuation.FridgeAttenuation" 0 0)
      (Utilities|FlowControl|Delay 0.5)
      (Rendering|Material|SetMaterial _staticmesh 0 "/Game/Movies/tv_static_player_Video_Mat.tv_static_player_Video_Mat")
      (Media|MediaPlayer|OpenSource (Variables|Default|GetScreen) "/Game/Movies/tv_static.tv_static")
      (Media|MediaPlayer|OpenSource (Variables|Default|GetLight) "/Game/Movies/tv_static.tv_static")
      (Rendering|SetVisibility _spotlight1 true false)
      (Audio|Components|Audio|Play _audio 1.0)
      (Variables|Default|SetOnOff true)
      (Class|AISenseHearing|ReportNoiseEvent (Transformation|GetWorldLocation (Variables|Default|GetStaticMesh)) 3.0 self 5e+02 "TV")
      (bind _returnvalue_2 (Actor|GetActorOfClass "/Game/Blueprints/Characters/AI2/AI.AI_C"))
      (AI|Components|Blackboard|SetValueasObject (AI|GetBlackboard _returnvalue_2) (Utilities|Name|MakeLiteralName "ObjectRef") self))))

(event EventUse
  (bind _returnvalue (Transformation|GetActorLocation))
  (bind _spotlight1 (Variables|Default|GetSpotLight1))
  (bind _staticmesh (Variables|Default|GetStaticMesh))
  (bind _audio (Variables|Default|GetAudio))
  (if (Variables|Default|GetOnOff)
    (Variables|Default|SetOnOff false)
    (Audio|PlaySoundatLocation "/Game/Sounds/TV_Turn_Off.TV_Turn_Off" _returnvalue "0, 0, 0" 1.0 1.0 0.0 "/Game/Sounds/Attenuation/FridgeAttenuation.FridgeAttenuation" 0 0)
    (if (Variables|Default|GetNeighbor%20tv%20on)
      (CallFunction|Off)
      (else
        (Rendering|Material|SetMaterial _staticmesh 0 "/Game/Materials/tv_monitor_dif_Mat.tv_monitor_dif_Mat")
        (Audio|Components|Audio|Stop _audio)
        (Rendering|SetVisibility _spotlight1 false false)))
    (else
      (Audio|PlaySoundatLocation "/Game/Sounds/TV_Turn_On.TV_Turn_On" _returnvalue "0, 0, 0" 1.0 1.0 0.0 "/Game/Sounds/Attenuation/FridgeAttenuation.FridgeAttenuation" 0 0)
      (Utilities|FlowControl|Delay 0.5)
      (Rendering|Material|SetMaterial _staticmesh 0 "/Game/Movies/tv_static_player_Video_Mat.tv_static_player_Video_Mat")
      (Media|MediaPlayer|OpenSource (Variables|Default|GetScreen) "/Game/Movies/tv_static.tv_static")
      (Media|MediaPlayer|OpenSource (Variables|Default|GetLight) "/Game/Movies/tv_static.tv_static")
      (Rendering|SetVisibility _spotlight1 true false)
      (Audio|Components|Audio|Play _audio 1.0)
      (Variables|Default|SetOnOff true)
      (Class|AISenseHearing|ReportNoiseEvent (Transformation|GetWorldLocation (Variables|Default|GetStaticMesh)) 3.0 self 5e+02 "TV")
      (bind _returnvalue_2 (Actor|GetActorOfClass "/Game/Blueprints/Characters/AI2/AI.AI_C"))
      (AI|Components|Blackboard|SetValueasObject (AI|GetBlackboard _returnvalue_2) (Utilities|Name|MakeLiteralName "ObjectRef") self))))

(fn ConstructionScript
  (|CallParentFunction))