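; BP_Umbrella1 is an umbrella pickup that lowers the first-person player's gravity while it is picked up, slowing falls.
; SetSocket points its Socket at the character's Umbrella component.
; Tick uses a DoOnce to reduce GravityScale once on pickup, then restores normal gravity and resets the gate every frame while not picked up.
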(event Collision|EventActorBeginOverlap
  (params (OtherActor :type Actor%20Object%20Reference)))

(event EventTick
  (params (DeltaSeconds :type Float%20%28single-precision%29))
  (bind _returnvalue (Game|GetPlayerCharacter 0))
  (if (Variables|Default|GetIsPickedUp?)
    (Utilities|FlowControl|DoOnce false :!label _label
      (:Completed
        (bind _asfirst_person_character (Utilities|Casting|CastToFirstPersonCharacter _returnvalue))
        (Variables|/Script/Engine.CharacterMovementComponent|SetGravityScale (Variables|/Script/Engine.Character|GetCharacterMovement _asfirst_person_character) 0.3)))
    (else
      (bind _asfirst_person_character_2 (Utilities|Casting|CastToFirstPersonCharacter _returnvalue))
      (Variables|/Script/Engine.CharacterMovementComponent|SetGravityScale (Variables|/Script/Engine.Character|GetCharacterMovement _asfirst_person_character_2) 1.0)
      (goto _label Reset))))

(event EventSetSocket
  (bind _asfirst_person_character (Utilities|Casting|CastToFirstPersonCharacter (Game|GetPlayerCharacter 0)))
  (Variables|Default|SetSocket (Variables|/Game/Blueprints/Characters/FirstPersonBP/Blueprints/FirstPersonCharacter.FirstPersonCharacter_C|GetUmbrella _asfirst_person_character)))

(fn ConstructionScript
  (|CallParentFunction))