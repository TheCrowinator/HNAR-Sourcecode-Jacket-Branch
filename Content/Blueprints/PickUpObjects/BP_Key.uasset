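; BP_Key is a pickup key item that releases a BP_Lock with a matching code.
; SetSocket assigns the first-person character's Key as its socket.
; Use runs the character's short visibility trace and, on a code match, enables physics on the lock's mesh and marks it as pickupable.
; A disconnected chain holds an unused sequence that plays a key animation with input disabled, unlocks the door and enables its nav link.
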(event EventBeginPlay
  (|CallParentFunction) ; This node is disabled and will not be called.\nDrag off pins to build functionality.
)

(event Collision|EventActorBeginOverlap
  (params (OtherActor :type Actor%20Object%20Reference)))

(event EventTick
  (params (DeltaSeconds :type Float%20%28single-precision%29)))

(event EventSetSocket
  (bind _asfirst_person_character (Utilities|Casting|CastToFirstPersonCharacter (Game|GetPlayerCharacter 0)))
  (Variables|Default|SetSocket (Variables|/Game/Blueprints/Characters/FirstPersonBP/Blueprints/FirstPersonCharacter.FirstPersonCharacter_C|GetKey _asfirst_person_character)))

(event EventUse
  (bind _asfirst_person_character (Utilities|Casting|CastToFirstPersonCharacter (Game|GetPlayerCharacter 0)))
  (bind (_out_hit _return_value) (Default|Trace _asfirst_person_character "TraceTypeQuery1" "None" 2.5e+02))
  (if _return_value
    (bind _asbp_lock (Utilities|Casting|CastToBP_Lock (.HitActor (Collision|BreakHitResult _out_hit))))
    (if (Utilities|Enum|Equal(Enum) (Variables|/Game/Blueprints/PickUpObjects/BP_Lock.BP_Lock_C|GetCode _asbp_lock) (Variables|Default|GetCode))
      (Physics|SetSimulatePhysics (Variables|/Game/Blueprints/PickUpObjects/BP_Interactable.BP_Interactable_C|GetStaticMesh _asbp_lock) true)
      (Variables|/Game/Blueprints/PickUpObjects/BP_Interactable.BP_Interactable_C|SetCanPickUp? _asbp_lock true))))

(fn ConstructionScript
  (|CallParentFunction))