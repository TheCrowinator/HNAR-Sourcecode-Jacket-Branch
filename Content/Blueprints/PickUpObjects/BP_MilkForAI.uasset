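; Pickup milk bottle actor, named as meant for AI, that can be switched between poisoned and clean states.
; SetSocket stores the player FirstPersonCharacter's MilkForAI reference in Socket.
; Poison and Unpoison swap the mesh's first material between poisoned and normal water-bottle materials and set IsPoisoned to match.
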(event Custom|Poison
  (Rendering|Material|SetMaterial (Variables|Default|GetStaticMesh) 0 "/Game/Materials/bottle_water_poisoned_m.bottle_water_poisoned_m")
  (Variables|Default|SetIsPoisoned? true))

(event Custom|Unpoison
  (Rendering|Material|SetMaterial (Variables|Default|GetStaticMesh) 0 "/Game/Materials/bottle_water_m.bottle_water_m")
  (Variables|Default|SetIsPoisoned? false))

(event EventBeginPlay
  (|CallParentFunction) ; This node is disabled and will not be called.\nDrag off pins to build functionality.
)

(event Collision|EventActorBeginOverlap
  (params (OtherActor :type Actor%20Object%20Reference)))

(event EventTick
  (params (DeltaSeconds :type Float%20%28single-precision%29)))

(event EventSetSocket
  (bind _asfirst_person_character (Utilities|Casting|CastToFirstPersonCharacter (Game|GetPlayerCharacter 0)))
  (Variables|Default|SetSocket (Variables|/Game/Blueprints/Characters/FirstPersonBP/Blueprints/FirstPersonCharacter.FirstPersonCharacter_C|GetMilkForAI _asfirst_person_character)))

(fn ConstructionScript
  (|CallParentFunction))