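; BP_Wrench is a pickup wrench tool that the player uses to open bolts on a ladder door.
; SetSocket assigns its socket from the first-person character's Wrench reference.
; Use runs a short visibility trace through the character and, on hitting a BP_LadderDoor_w_bolt, passes the hit component to its OpenBolt.
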(event EventBeginPlay
  (|CallParentFunction) ; This node is disabled and will not be called.\nDrag off pins to build functionality.
)

(event Collision|EventActorBeginOverlap
  (params (OtherActor :type Actor%20Object%20Reference)))

(event EventTick
  (params (DeltaSeconds :type Float%20%28single-precision%29)))

(event EventSetSocket
  (bind _asfirst_person_character (Utilities|Casting|CastToFirstPersonCharacter (Game|GetPlayerCharacter 0)))
  (Variables|Default|SetSocket (Variables|/Game/Blueprints/Characters/FirstPersonBP/Blueprints/FirstPersonCharacter.FirstPersonCharacter_C|GetWrench _asfirst_person_character)))

(event EventUse
  (bind _asfirst_person_character (Utilities|Casting|CastToFirstPersonCharacter (Game|GetPlayerCharacter 0)))
  (bind (_out_hit _return_value) (Default|Trace _asfirst_person_character "TraceTypeQuery1" "None" 2.5e+02))
  (if _return_value
    (bind _asbp_ladder_door_w_bolt (Utilities|Casting|CastToBP_LadderDoor_w_bolt (.HitActor (Collision|BreakHitResult _out_hit))))
    (Default|OpenBolt _asbp_ladder_door_w_bolt (.HitComponent (Collision|BreakHitResult _out_hit)))))

(fn ConstructionScript
  (|CallParentFunction))