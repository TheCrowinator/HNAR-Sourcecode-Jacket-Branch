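; Pickup chair that can be thrown or wedged under a closed door's ChairBlock to barricade it.
; Use traces for the door, drops the chair from inventory and snaps it to the Stool transform.
; Hard thrown impacts play sound and can alert the AI through noise and blackboard, except on windows.
; A looping timer re-enables the door's NavLink on pickup; NeighborKick restores physics and releases the door.
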(event Custom|Tick
  (bind _door (Variables|Default|GetDoor))
  (Utilities|IsValid _door
    (:Is%20Valid
      (if (== (Variables|/Game/Blueprints/BP_Door.BP_Door_C|GetSelectChair _door) self)
        (if (Variables|Default|GetIsPickedUp?)
          (Utilities|FlowControl|DoOnce false :!label _label
            (:Completed
              (Utilities|FlowControl|Delay 0.02)
              (Class|NavLinkProxy|SetSmartLinkEnabled (Variables|/Game/Blueprints/BP_Door.BP_Door_C|GetNavLink _door) true)
              (Variables|/Game/Blueprints/BP_Door.BP_Door_C|SetSelectChair _door 0)))
          (else
            (goto _label Reset)))))))

(event Custom|CustomEvent
  (params (SelfActor :type Actor%20Object%20Reference) (OtherActor :type Actor%20Object%20Reference) (NormalImpulse :type Vector) (Hit :type Hit%20Result%20Structure%20%28by%20ref%29))
  (if (> (Math|Vector|VectorLength NormalImpulse) (Variables|Default|GetImpulse%20Threshold))
    (if (Variables|Default|GetPlayerThrown?)
      (if (Variables|Default|GetCanBeHeard?)
        (if (Utilities|String|Contains (Utilities|GetDisplayName OtherActor) "BP_Window")
          (Math|Integer|IncrementInt (Variables|/Game/Blueprints/Characters/AI2/AI.AI_C|GetItemFallCount (stale _returnvalue)) :!label _label
            (:%20%20
              _))
          (else
            (Class|AISenseHearing|ReportNoiseEvent (Transformation|GetActorLocation) 3.0 self 3e+02 "ThrownItem")
            (Development|PrintString "Thrown Item Loudly" true true "(R=0.000000,G=1.000000,B=0.707907,A=1.000000)")
            (bind _returnvalue (Actor|GetActorOfClass "/Game/Blueprints/Characters/AI2/AI.AI_C"))
            (Utilities|IsValid _returnvalue
              (:Is%20Valid
                (AI|Components|Blackboard|SetValueasObject (AI|GetBlackboard _returnvalue) (Utilities|Name|MakeLiteralName "ObjectRef") self)
                (goto _label))
              (:Is%20Not%20Valid
                _)))))
      (Variables|Default|SetPlayerThrown? false))
    (Utilities|FlowControl|DoOnce false :!label _label_2
      (:Completed
        (Audio|PlaySoundatLocation (Variables|Default|GetHit%20Sound) (.impactpoint Hit) "0, 0, 0" 1.0 1.0 0.0 0 0 0)
        (Utilities|FlowControl|Delay 0.1)
        (goto _label_2 Reset)))))

(event EventUse2)

(event EventBeginPlay
  (Utilities|Time|SetTimerbyEvent (delegate Custom|Tick) 0.01 true)
  (Collision|BindEventtoOnActorHit (delegate Custom|CustomEvent)))

(event EventSetSocket
  (bind _asfirst_person_character (Utilities|Casting|CastToFirstPersonCharacter (Game|GetPlayerCharacter 0)))
  (Variables|Default|SetSocket (Variables|/Game/Blueprints/Characters/FirstPersonBP/Blueprints/FirstPersonCharacter.FirstPersonCharacter_C|GetStool _asfirst_person_character)))

(event EventNeighborKick
  (params (AI :type AI%20Object%20Reference))
  (bind _door (Variables|Default|GetDoor))
  (|CallParentFunction AI)
  (Utilities|FlowControl|Delay 0.65)
  (Physics|SetSimulatePhysics (Variables|Default|GetStaticMesh) true)
  (Utilities|IsValid _door
    (:Is%20Valid
      (Variables|/Game/Blueprints/BP_Door.BP_Door_C|SetSelectChair _door 0))))

(event EventUse
  (bind _asfirst_person_character (Utilities|Casting|CastToFirstPersonCharacter (Game|GetPlayerCharacter 0)))
  (bind (_out_hit _return_value) (Default|Trace _asfirst_person_character "TraceTypeQuery3" "None" 2.5e+02))
  (if _return_value
    (bind _asbp_door (Utilities|Casting|CastToBP_Door (.HitActor (Collision|BreakHitResult _out_hit))))
    (bind _asbp_double_door (Utilities|Casting|CastToBP_DoubleDoor (.HitActor (Collision|BreakHitResult _out_hit)))
      (:then
        (if (not (Variables|/Game/Blueprints/BP_DoubleDoor.BP_DoubleDoor_C|GetOpen_1 _asbp_double_door))
          (if (Variables|/Game/Blueprints/BP_Door.BP_Door_C|GetCanLockDoorWithChair? _asbp_door) :!label _label
            (if (not (Variables|/Game/Blueprints/BP_Door.BP_Door_C|GetIsLockedWithChair? _asbp_door))
              (if (not (Variables|/Game/Blueprints/BP_Door.BP_Door_C|GetOpen _asbp_door))
                (if (== (.HitComponent (Collision|BreakHitResult _out_hit)) (Variables|/Game/Blueprints/BP_Door.BP_Door_C|GetChairBlock _asbp_door))
                  (Variables|Default|SetDoor _asbp_door)
                  (Utilities|Array|RemoveItem (Variables|/Game/Blueprints/Characters/FirstPersonBP/Blueprints/FirstPersonCharacter.FirstPersonCharacter_C|GetInventory _asfirst_person_character) self)
                  (Transformation|DetachFromActor "KeepRelative" "KeepRelative" "KeepWorld")
                  (Math|Integer|DecrementInt (Variables|/Game/Blueprints/Characters/FirstPersonBP/Blueprints/FirstPersonCharacter.FirstPersonCharacter_C|GetSelectedItem _asfirst_person_character)
                    (:%20%20
                      (Collision|SetCollisionEnabled (Variables|Default|GetStaticMesh) "QueryAndPhysics")
                      (Variables|Default|SetIsPickedUp? false)
                      (Transformation|SetActorLocationAndRotation (.location (Transformation|GetWorldTransform (Variables|/Game/Blueprints/BP_Door.BP_Door_C|GetStool _asbp_door))) (.rotation (Transformation|GetWorldTransform (Variables|/Game/Blueprints/BP_Door.BP_Door_C|GetStool _asbp_door))))
                      (Default|SetChair _asbp_door self)
                      (Audio|PlaySoundatLocation "/Game/Sounds/prop_door_close_Cue.prop_door_close_Cue" (Transformation|GetWorldLocation (Variables|/Game/Blueprints/BP_Door.BP_Door_C|GetScene1 _asbp_door)) "0, 0, 0" 1.0 1.0 0.05 "/Game/Sounds/Attenuation/ItemAtten.ItemAtten" 0 0)))))))))
      (:CastFailed
        (goto _label)))))

(fn ConstructionScript
  (|CallParentFunction))