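; Physics-based interactable item that can be picked up, dropped, heard by the AI when thrown and kicked aside by the neighbor AI.
; Pickup and drop toggle physics and collision, while use, interact and socket events are empty stubs.
; Hard hits play a sound; player throws can report noise, set the AI's blackboard target and count falls, with special handling for windows.
; AI contact triggers a timed kick animation and impulse, guarded by a resetting DoOnce.
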(event OnComponentHit(StaticMesh)
  (params (HitComponent :type Primitive%20Component%20Object%20Reference) (OtherActor :type Actor%20Object%20Reference) (OtherComp :type Primitive%20Component%20Object%20Reference) (NormalImpulse :type Vector :default "0, 0, 0") (Hit :type Hit%20Result%20Structure%20%28by%20ref%29))
  (bind _asai (Utilities|Casting|CastToAI OtherActor))
  (if (Variables|Default|GetCanKick?)
    (if (Variables|/Game/Blueprints/Characters/AI2/AI.AI_C|GetCanAIKick _asai)
      (if (not (Utilities|Enum|Equal(Enum) (Class|SkeletalMeshComponent|GetAnimationMode (Variables|/Script/Engine.Character|GetMesh _asai)) "AnimationSingleNode"))
        (CallFunction|NeighborKick _asai)))))

(event Custom|NeighborKick
  (params (AI :type AI%20Object%20Reference))
  (bind _alphaanims (Variables|/Game/Blueprints/Characters/AI2/AI.AI_C|GetAlphaAnims AI))
  (if (not (Variables|Default|GetIsPickedUp?))
    (Utilities|FlowControl|DoOnce false :!label _label
      (:Completed
        (Utilities|FlowControl|Delay 0.2)
        (Default|DisableMovement AI)
        (Default|PlayAnimAI AI (select _alphaanims "/Game/Neighbor/Animations/neighbour_lowpoly_Anim_rig_kick.neighbour_lowpoly_Anim_rig_kick" "/Game/Neighbor/Guest/neighbor_lowpoly_Anim_rig_kick.neighbor_lowpoly_Anim_rig_kick") false)
        (Utilities|FlowControl|Delay (select _alphaanims 0.55 0.6))
        (Physics|AddImpulse (Variables|Default|GetStaticMesh) (* (Math|Rotator|GetRotationXVector (Transformation|GetWorldRotation (Variables|/Game/Blueprints/Characters/AI2/AI.AI_C|GetKick%20arrow AI))) 1e+05) "None" false)
        (Development|PrintString "KICKED RTHING" true true "(R=1.000000,G=0.755026,B=0.000000,A=1.000000)" 1e+01)
        (Utilities|FlowControl|Delay (select _alphaanims 0.81 0.48))
        (Default|EnableMovement AI)
        (Components|Animation|SetAnimationMode (Variables|/Script/Engine.Character|GetMesh AI) "AnimationBlueprint")
        (goto _label Reset)))))

(event Custom|Pick%20Up
  (bind _staticmesh (Variables|Default|GetStaticMesh))
  (Physics|SetSimulatePhysics _staticmesh false)
  (Collision|SetCollisionEnabled _staticmesh "NoCollision")
  (Variables|Default|SetIsPickedUp? true)
  (Audio|PlaySoundatLocation (Variables|Default|GetPick%20Up%20Sound) (Transformation|GetWorldLocation _staticmesh) "0, 0, 0" 1.0 1.0 0.0 0 0 0))

(event Custom|Use%202)

(event Custom|Interact)

(event Custom|Drop
  (bind _staticmesh (Variables|Default|GetStaticMesh))
  (Physics|SetSimulatePhysics _staticmesh true)
  (Collision|SetCollisionEnabled _staticmesh "QueryAndPhysics")
  (Variables|Default|SetIsPickedUp? false))

(event Custom|SetSocket)

(event Custom|HitEvent
  (params (SelfActor :type Actor%20Object%20Reference) (OtherActor :type Actor%20Object%20Reference) (NormalImpulse :type Vector) (Hit :type Hit%20Result%20Structure%20%28by%20ref%29))
  (if (> (Math|Vector|VectorLength NormalImpulse) (Variables|Default|GetImpulse%20Threshold))
    (if (Variables|Default|GetPlayerThrown?)
      (if (Variables|Default|GetCanBeHeard?)
        (if (Utilities|String|Contains (Utilities|GetDisplayName OtherActor) "BP_Window")
          (Math|Integer|IncrementInt (Variables|/Game/Blueprints/Characters/AI2/AI.AI_C|GetItemFallCount (stale _returnvalue)) :!label _label
            (:%20%20
              _))
          (else
            (Class|AISenseHearing|ReportNoiseEvent (Transformation|GetActorLocation) 3.0 self 3e+02 "ThrownItem")
            (Development|PrintString "Thrown Item Loudly" true true "(R=0.000000,G=1.000000,B=0.707907,A=1.000000)")
            (bind _returnvalue (Actor|GetActorOfClass "/Game/Blueprints/Characters/AI2/AI.AI_C"))
            (Utilities|IsValid _returnvalue
              (:Is%20Valid
                (AI|Components|Blackboard|SetValueasObject (AI|GetBlackboard _returnvalue) (Utilities|Name|MakeLiteralName "ObjectRef") self)
                (goto _label))
              (:Is%20Not%20Valid
                _)))))
      (Variables|Default|SetPlayerThrown? false))
    (Utilities|FlowControl|DoOnce false :!label _label_2
      (:Completed
        (Audio|PlaySoundatLocation (Variables|Default|GetHit%20Sound) (.impactpoint Hit) "0, 0, 0" 1.0 1.0 0.0 0 0 0)
        (Utilities|FlowControl|Delay 0.1)
        (goto _label_2 Reset)))))

(event Custom|SetNeighborSocket)

(event Custom|Use)

(event EventBeginPlay
  (bind _staticmesh (Variables|Default|GetStaticMesh))
  (Utilities|FlowControl|Sequence
    (:then_0
      (Class|PrimitiveComponent|SetNotifyRigidBodyCollision (Variables|Default|GetStaticMesh) true)
      (Collision|BindEventtoOnActorHit (delegate Custom|HitEvent)))
    (:then_1
      (Variables|Default|SetIsPickedUp? false))
    (:then_2
      (if (Variables|Default|GetHang?)
        (Physics|SetSimulatePhysics _staticmesh false)
        (else
          (Physics|SetSimulatePhysics _staticmesh true))))
    (:then_3
      (Utilities|FlowControl|Delay 1.0)
      (Variables|Default|SetStartTransform (Transformation|GetActorTransform)))))

(fn ConstructionScript)