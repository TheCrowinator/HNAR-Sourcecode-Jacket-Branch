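; Blue lamp pickup that can be thrown by the player to make noise that draws the AI's attention.
; At BeginPlay it takes the character's Lamp socket and binds a hit handler, which plays impact sounds throttled by a short DoOnce reset.
; Hard, audible thrown impacts report noise, set the lamp as the AI blackboard's ObjectRef and increment its fall count.
; Window hits skip the noise and only increment that count.
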(event Custom|CustomEvent
  (params (SelfActor :type Actor%20Object%20Reference) (OtherActor :type Actor%20Object%20Reference) (NormalImpulse :type Vector) (Hit :type Hit%20Result%20Structure%20%28by%20ref%29))
  (if (> (Math|Vector|VectorLength NormalImpulse) (Variables|Default|GetImpulse%20Threshold))
    (if (Variables|Default|GetPlayerThrown?)
      (if (Variables|Default|GetCanBeHeard?)
        (if (Utilities|String|Contains (Utilities|GetDisplayName OtherActor) "BP_Window")
          (Math|Integer|IncrementInt (Variables|/Game/Blueprints/Characters/AI2/AI.AI_C|GetItemFallCount (stale _returnvalue)) :!label _label
            (:%20%20
              _))
          (else
            (Class|AISenseHearing|ReportNoiseEvent (Transformation|GetActorLocation) 3.0 self 3e+02 "ThrownItem")
            (Development|PrintString "Thrown Item Loudly" true true "(R=0.000000,G=1.000000,B=0.707907,A=1.000000)")
            (bind _returnvalue (Actor|GetActorOfClass "/Game/Blueprints/Characters/AI2/AI.AI_C"))
            (Utilities|IsValid _returnvalue
              (:Is%20Valid
                (AI|Components|Blackboard|SetValueasObject (AI|GetBlackboard _returnvalue) (Utilities|Name|MakeLiteralName "ObjectRef") self)
                (goto _label))
              (:Is%20Not%20Valid
                _)))))
      (Variables|Default|SetPlayerThrown? false))
    (Utilities|FlowControl|DoOnce false :!label _label_2
      (:Completed
        (Audio|PlaySoundatLocation (Variables|Default|GetHit%20Sound) (.impactpoint Hit) "0, 0, 0" 1.0 1.0 0.0 0 0 0)
        (Utilities|FlowControl|Delay 0.1)
        (goto _label_2 Reset)))))

(event EventBeginPlay
  (bind _asfirst_person_character (Utilities|Casting|CastToFirstPersonCharacter (Game|GetPlayerCharacter 0)))
  (Variables|Default|SetSocket (Variables|/Game/Blueprints/Characters/FirstPersonBP/Blueprints/FirstPersonCharacter.FirstPersonCharacter_C|GetLamp _asfirst_person_character))
  (Collision|BindEventtoOnActorHit (delegate Custom|CustomEvent)))

(fn ConstructionScript
  (|CallParentFunction))