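; Pickup binoculars that give the player a zoomed view and can be thrown to make noise the AI hears.
; Use2 narrows the camera FOV and swaps the HUD for an overlay widget; Tick polls mouse and gamepad input to restore them.
; Hard hits play a throttled impact sound.
; Audible throws report noise, set the AI's blackboard ObjectRef and raise ItemFallCount, while window hits only attempt the count increment.
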(event Custom|CustomEvent
  (params (SelfActor :type Actor%20Object%20Reference) (OtherActor :type Actor%20Object%20Reference) (NormalImpulse :type Vector) (Hit :type Hit%20Result%20Structure%20%28by%20ref%29))
  (if (> (Math|Vector|VectorLength NormalImpulse) (Variables|Default|GetImpulse%20Threshold))
    (if (Variables|Default|GetPlayerThrown?)
      (if (Variables|Default|GetCanBeHeard?)
        (if (Utilities|String|Contains (Utilities|GetDisplayName OtherActor) "BP_Window")
          (Math|Integer|IncrementInt (Variables|/Game/Blueprints/Characters/AI2/AI.AI_C|GetItemFallCount (stale _returnvalue)) :!label _label
            (:%20%20
              _))
          (else
            (Class|AISenseHearing|ReportNoiseEvent (Transformation|GetActorLocation) 3.0 self 3e+02 "ThrownItem")
            (Development|PrintString "Thrown Item Loudly" true true "(R=0.000000,G=1.000000,B=0.707907,A=1.000000)")
            (bind _returnvalue (Actor|GetActorOfClass "/Game/Blueprints/Characters/AI2/AI.AI_C"))
            (Utilities|IsValid _returnvalue
              (:Is%20Valid
                (AI|Components|Blackboard|SetValueasObject (AI|GetBlackboard _returnvalue) (Utilities|Name|MakeLiteralName "ObjectRef") self)
                (goto _label))
              (:Is%20Not%20Valid
                _)))))
      (Variables|Default|SetPlayerThrown? false))
    (Utilities|FlowControl|DoOnce false :!label _label_2
      (:Completed
        (Audio|PlaySoundatLocation (Variables|Default|GetHit%20Sound) (.impactpoint Hit) "0, 0, 0" 1.0 1.0 0.0 0 0 0)
        (Utilities|FlowControl|Delay 0.1)
        (goto _label_2 Reset)))))

(event EventBeginPlay
  (bind _asfirst_person_character (Utilities|Casting|CastToFirstPersonCharacter (Game|GetPlayerCharacter 0)))
  (Variables|Default|SetSocket (Variables|/Game/Blueprints/Characters/FirstPersonBP/Blueprints/FirstPersonCharacter.FirstPersonCharacter_C|GetBinoculars _asfirst_person_character))
  (bind _returnvalue (UserInterface|CreateWidget "/Game/Blueprints/UI/W_BinocularView.W_BinocularView_C"))
  (bind _output_get (Variables|Default|SetBinocularView _returnvalue))
  (UserInterface|Viewport|AddtoViewport _output_get 0)
  (Widget|SetVisibility _output_get "Hidden")
  (Collision|BindEventtoOnActorHit (delegate Custom|CustomEvent)))

(event Collision|EventActorBeginOverlap
  (params (OtherActor :type Actor%20Object%20Reference)))

(event EventTick
  (params (DeltaSeconds :type Float%20%28single-precision%29))
  (bind _returnvalue (Game|GetPlayerController 0))
  (Utilities|FlowControl|Sequence
    (:then_0
      (if (Class|PlayerController|WasInputKeyJustReleased _returnvalue "LeftMouseButton")
        (bind _asfirst_person_character (Utilities|Casting|CastToFirstPersonCharacter (Game|GetPlayerCharacter 0) :!label _label))
        (Camera|SetFieldOfView (Variables|/Game/Blueprints/Characters/FirstPersonBP/Blueprints/FirstPersonCharacter.FirstPersonCharacter_C|GetFirstPersonCamera _asfirst_person_character) 1e+02)
        (Widget|SetVisibility (Variables|Default|GetBinocularView) "Hidden")
        (Widget|SetVisibility (Variables|/Game/Blueprints/Characters/FirstPersonBP/Blueprints/FirstPersonCharacter.FirstPersonCharacter_C|GetHUD _asfirst_person_character) "Visible")))
    (:then_1
      (if (Game|Player|IsInputKeyDown _returnvalue "RightMouseButton")
        (if (Game|Player|WasInputKeyJustPressed _returnvalue "LeftMouseButton")
          (goto _label))))
    (:then_2
      (if (Class|PlayerController|WasInputKeyJustReleased _returnvalue "Gamepad_RightShoulder")
        (goto _label)))
    (:then_3
      (if (Game|Player|IsInputKeyDown _returnvalue "Gamepad_RightTrigger")
        (if (Game|Player|WasInputKeyJustPressed _returnvalue "Gamepad_RightShoulder")
          (goto _label))))))

(event EventUse)

(event EventUse2
  (bind _asfirst_person_character (Utilities|Casting|CastToFirstPersonCharacter (Game|GetPlayerCharacter 0)))
  (Camera|SetFieldOfView (Variables|/Game/Blueprints/Characters/FirstPersonBP/Blueprints/FirstPersonCharacter.FirstPersonCharacter_C|GetFirstPersonCamera _asfirst_person_character) 2e+01)
  (Widget|SetVisibility (Variables|Default|GetBinocularView) "Visible")
  (Widget|SetVisibility (Variables|/Game/Blueprints/Characters/FirstPersonBP/Blueprints/FirstPersonCharacter.FirstPersonCharacter_C|GetHUD _asfirst_person_character) "Hidden"))

(fn ConstructionScript
  (|CallParentFunction))