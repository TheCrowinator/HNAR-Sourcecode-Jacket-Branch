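; BP_Crowbar is a crowbar pickup item that the player uses on boards to unlock doors.
; SetSocket assigns the first-person character's Crowbar component as the item's socket.
; Use runs a short visibility trace from the character and, on a BP_Board not flagged CanPickUp, unlocks its door if LockDoor is set, then clears that door reference after a brief delay.
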(event EventBeginPlay
  (|CallParentFunction) ; This node is disabled and will not be called.\nDrag off pins to build functionality.
)

(event Collision|EventActorBeginOverlap
  (params (OtherActor :type Actor%20Object%20Reference)))

(event EventTick
  (params (DeltaSeconds :type Float%20%28single-precision%29)))

(event EventSetSocket
  (bind _asfirst_person_character (Utilities|Casting|CastToFirstPersonCharacter (Game|GetPlayerCharacter 0)))
  (Variables|Default|SetSocket (Variables|/Game/Blueprints/Characters/FirstPersonBP/Blueprints/FirstPersonCharacter.FirstPersonCharacter_C|GetCrowbar _asfirst_person_character)))

(event EventUse
  (bind _asfirst_person_character (Utilities|Casting|CastToFirstPersonCharacter (Game|GetPlayerCharacter 0)))
  (bind (_out_hit _return_value) (Default|Trace _asfirst_person_character "TraceTypeQuery1" "None" 2.5e+02))
  (if _return_value
    (bind _asbp_board (Utilities|Casting|CastToBP_Board (.HitActor (Collision|BreakHitResult _out_hit))))
    (if (not (Variables|/Game/Blueprints/PickUpObjects/BP_Interactable.BP_Interactable_C|GetCanPickUp? _asbp_board))
      (if (Variables|/Game/Blueprints/PickUpObjects/BP_Board.BP_Board_C|GetLockDoor? _asbp_board)
        (Variables|/Game/Blueprints/BP_Door.BP_Door_C|SetLocked (Variables|/Game/Blueprints/PickUpObjects/BP_Board.BP_Board_C|GetDoor _asbp_board) false))
      (Utilities|FlowControl|Delay 0.1)
      (Variables|/Game/Blueprints/PickUpObjects/BP_Board.BP_Board_C|SetDoor _asbp_board 0))))

(fn ConstructionScript
  (|CallParentFunction))