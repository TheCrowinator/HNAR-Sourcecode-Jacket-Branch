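; BP_Shovel is a usable pickup tool that lets the player dig at graves.
; SetSocket sets its Socket to the Shovel member of the FirstPersonCharacter.
; Use runs the character's short-range visibility Trace and calls ShovelDirt on a hit BP_Grave, only when the hit component is its GraveTop.
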(event EventBeginPlay
  (|CallParentFunction) ; This node is disabled and will not be called.\nDrag off pins to build functionality.
)

(event Collision|EventActorBeginOverlap
  (params (OtherActor :type Actor%20Object%20Reference)))

(event EventTick
  (params (DeltaSeconds :type Float%20%28single-precision%29)))

(event EventSetSocket
  (bind _asfirst_person_character (Utilities|Casting|CastToFirstPersonCharacter (Game|GetPlayerCharacter 0)))
  (Variables|Default|SetSocket (Variables|/Game/Blueprints/Characters/FirstPersonBP/Blueprints/FirstPersonCharacter.FirstPersonCharacter_C|GetShovel _asfirst_person_character)))

(event EventUse
  (bind _asfirst_person_character (Utilities|Casting|CastToFirstPersonCharacter (Game|GetPlayerCharacter 0)))
  (bind _out_hit (Default|Trace _asfirst_person_character "TraceTypeQuery1" "None" 2.5e+02))
  (bind _asbp_grave (Utilities|Casting|CastToBP_Grave (.HitActor (Collision|BreakHitResult _out_hit))))
  (if (== (.HitComponent (Collision|BreakHitResult _out_hit)) (Variables|/Game/Blueprints/PuzzleBPs/BP_Grave.BP_Grave_C|GetGrave_top _asbp_grave))
    (Default|ShovelDirt _asbp_grave)))

(fn ConstructionScript
  (|CallParentFunction))