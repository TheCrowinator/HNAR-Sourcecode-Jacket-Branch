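; BP_Jumping_NavLink is a smart nav link that makes AI characters jump to the link's destination.
; When an agent reaches it, the AI crouches, is launched, and uncrouches after JumpDuration.
; CalculateVelocity solves the ballistic launch velocity from both endpoints and the duration, using Power as the gravity term.
; BeginPlay adds a nav modifier, but logic toggling its area class and the link by BP_Neighbor's state is unconnected.
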(event EventBeginPlay
  (bind _returnvalue (AddComponent|AddNavModifierComponent))
  (Variables|Default|SetNavModifier _returnvalue)
  (Variables|Default|SetLocation (Transformation|GetActorLocation)))

(event EventTick
  (params (DeltaSeconds :type Float%20%28single-precision%29)))

(event EventSmartLinkReached
  (params (Agent :type Actor%20Object%20Reference) (Destination :type Vector%20%28by%20ref%29 :default "0, 0, 0"))
  (bind _asai (Utilities|Casting|CastToAI Agent))
  (Character|Crouch _asai)
  (bind _velocity (CallFunction|CalculateVelocity Destination (Transformation|GetActorLocation _asai) (Variables|Jump|GetJumpDuration)))
  (Character|LaunchCharacter _asai _velocity true true)
  (Utilities|FlowControl|Delay (Variables|Jump|GetJumpDuration))
  (Character|UnCrouch _asai))

(fn ConstructionScript)

(fn CalculateVelocity
  (params (DestinationLocation :type Vector) (StartingLocation :type Vector) (Duration :type Float%20%28single-precision%29))
  (bind (_x _y _z) (Math|Vector|BreakVector StartingLocation))
  (bind (_x_2 _y_2 _z_2) (Math|Vector|BreakVector DestinationLocation))
  (LocalVariables|SetInDuration Duration)
  (return (Math|Vector|MakeVector (/ (- _x_2 _x) (LocalVariables|GetInDuration)) (/ (- _y_2 _y) (LocalVariables|GetInDuration)) (/ (- _z_2 (+ _z (* (Math|Float|Square (LocalVariables|GetInDuration)) -0.5 (Variables|Jump|GetPower)))) (LocalVariables|GetInDuration)))))