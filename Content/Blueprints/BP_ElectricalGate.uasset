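; BP_ElectricalGate is a gate that closes while its linked PowerSwitch has working power and opens when power is lost.
; Tick polls PowerWorking and routes each state through its own DoOnce, which the opposite transition resets, so each move fires once per change.
; MoveComponentTo animates StaticMesh1 between unrotated and tilted poses at the same location, and the Open flag tracks the state.
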(event EventBeginPlay)

(event Collision|EventActorBeginOverlap
  (params (OtherActor :type Actor%20Object%20Reference)))

(event EventTick
  (params (DeltaSeconds :type Float%20%28single-precision%29))
  (if (Variables|/Game/Blueprints/BP_PowerSwitch.BP_PowerSwitch_C|GetPowerWorking? (Variables|Default|GetPowerSwitch))
    (Utilities|FlowControl|DoOnce false :!label _label
      (:Completed
        (Components|MoveComponentTo (Variables|Default|GetStaticMesh1) "254.000000, 0,185.000000" "0, 0, 0" false false 2.0 false)
        (Variables|Default|SetOpen? false)
        (goto _label_2 Reset)))
    (else
      (Utilities|FlowControl|DoOnce false :!label _label_2
        (:Completed
          (Components|MoveComponentTo (Variables|Default|GetStaticMesh1) "254.000000, 0,185.000000" "0,20.000000, 0" false false 2.0 false)
          (Variables|Default|SetOpen? true)
          (goto _label Reset))))))

(fn ConstructionScript)