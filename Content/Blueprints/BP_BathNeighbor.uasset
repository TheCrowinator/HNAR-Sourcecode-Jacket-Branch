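; BP_BathNeighbor is an actor for a toggleable water faucet, apparently in a neighbor's bath.
; An IsOn flag tracks its state: turning on plays the running audio and squeak cue and activates the particle system, while turning off squeaks, stops the audio and deactivates particles.
; TurnOnOff toggles the state, and ForceTurnOn switches it on only if it is off, sharing the same turn-on logic.
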(event Custom|TurnOnOff
  (bind _audio (Variables|Default|GetAudio))
  (bind _particlesystem (Variables|Default|GetParticleSystem))
  (if (Variables|Default|GetIsOn?)
    (Audio|Components|Audio|Play (Variables|Default|Getfaucet_squeak_Cue) 0.0)
    (Audio|Components|Audio|Stop _audio)
    (Components|Activation|Deactivate _particlesystem)
    (Variables|Default|SetIsOn? false)
    (else
      (Audio|Components|Audio|Play _audio 0.0)
      (Components|Activation|Activate _particlesystem false)
      (Variables|Default|SetIsOn? true))))

(event Custom|ForceTurnOn
  (if (not (Variables|Default|GetIsOn?))
    (Audio|Components|Audio|Play (Variables|Default|GetAudio) 0.0)
    (Components|Activation|Activate (Variables|Default|GetParticleSystem) false)
    (Variables|Default|SetIsOn? true)))

(event EventBeginPlay)

(event Collision|EventActorBeginOverlap
  (params (OtherActor :type Actor%20Object%20Reference)))

(event EventTick
  (params (DeltaSeconds :type Float%20%28single-precision%29)))

(fn ConstructionScript)