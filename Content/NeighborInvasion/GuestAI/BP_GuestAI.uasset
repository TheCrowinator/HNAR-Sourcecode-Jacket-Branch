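; Guest AI character for Neighbor Invasion that switches between walk and run speeds and voices calm or nervous speech loops.
; Tick reads the CanFollow blackboard key to pick the Croak sound, with two cross-resetting DoOnce gates so each swap fires only on a change.
; Walk and Run events set movement speed and trigger those gates.
; BeginPlay caches an Arrow actor, and PlayRandomAnim plays a supplied animation, returning its length.
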(event Custom|Walk
  (bind _croak (Variables|Default|Getcroak))
  (Variables|/Script/Engine.CharacterMovementComponent|SetMaxWalkSpeed (Variables|Character|GetCharacterMovement) 3e+02)
  (Utilities|FlowControl|DoOnce false
    (:Completed
      (Audio|Components|Audio|SetSound _croak "/Game/Sounds/Guest/SN_Speak_CALM_loop_Cue.SN_Speak_CALM_loop_Cue")
      (Utilities|FlowControl|DoOnce false) ; enters at Reset
    )))

(event Custom|Run
  (bind _croak (Variables|Default|Getcroak))
  (Variables|/Script/Engine.CharacterMovementComponent|SetMaxWalkSpeed (Variables|Character|GetCharacterMovement) 6e+02)
  (Utilities|FlowControl|DoOnce false
    (:Completed
      (Audio|Components|Audio|SetSound _croak "/Game/Sounds/Guest/SN_Speak_NERVOUS_loop_Cue.SN_Speak_NERVOUS_loop_Cue")
      (Utilities|FlowControl|DoOnce false) ; enters at Reset
    )))

(event EventBeginPlay
  (CallFunction|Walk)
  (bind _returnvalue (Actor|GetActorOfClass "/Game/Blueprints/Arrow.Arrow_C"))
  (Variables|Default|SetArrow _returnvalue))

(event Collision|EventActorBeginOverlap
  (params (OtherActor :type Actor%20Object%20Reference)))

(event EventTick
  (params (DeltaSeconds :type Float%20%28single-precision%29))
  (bind _croak (Variables|Default|Getcroak))
  (if (ScalableFloat|GetValueasBool (AI|GetBlackboard 0) (Utilities|Name|MakeLiteralName "CanFollow"))
    (Utilities|FlowControl|DoOnce false :!label _label
      (:Completed
        (Audio|Components|Audio|SetSound _croak "/Game/Sounds/Guest/SN_Speak_NERVOUS_loop_Cue.SN_Speak_NERVOUS_loop_Cue")
        (goto _label_2 Reset)))
    (else
      (Utilities|FlowControl|DoOnce false :!label _label_2
        (:Completed
          (Audio|Components|Audio|SetSound _croak "/Game/Sounds/Guest/SN_Speak_CALM_loop_Cue.SN_Speak_CALM_loop_Cue")
          (goto _label Reset))))))

(fn ConstructionScript)

(fn PlayRandomAnim
  (params (NewAnimToPlay :type Anim%20Sequence%20Base%20Object%20Reference) (bLooping :type Boolean))
  (Components|Animation|PlayAnimation (Variables|Character|GetMesh) NewAnimToPlay bLooping)
  (bind _returnvalue (Animation|GetPlayLength NewAnimToPlay))
  (return _returnvalue))