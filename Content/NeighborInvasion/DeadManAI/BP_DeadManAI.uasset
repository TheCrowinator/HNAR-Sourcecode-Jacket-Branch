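; Dead Man AI character for Neighbor Invasion that voices idle or hunt sounds according to its movement state.
; Walk and Run events set movement speed and the sound-state enum, and BeginPlay caches a BP_Cake reference.
; A self-timed CustomTick with a random delay plays the matching sound at irregular intervals.
; When the blackboard's IsShot is true, it stops the playing sound once and switches to a third state.
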(event Custom|Walk
  (Variables|/Script/Engine.CharacterMovementComponent|SetMaxWalkSpeed (Variables|Character|GetCharacterMovement) 1.5e+02)
  (Variables|Default|SetEnum "NewEnumerator0"))

(event Custom|Run
  (Variables|/Script/Engine.CharacterMovementComponent|SetMaxWalkSpeed (Variables|Character|GetCharacterMovement) 6e+02)
  (Variables|Default|SetEnum "NewEnumerator1"))

(event Custom|CustomTick
  (bind _deadmanidle (Variables|Default|GetDeadmanIdle))
  (bind _deadmanhunt (Variables|Default|GetDeadmanHunt))
  (Utilities|Time|SetTimerbyEvent (delegate Custom|CustomTick) 0.1 true)
  (Utilities|FlowControl|Delay (Math|Random|RandomFloatinRange 5.0 2e+01))
  (Utilities|FlowControl|Sequence
    (:then_0
      (if (Utilities|Enum|Equal(Enum) (Variables|Default|GetEnum) "NewEnumerator0")
        (Audio|Components|Audio|Play _deadmanidle 0.0)
        (elif (Utilities|Enum|Equal(Enum) (Variables|Default|GetEnum) "NewEnumerator1")
          (Audio|Components|Audio|Play _deadmanhunt 0.0))))
    (:then_1
      (if (ScalableFloat|GetValueasBool (AI|GetBlackboard 0) (Utilities|Name|MakeLiteralName "IsShot"))
        (Utilities|FlowControl|DoOnce false :!label _label
          (:Completed
            (if (Audio|Components|Audio|IsPlaying _deadmanhunt)
              (Audio|Components|Audio|Stop _deadmanhunt)
              (Variables|Default|SetEnum "NewEnumerator2")
              (elif (Audio|Components|Audio|IsPlaying _deadmanidle)
                (Audio|Components|Audio|Stop _deadmanidle)
                (Variables|Default|SetEnum "NewEnumerator2")))))
        (else
          (goto _label Reset))))))

(event Custom|ResetSoundValue
  (Variables|Default|SetEnum "NewEnumerator0"))

(event EventBeginPlay
  (bind _returnvalue (Actor|GetActorOfClass "/Game/Blueprints/PickUpObjects/BP_Cake.BP_Cake_C"))
  (Variables|Default|SetCake _returnvalue)
  (CallFunction|CustomTick))

(fn ConstructionScript)