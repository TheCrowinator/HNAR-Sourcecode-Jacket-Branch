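; BP_MoonCreator is a tool actor that bakes a procedural moon texture into the RT_Moon render target.
; A dynamic material instance on its Plane receives the atmosphere, color, detail and resolution settings.
; Render clears the target, then draws that material twice: with Mask at 1 using DetailMap, then at 0 with ColorMap in the same texture slot.
; It runs from the Construction Script and again on BeginPlay.
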(event Custom|Render
  (Rendering|Material|SetScalarParameterValue (Variables|Default|GetMaterialInst) "AtmosphereSize" (Variables|Default|GetAtmosphereSize) :!class /Script/Engine.MaterialInstanceDynamic)
  (Rendering|Material|SetScalarParameterValue (Variables|Default|GetMaterialInst) "AtmosphereInShadow" (Variables|Default|GetAtmosphereInShadow) :!class /Script/Engine.MaterialInstanceDynamic)
  (Rendering|Material|SetScalarParameterValue (Variables|Default|GetMaterialInst) "DetailScale" (Variables|Default|GetDetailScale) :!class /Script/Engine.MaterialInstanceDynamic)
  (Rendering|Material|SetScalarParameterValue (Variables|Default|GetMaterialInst) "TetureResolution" (Variables|Default|GetSampleResolution) :!class /Script/Engine.MaterialInstanceDynamic)
  (Rendering|Material|SetScalarParameterValue (Variables|Default|GetMaterialInst) "ColorBase" (Variables|Default|GetColorBase) :!class /Script/Engine.MaterialInstanceDynamic)
  (Rendering|Material|SetScalarParameterValue (Variables|Default|GetMaterialInst) "ColorScale" (Variables|Default|GetColorScale) :!class /Script/Engine.MaterialInstanceDynamic)
  (Rendering|Material|SetScalarParameterValue (Variables|Default|GetMaterialInst) "AtmosphereExp" (Variables|Default|GetAtmosphereExp) :!class /Script/Engine.MaterialInstanceDynamic)
  (Rendering|Material|SetScalarParameterValue (Variables|Default|GetMaterialInst) "AtmosphereBase" (Variables|Default|GetAtmosphereBase) :!class /Script/Engine.MaterialInstanceDynamic)
  (Rendering|Material|SetTextureParameterValue (Variables|Default|GetMaterialInst) "DetailMap" (Variables|Default|GetDetailMap))
  (Rendering|ClearRenderTarget2D "/Game/FastStylizedProceduralSky2/Tools/MoonCreator/RT_Moon.RT_Moon")
  (Rendering|Material|SetScalarParameterValue (Variables|Default|GetMaterialInst) "Mask" 1.0 :!class /Script/Engine.MaterialInstanceDynamic)
  (Rendering|DrawMaterialtoRenderTarget "/Game/FastStylizedProceduralSky2/Tools/MoonCreator/RT_Moon.RT_Moon" (Variables|Default|GetMaterialInst))
  (Rendering|Material|SetScalarParameterValue (Variables|Default|GetMaterialInst) "Mask" 0.0 :!class /Script/Engine.MaterialInstanceDynamic)
  (Rendering|Material|SetTextureParameterValue (Variables|Default|GetMaterialInst) "DetailMap" (Variables|Default|GetColorMap))
  (Rendering|DrawMaterialtoRenderTarget "/Game/FastStylizedProceduralSky2/Tools/MoonCreator/RT_Moon.RT_Moon" (Variables|Default|GetMaterialInst)))

(event EventBeginPlay
  (CallFunction|Render))

(event Collision|EventActorBeginOverlap
  (params (OtherActor :type Actor%20Object%20Reference)))

(event EventTick
  (params (DeltaSeconds :type Float%20%28single-precision%29)))

(fn ConstructionScript
  (bind _returnvalue (Rendering|Material|CreateDynamicMaterialInstance (Variables|Default|GetPlane) 0 0 :!class /Script/Engine.PrimitiveComponent))
  (Variables|Default|SetMaterialInst _returnvalue)
  (CallFunction|Render))