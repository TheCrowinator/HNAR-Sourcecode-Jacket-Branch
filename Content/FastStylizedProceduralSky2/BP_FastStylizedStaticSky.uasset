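; BP_FastStylizedStaticSky is a static sky actor that displays a chosen sky texture on its mesh.
; The construction script creates a dynamic material instance from either a skydome or a sky cube material, based on UseSkydome.
; It passes SkyTexture to the matching texture parameter, and the dome path also sets a sky sphere UV toggle.
; It has no active runtime logic, as all event graph nodes are disabled.
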(event EventBeginPlay)

(event Collision|EventActorBeginOverlap
  (params (OtherActor :type Actor%20Object%20Reference)))

(event EventTick
  (params (DeltaSeconds :type Float%20%28single-precision%29)))

(fn ConstructionScript
  (bind _staticmesh (Variables|Default|GetStaticMesh))
  (if (Variables|Default|GetUseSkydome)
    (bind _returnvalue (Rendering|Material|CreateDynamicMaterialInstance _staticmesh 0 "/Game/FastStylizedProceduralSky2/Materials/MI_StaticSkyDome.MI_StaticSkyDome" :!class /Script/Engine.PrimitiveComponent))
    (bind _output_get (Variables|Default|SetMaterialInstance _returnvalue))
    (Rendering|Material|SetTextureParameterValue _output_get "WorldLayer" (Variables|Default|GetSkyTexture))
    (Rendering|Material|SetScalarParameterValue _output_get "SkySphereUV" (select (Variables|Default|GetUseSkySphereUV) 1.0 0.0) :!class /Script/Engine.MaterialInstanceDynamic)
    (else
      (bind _returnvalue_2 (Rendering|Material|CreateDynamicMaterialInstance _staticmesh 0 "/Game/FastStylizedProceduralSky2/Materials/MI_StaticSkyCube.MI_StaticSkyCube" :!class /Script/Engine.PrimitiveComponent))
      (bind _output_get_2 (Variables|Default|SetMaterialInstance _returnvalue_2))
      (Rendering|Material|SetTextureParameterValue _output_get_2 "WorldLayerCube" (Variables|Default|GetSkyTexture)))))