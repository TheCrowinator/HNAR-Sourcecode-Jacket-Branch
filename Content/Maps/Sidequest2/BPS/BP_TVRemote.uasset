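; BP_TVRemote is a TV remote item that lets the player interact with a TV from a distance.
; On Use, it line-traces forward from the first-person camera on the Camera channel and calls Interact on a hit BP_TV, printing a debug message for any other hit.
; SetSocket assigns the player character's RemoteTV to the item's Socket variable.
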(event EventBeginPlay
  (|CallParentFunction) ; This node is disabled and will not be called.\nDrag off pins to build functionality.
)

(event Collision|EventActorBeginOverlap
  (params (OtherActor :type Actor%20Object%20Reference)))

(event EventTick
  (params (DeltaSeconds :type Float%20%28single-precision%29)))

(event EventUse
  (bind _asfirst_person_character (Utilities|Casting|CastToFirstPersonCharacter (Game|GetPlayerCharacter 0)))
  (bind (_outhit _returnvalue) (Collision|LineTraceByChannel (Transformation|GetWorldLocation (Variables|/Game/Blueprints/Characters/FirstPersonBP/Blueprints/FirstPersonCharacter.FirstPersonCharacter_C|GetFirstPersonCamera _asfirst_person_character)) (+ (* (Math|Vector|GetForwardVector (Variables|/Game/Blueprints/Characters/FirstPersonBP/Blueprints/FirstPersonCharacter.FirstPersonCharacter_C|GetFirstPersonCamera _asfirst_person_character)) 1525.0) (Transformation|GetWorldLocation (Variables|/Game/Blueprints/Characters/FirstPersonBP/Blueprints/FirstPersonCharacter.FirstPersonCharacter_C|GetFirstPersonCamera _asfirst_person_character))) "TraceTypeQuery2" false 0 "None"))
  (if _returnvalue
    (bind _asbp_tv (Utilities|Casting|CastToBP_TV (.HitActor (Collision|BreakHitResult _outhit)))
      (:then
        (Default|Interact _asbp_tv))
      (:CastFailed
        (Development|PrintString "OH BOY NATE YOUR CODE IS SHIT")))))

(event EventSetSocket
  (bind _asfirst_person_character (Utilities|Casting|CastToFirstPersonCharacter (Game|GetPlayerCharacter 0)))
  (Variables|Default|SetSocket (Variables|/Game/Blueprints/Characters/FirstPersonBP/Blueprints/FirstPersonCharacter.FirstPersonCharacter_C|GetRemote_TV _asfirst_person_character)))

(fn ConstructionScript
  (|CallParentFunction))