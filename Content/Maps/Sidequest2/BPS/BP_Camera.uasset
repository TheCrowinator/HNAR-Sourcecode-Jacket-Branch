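; BP_Camera is a security camera that spots the player and alerts the AI.
; A looping self-rescheduled timer event checks whether the player overlaps the Cone, then line-traces from the camera to confirm visibility.
; DoOnce gates fire on each change: detection starts the audio, reports a noise and sets the camera as the AI blackboard's ObjectRef, while losing sight stops the audio.
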(event Custom|Tick
  (bind _audio (Variables|Default|GetAudio))
  (Utilities|Time|SetTimerbyEvent (delegate Custom|Tick) 0.01)
  (bind _asfirst_person_character (Utilities|Casting|CastToFirstPersonCharacter (Game|GetPlayerCharacter 0)))
  (if (Collision|IsOverlappingActor (Variables|Default|GetCone) _asfirst_person_character :!class /Script/Engine.PrimitiveComponent)
    (bind (_outhit _returnvalue) (Collision|LineTraceByChannel (Transformation|GetWorldLocation (Variables|Default|GetCamera)) (Transformation|GetActorLocation _asfirst_person_character) "TraceTypeQuery1" false 0 "None"))
    (if _returnvalue
      (Utilities|FlowControl|Sequence
        (:then_0
          (goto _label_3 Reset))
        (:then_1
          (Utilities|Casting|CastToFirstPersonCharacter (.HitActor (Collision|BreakHitResult _outhit))
            (:then
              (Utilities|FlowControl|DoOnce false :!label _label
                (:Completed
                  (Audio|Components|Audio|Play _audio 0.0)
                  (Class|AISenseHearing|ReportNoiseEvent (Transformation|GetActorLocation) 5.0 self 6e+02 "Camera")
                  (bind _returnvalue_2 (Actor|GetActorOfClass "/Game/Blueprints/Characters/AI2/AI.AI_C"))
                  (Utilities|IsValid _returnvalue_2
                    (:Is%20Valid
                      (AI|Components|Blackboard|SetValueasObject (AI|GetBlackboard _returnvalue_2) (Utilities|Name|MakeLiteralName "ObjectRef") self))))))
            (:CastFailed
              (Utilities|FlowControl|Sequence :!label _label_2
                (:then_0
                  (goto _label Reset))
                (:then_1
                  (Utilities|FlowControl|DoOnce false :!label _label_3
                    (:Completed
                      (Audio|Components|Audio|Stop _audio)))))))))
      (else
        (goto _label_2)))
    (else
      (goto _label_2))))

(event EventBeginPlay
  (CallFunction|Tick))

(event Collision|EventActorBeginOverlap
  (params (OtherActor :type Actor%20Object%20Reference)))

(event EventTick
  (params (DeltaSeconds :type Float%20%28single-precision%29)))

(fn ConstructionScript)