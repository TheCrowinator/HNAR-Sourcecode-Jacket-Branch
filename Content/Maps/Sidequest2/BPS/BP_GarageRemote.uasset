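; Garage remote item that opens or closes a garage door the player is looking at.
; On Use, a camera-channel line trace from the first-person camera finds a BP_GarageDoor and toggles it based on its IsOpen state.
; A successful hit briefly switches the remote's bulb material to green before returning it to red.
; SetSocket assigns the player character's RemoteG as the item's socket.
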(event EventBeginPlay
  (|CallParentFunction) ; This node is disabled and will not be called.\nDrag off pins to build functionality.
)

(event Collision|EventActorBeginOverlap
  (params (OtherActor :type Actor%20Object%20Reference)))

(event EventTick
  (params (DeltaSeconds :type Float%20%28single-precision%29)))

(event EventUse
  (bind _sphere (Variables|Default|GetSphere))
  (bind _asfirst_person_character (Utilities|Casting|CastToFirstPersonCharacter (Game|GetPlayerCharacter 0)))
  (bind (_outhit _returnvalue) (Collision|LineTraceByChannel (Transformation|GetWorldLocation (Variables|/Game/Blueprints/Characters/FirstPersonBP/Blueprints/FirstPersonCharacter.FirstPersonCharacter_C|GetFirstPersonCamera _asfirst_person_character)) (+ (* (Math|Vector|GetForwardVector (Variables|/Game/Blueprints/Characters/FirstPersonBP/Blueprints/FirstPersonCharacter.FirstPersonCharacter_C|GetFirstPersonCamera _asfirst_person_character)) 1525.0) (Transformation|GetWorldLocation (Variables|/Game/Blueprints/Characters/FirstPersonBP/Blueprints/FirstPersonCharacter.FirstPersonCharacter_C|GetFirstPersonCamera _asfirst_person_character))) "TraceTypeQuery2" false 0 "None"))
  (if _returnvalue
    (bind _asbp_garage_door (Utilities|Casting|CastToBP_GarageDoor (.HitActor (Collision|BreakHitResult _outhit)))
      (:then
        (Utilities|FlowControl|Sequence
          (:then_0
            (if (Variables|/Game/Blueprints/BP_GarageDoor.BP_GarageDoor_C|GetIsOpen? _asbp_garage_door)
              (Default|Close _asbp_garage_door)
              (else
                (Default|Open _asbp_garage_door))))
          (:then_1
            (Rendering|Material|SetMaterial _sphere 0 "/Game/Materials/bulb_green.bulb_green")
            (Utilities|FlowControl|Delay 0.5)
            (Rendering|Material|SetMaterial _sphere 0 "/Game/Materials/bulb_red.bulb_red"))))
      (:CastFailed
        (Development|PrintString "OH BOY NATE YOUR CODE IS SHIT the door wont open plz fix bitch")))))

(event EventSetSocket
  (bind _asfirst_person_character (Utilities|Casting|CastToFirstPersonCharacter (Game|GetPlayerCharacter 0)))
  (Variables|Default|SetSocket (Variables|/Game/Blueprints/Characters/FirstPersonBP/Blueprints/FirstPersonCharacter.FirstPersonCharacter_C|GetRemote_G _asfirst_person_character)))

(fn ConstructionScript
  (|CallParentFunction))